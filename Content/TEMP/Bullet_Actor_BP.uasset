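; A test bullet actor that moves its ECS entity along its owner's forward vector through Ck transform requests.
; On BeginPlay it copies the owner's rotation, then steps immediately and on a looping timer.
; Each server-only step requests a fixed location offset and draws a debug sphere ahead of the actor.
; The construction script resets the transform to identity; per-frame movement and copying the entity transform to the actor are disconnected.
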(event `ServerTick`
  (bind _returnvalue (* (`self.GetActorForwardVector` (`self.GetOwner`)) 500.0))
  (if (`KismetSystemLibrary.IsServer`) :!label _label
    (`Ck_Utils_Transform_UE.Request_AddLocationOffset` (`Ck_EcsConstructionScript_ActorComponent_UE._Entity` (`self.Ecs_ConstructionScript_AC`)) (make `Ck_Request_Transform_AddLocationOffset` _returnvalue))
    (`KismetSystemLibrary.DrawDebugSphere` (+ (`self.K2_GetActorLocation`) _returnvalue) 100.0 12 (struct :`R` 1.0 :`B` 0.045875 :`A` 1.0) 2.0 5.0)))

(event `self.ReceiveBeginPlay`
  (`self.K2_SetActorRotation` (`self.K2_GetActorRotation` (`self.GetOwner`)))
  (`KismetSystemLibrary.K2_SetTimerDelegate` (delegate `ServerTick`) 2.0 true)
  (goto _label))

(event `self.ReceiveTick`
  (params (DeltaSeconds :type "Float (single-precision)"))
  (if (`KismetSystemLibrary.IsServer`)
    _))

(fn `UserConstructionScript`
  (`self.K2_SetActorTransform` (`KismetMathLibrary.MakeTransform` (0.0 0.0 0.0))))