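; A Blueprint task that listens for events on an ability owner and fires its EventFired output when an event name exactly matches one of the supplied tags.
; On activation it binds to the owner's events, ignoring payloads already in flight.
; Each incoming batch fires at most once, for the first match.
; It keeps listening until End or Deactivate unbinds it.
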(event `self.Activate_BP`
  (`Ck_Utils_AbilityOwner_UE.BindTo_OnEvents` (`self.InAbilityOwnerHandle`) "IgnorePayloadInFlight" (delegate `OnEvent`)))

(event `OnEvent`
  (params (InHandle :type "Ck_Handle Structure") (InEvents :type "Array of Ck_AbilityOwner_Event Structure (by ref)"))
  (for _array_element InEvents
    (bind __eventname (break `Ck_AbilityOwner_Event` _array_element))
    (if (`BlueprintGameplayTagLibrary.HasTag` (`self.InTagsToTest`) __eventname true)
      (`self.EventFired` __eventname)
      (break))))

(event `Deactivate`
  (`Ck_Utils_AbilityOwner_UE.UnbindFrom_OnEvents` (`self.InAbilityOwnerHandle`) (delegate `OnEvent`)))

(fn `End`
  (`self.Deactivate`))