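; A CkUI widget component Blueprint that links its widget to the actor that owns the component.
; After the parent's post-init widget step, non-server instances ensure the widget is valid, cast it to Ck_UserWidget_UE and call BindToActor with the owner.
; An invalid widget or one of the wrong type triggers an ensure naming the component and actor.
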(event `self.OnPostInitWidget`
  (bind _returnvalue (`self.GetWidget`))
  (`parent.OnPostInitWidget`)
  (if (not (`KismetSystemLibrary.IsServer`))
    (`Ck_Utils_Ensure_UE.EnsureMsgf_IsValid` _returnvalue (`|FormatText` "WidgetComponent [{comp}] on Actor [{actor}] has an INVALID Widget! WidgetClass supplied: [{widgetClass}]" self (`self.GetOwner`) (`KismetSystemLibrary.GetClassDisplayName` (`GameplayStatics.GetObjectClass` (`self.GetWidget`))))
      (:`Valid`
        (bind _asck_user_widget_ue (cast `Ck_UserWidget_UE` _returnvalue)
          (:`then`
            (`Ck_UserWidget_UE.BindToActor` _asck_user_widget_ue (`self.GetOwner`)))
          (:`CastFailed`
            (`Ck_Utils_Ensure_UE.TriggerEnsure` (`|FormatText` "WidgetComponent [{comp}] on Actor [{actor}] is handling Widget [{widget}] that is NOT of type UCk_UserWidget_UE. Unable to BindToActor properly." self (`self.GetOwner`) (`KismetSystemLibrary.GetClassDisplayName` (`GameplayStatics.GetObjectClass` (`self.GetWidget`)))))))))))