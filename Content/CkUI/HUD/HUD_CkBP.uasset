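; HUD Blueprint that spawns the game's HUD widget and keeps it bound to the player's controlled pawn.
; On BeginPlay it validates and async-loads the soft HUD widget class, then creates the widget for the primary player controller.
; Once created, it waits for the game session login event, binds the widget to the pawn, then rebinds it whenever possession changes.
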(event `self.ReceiveBeginPlay`
  (`parent.ReceiveBeginPlay`)
  (`Ck_Utils_Ensure_UE.EnsureMsgf` (`KismetSystemLibrary.IsValidSoftClassReference` (`self._HUD_WidgetClass`)) (`|FormatText` self "Invalid HUD Widget Class set in HUD [{self}]")
    (:`Valid`
      (bind _class (`|LoadAssetClass` (`self._HUD_WidgetClass`))
        (:`Completed`
          (bind _asck_hud_user_widget_ue (castclass `Ck_HUD_UserWidget_UE` _class))
          (bind _returnvalue (`|CreateWidget` _asck_hud_user_widget_ue (`Ck_Utils_Game_UE.Get_PrimaryPlayerController`)))
          (set `self._HUD_WidgetInstance` _returnvalue)
          (`self.OnHUD_WidgetCreated`))))))

(event `OnHUD_WidgetCreated`
  ;[0.05469 0 1] OnHUD_WidgetCreated
  (`Ck_GameSession_Subsystem_UE.BindTo_OnLoginEvent` (subsystem `Ck_GameSession_Subsystem_UE`) "FireIfPayloadInFlight" "Unbind" (delegate `CustomEvent`)))

(event `CustomEvent`
  (params (InPlayerController :type "PlayerController Object Reference") (InAllPlayerControllers :type "Array of PlayerController Object Reference (by ref)"))
  (bind _returnvalue (`Controller.K2_GetPawn` InPlayerController))
  ;[0.05469 0 1] OnHUD_WidgetCreated
  (`/Engine/EditorBlueprintResources/StandardMacros.IsValid` _returnvalue
    (:`Is Valid`
      (`Ck_UserWidget_UE.BindToActor` (`self._HUD_WidgetInstance`) _returnvalue))
    (:`Is Not Valid`
      _))
  (add `Controller.OnPossessedPawnChanged` InPlayerController (delegate `OnPossessedPawnChanged`)))

(event `OnPossessedPawnChanged`
  (params (OldPawn :type "Pawn Object Reference") (NewPawn :type "Pawn Object Reference"))
  ;[0.05469 0 1] OnHUD_WidgetCreated
  (`Ck_UserWidget_UE.UnbindFromActor` (`self._HUD_WidgetInstance`) OldPawn)
  (`/Engine/EditorBlueprintResources/StandardMacros.IsValid` NewPawn
    (:`Is Valid`
      (`Ck_UserWidget_UE.BindToActor` (`self._HUD_WidgetInstance`) NewPawn))))

(fn `UserConstructionScript`)