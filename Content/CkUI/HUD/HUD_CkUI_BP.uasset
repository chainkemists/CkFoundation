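; HUD Blueprint that spawns the player's main HUD widget and keeps it bound to the pawn they control.
; On BeginPlay it validates the soft widget class, async-loads it, then creates the Ck_HUD_UserWidget for player controller 0 and adds it to the viewport.
; Once created, the widget binds to the current pawn and follows possession changes, unbinding from the old pawn and binding to the new one.
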(event `self.ReceiveBeginPlay`
  (`parent.ReceiveBeginPlay`)
  (`Ck_Utils_Ensure_UE.EnsureMsgf` (`KismetSystemLibrary.IsValidSoftClassReference` (`self._HUD_WidgetClass`)) (`|FormatText` self "Invalid HUD Widget Class set in HUD [{self}]")
    (:`Valid`
      (bind _class (`|LoadAssetClass` (`self._HUD_WidgetClass`))
        (:`Completed`
          (bind _asck_hud_user_widget_ue (castclass `Ck_HUD_UserWidget_UE` _class))
          (bind _returnvalue (`|CreateWidget` _asck_hud_user_widget_ue (`GameplayStatics.GetPlayerController` 0)))
          (bind _output_get (set `self._HUD_WidgetInstance` _returnvalue))
          (`UserWidget.AddToViewport` _output_get 0)
          (`self.OnHUD_WidgetCreated`))))))

(event `OnHUD_WidgetCreated`
  (bind _returnvalue (`GameplayStatics.GetPlayerController` 0))
  (bind _returnvalue_2 (`Controller.K2_GetPawn` _returnvalue))
  ;[0.05469 0 1] OnHUD_WidgetCreated
  (`/Engine/EditorBlueprintResources/StandardMacros.IsValid` _returnvalue_2
    (:`Is Valid`
      (`Ck_UserWidget_UE.BindToActor` (`self._HUD_WidgetInstance`) _returnvalue_2))
    (:`Is Not Valid`
      _))
  (add `Controller.OnPossessedPawnChanged` _returnvalue (delegate `OnPossessedPawnChanged`)))

(event `OnPossessedPawnChanged`
  (params (OldPawn :type "Pawn Object Reference") (NewPawn :type "Pawn Object Reference"))
  ;[0.05469 0 1] OnHUD_WidgetCreated
  (`/Engine/EditorBlueprintResources/StandardMacros.IsValid` OldPawn
    (:`Is Valid`
      (`Ck_UserWidget_UE.UnbindFromActor` (`self._HUD_WidgetInstance`) OldPawn))
    (:`Is Not Valid`
      _))
  (`/Engine/EditorBlueprintResources/StandardMacros.IsValid` NewPawn
    (:`Is Valid`
      (`Ck_UserWidget_UE.BindToActor` (`self._HUD_WidgetInstance`) NewPawn))))

(fn `UserConstructionScript`)