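; Base Blueprint StateTree condition that supplies the description text shown for a condition.
; ReceiveGetDescription passes the class display name to GetDescriptionWithNot, which prepends a NOT prefix when Invert is set.
; The prefix follows the requested formatting, bold markup for rich text and plain otherwise.
; The file contains no condition test logic, only description formatting.
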(fn `Get_DescriptionWithNot`
  (params (Formatting :type "EStateTreeNodeFormatting Enum" :default "RichText") (Description :type Text))
  (returns (Result :type Text))
  (return (`|FormatText` "{Prefix} {Description}" (select `EStateTreeNodeFormatting` Formatting :`RichText` (`KismetMathLibrary.SelectText` "<b>NOT</>" "" (`self.Invert`)) :`Text` (`KismetMathLibrary.SelectText` "NOT" "" (`self.Invert`))) Description)))

(fn `ReceiveGetDescription`
  (params (Formatting :type "EStateTreeNodeFormatting Enum" :default "RichText"))
  (returns (ReturnValue :type Text))
  (return (`self.Get_DescriptionWithNot` Formatting (`KismetTextLibrary.Conv_StringToText` (`KismetSystemLibrary.GetClassDisplayName` (`GameplayStatics.GetObjectClass` self))))))