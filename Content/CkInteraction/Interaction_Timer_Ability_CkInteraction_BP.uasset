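; Ability that decides when an interaction completes, running on the interaction entity that owns it.
; On activation it branches on the interaction's completion policy: Instant requests a successful end immediately.
; Timed listens for value changes on the interaction's time attribute and requests a successful end when the value equals exactly 1.0.
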(event `self.DoOnActivateAbility`
  (params (InActivationPayload :type "Ck_Ability_Payload_OnActivate Structure (by ref)"))
  (`parent.DoOnActivateAbility` InActivationPayload)
  (bind _output_get (set `self.Interaction` (`Ck_Utils_Interaction_UE.DoCastChecked` (`self.DoGet_AbilityOwnerEntity`))))
  (switch `ECk_Interaction_CompletionPolicy` (`Ck_Utils_Interaction_UE.Get_InteractionCompletionPolicy` _output_get)
    (:`Instant`
      (`Ck_Utils_Interaction_UE.Request_EndInteraction` (`self.Interaction`) (make `Ck_Request_Interaction_EndInteraction` "Succeeded")))
    (:`Timed`
      (bind (_taskobject _initialattributevalue_initialvalue_ _attributevaluechanged_attributeownerhandle _attributevaluechanged_atributehandle _attributevaluechanged_value_) (`|Blueprint_Template` (`Ck_Utils_Interaction_UE.Get_InteractionTimeAttribute` (`Ck_Utils_Interaction_UE.DoCastChecked` (`self.DoGet_AbilityOwnerEntity`))))
        (:`AttributeValueChanged`
          (if (== _attributevaluechanged_value_ 1.0)
            (`Ck_Utils_Interaction_UE.Request_EndInteraction` (`self.Interaction`) (make `Ck_Request_Interaction_EndInteraction` "Succeeded"))))))))