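; Base interact-source ability that turns interaction sensor overlaps into interaction requests while active.
; On activation it binds to the owner's Sensor.Interaction begin and end overlaps, unbinding on deactivation.
; Each overlap maps the marker name to an interaction channel, then resolves that channel's source and target from the sensor and marker owners.
; Begin overlap starts the interaction on the target if permitted; end overlap cancels it on the source.
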(event `self.DoOnActivateAbility`
  (params (InActivationPayload :type "Ck_Ability_Payload_OnActivate Structure (by ref)"))
  (`parent.DoOnActivateAbility` InActivationPayload)
  (bind _output_get (set `self.SensorHandle` (`Ck_Utils_Sensor_UE.TryGet_Sensor` (`self.DoGet_ContextEntityWithActor`) (struct :`TagName` "Sensor.Interaction"))))
  (bind _outhandle (`/CkFoundation/CkEcs/EntityHandle_CkEcs_ML.ValidateEntityHandle` _output_get)
    (:`IsValid`
      (bind _returnvalue (`Ck_Utils_Sensor_UE.BindTo_OnBeginOverlap` _outhandle "FireIfPayloadInFlightThisFrame" (delegate `OnBeginOverlap`)))
      (`Ck_Utils_Sensor_UE.BindTo_OnEndOverlap` _returnvalue "FireIfPayloadInFlightThisFrame" (delegate `OnEndOverlap`)))
    (:`NotValid`
      (`Ck_Utils_Ensure_UE.TriggerEnsure` "Interaction Sensor NOT found!"))))

(event `OnBeginOverlap`
  (params (InHandle :type "Ck_Handle Structure") (InPayload :type "Ck_Sensor_Payload_OnBeginOverlap Structure"))
  (bind (__sensordetails __markerdetails) (break `Ck_Sensor_Payload_OnBeginOverlap` InPayload))
  (bind _interactsource (`self.InteractSource`))
  (bind _output_get (set `self.InteractionChannel` (`self.GetInteractionChannelFromMarker` __markerdetails)))
  (if (`BlueprintGameplayTagLibrary.IsGameplayTagValid` _output_get)
    (bind _output_get_2 (set `self.InteractSource` (`self.GetInteractionSourceFromSensor` __sensordetails (`self.InteractionChannel`))))
    (`/CkFoundation/CkEcs/EntityHandle_CkEcs_ML.ValidateEntityHandle` _output_get_2
      (:`IsValid`
        (bind _output_get_3 (set `self.InteractTarget` (`self.GetInteractionTargetFromMarker` __markerdetails (`self.InteractionChannel`))))
        (`/CkFoundation/CkEcs/EntityHandle_CkEcs_ML.ValidateEntityHandle` _output_get_3
          (:`IsValid`
            (switch `ECk_CanInteractWithResult` (`Ck_Utils_InteractTarget_UE.Get_CanInteractWith` (`self.InteractTarget`) (`self.InteractSource`))
              (:`CanInteractWith`
                (`Ck_Utils_InteractTarget_UE.Request_StartInteraction` (`self.InteractTarget`) (make `Ck_Try_InteractTarget_StartInteraction` _interactsource _interactsource))))))))))

(event `OnEndOverlap`
  (params (InHandle :type "Ck_Handle Structure") (InPayload :type "Ck_Sensor_Payload_OnEndOverlap Structure"))
  (bind (__sensordetails __markerdetails) (break `Ck_Sensor_Payload_OnEndOverlap` InPayload))
  (bind _output_get (set `self.InteractionChannel` (`self.GetInteractionChannelFromMarker` __markerdetails)))
  (if (`BlueprintGameplayTagLibrary.IsGameplayTagValid` _output_get)
    (bind _output_get_2 (set `self.InteractSource` (`self.GetInteractionSourceFromSensor` __sensordetails (`self.InteractionChannel`))))
    (`/CkFoundation/CkEcs/EntityHandle_CkEcs_ML.ValidateEntityHandle` _output_get_2
      (:`IsValid`
        (bind _output_get_3 (set `self.InteractTarget` (`self.GetInteractionTargetFromMarker` __markerdetails (`self.InteractionChannel`))))
        (`/CkFoundation/CkEcs/EntityHandle_CkEcs_ML.ValidateEntityHandle` _output_get_3
          (:`IsValid`
            (`Ck_Utils_InteractSource_UE.Request_CancelInteraction` (`self.InteractSource`) (make `Ck_Request_InteractSource_CancelInteraction` (`self.InteractTarget`)))))))))

(event `self.DoOnDeactivateAbility`
  (`parent.DoOnDeactivateAbility`)
  (bind _returnvalue (`Ck_Utils_Sensor_UE.UnbindFrom_OnBeginOverlap` (`self.SensorHandle`) (`|CreateDelegate` :!event `OnBeginOverlap`)))
  (`Ck_Utils_Sensor_UE.UnbindFrom_OnEndOverlap` _returnvalue (`|CreateDelegate` :!event `OnEndOverlap`)))

(fn `GetInteractionChannelFromMarker`
  (params (Ck_Marker_BasicDetails :type "Ck_Marker_BasicDetails Structure (by ref)"))
  (returns (OutputPin :type "GameplayTag Structure"))
  (bind (_value _returnvalue) (`BlueprintMapLibrary.Map_Find` (`self.MarkerNameToInteractionChannel`) (`._MarkerName` (break `Ck_Marker_BasicDetails` Ck_Marker_BasicDetails))))
  (if _returnvalue
    (return _value)
    (else
      (return))))

(fn `GetInteractionSourceFromSensor`
  (params (Ck_Sensor_BasicDetails :type "Ck_Sensor_BasicDetails Structure (by ref)") (InInteractionChannel :type "GameplayTag Structure"))
  (returns (ReturnValue :type "Ck_Handle_InteractSource Structure"))
  (return (`Ck_Utils_InteractSource_UE.TryGet` (`._Handle` (break `Ck_EntityOwningActor_BasicDetails` (`._SensorAttachedEntityAndActor` (break `Ck_Sensor_BasicDetails` Ck_Sensor_BasicDetails)))) InInteractionChannel)))

(fn `GetInteractionTargetFromMarker`
  (params (Ck_Marker_BasicDetails :type "Ck_Marker_BasicDetails Structure (by ref)") (InInteractionChannel :type "GameplayTag Structure"))
  (returns (ReturnValue :type "Ck_Handle_InteractTarget Structure"))
  (return (`Ck_Utils_InteractTarget_UE.TryGet` (`._Handle` (break `Ck_EntityOwningActor_BasicDetails` (`._MarkerAttachedEntityAndActor` (break `Ck_Marker_BasicDetails` Ck_Marker_BasicDetails)))) InInteractionChannel)))