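; Base Blueprint for fractured destructible objects in CkChaos, set up as an entity-bridged actor.
; DoConstruct adds a feature to the entity, passing along the actor's replication setting.
; A disconnected draft in the event graph would listen for resolver data bundles and apply replicated radial strain to the geometry collection owner at the hit impact point.
; The replication-complete event is empty, so that damage logic never runs here.
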(event `self.EntityBridge_AC._OnReplicationComplete_MC`
  (params (InEntity :type "Ck_Handle Structure")))

(fn `DoConstruct`
  (params (InHandle :type "Ck_Handle Structure (by ref)"))
  (`Ck_Utils_GeometryCollectionOwner_UE.Add` InHandle)
  (return))

(fn `UserConstructionScript`)