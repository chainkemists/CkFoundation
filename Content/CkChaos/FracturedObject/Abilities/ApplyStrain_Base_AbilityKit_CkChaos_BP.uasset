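; Base Chaos ability that applies replicated radial strain to the geometry collection owner it is given to, for fracturing objects.
; On give, it validates its DataBundle name tag and listens for bundles completing all phases.
; A matching bundle is stored and activates the ability, which sends the strain request and immediately deactivates.
; Derived abilities must override GetImpactPointOverride to extract the strain location from the bundle; the base version only triggers an ensure.
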(event `self.DoOnGiveAbility`
  (params (InOptionalPayload :type "Ck_Ability_Payload_OnGranted Structure (by ref)"))
  (`parent.DoOnGiveAbility` InOptionalPayload)
  (`Ck_Utils_Ensure_UE.EnsureMsgf` (`BlueprintGameplayTagLibrary.IsGameplayTagValid` (`self.DataBundleName`)) (`|FormatText` "DataBundle Name is INVALID. This Ability on Context [{Context}] will not function as expected." (`Ck_Utils_Handle_UE.Conv_HandleToText` (`self.DoGet_ContextEntityWithActor`)))
    (:`Valid`
      (bind (_taskobject _onnewdatabundle_indatabundle _onphasestart_indatabundle _onphasestart_inphase _onphasecomplete_indatabundle _onphasecomplete_inphase _onphasecomplete_inpayload _onallphasescomplete_indatabundle) (`|Blueprint_Template` (`Ck_Utils_ResolverTarget_UE.DoCastChecked` (`self.DoGet_ContextEntityWithActor`)))
        (:`OnAllPhasesComplete`
          (if (`Ck_Utils_GameplayLabel_UE.Matches` _onallphasescomplete_indatabundle (`self.DataBundleName`))
            (set `self._DataBundleHandle` _onallphasescomplete_indatabundle)
            (`self.DoRequest_ActivateAbility` (struct))))))))

(event `self.DoOnActivateAbility`
  (params (InActivationPayload :type "Ck_Ability_Payload_OnActivate Structure (by ref)"))
  (`parent.DoOnActivateAbility` InActivationPayload)
  (bind _impactpoint (`self.Get Impact Point (Override)` (`self._DataBundleHandle`)))
  (`Ck_Utils_GeometryCollectionOwner_UE.Request_ApplyRadianStrain` (`Ck_Utils_GeometryCollectionOwner_UE.DoCastChecked` (`self.DoGet_ContextEntityWithActor`)) (make `Ck_Request_GeometryCollectionOwner_ApplyRadialStrain_Replicated` _impactpoint (`self.StrainData`)))
  (`self.DoRequest_DeactivateAbility`))

(fn `Get Impact Point (Override)`
  (params (InHandle :type "Ck_Handle_ResolverDataBundle Structure (by ref)"))
  (returns (ImpactPoint :type "Vector Structure"))
  (`Ck_Utils_Ensure_UE.TriggerEnsure` "This function MUST be overridden in a derived Ability")
  (return (0.0 0.0 0.0)))