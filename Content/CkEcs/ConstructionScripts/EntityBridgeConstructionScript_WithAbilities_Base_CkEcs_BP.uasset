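; Base entity bridge construction script that gives a constructed CkEcs entity an ability owner fragment with default abilities.
; DoConstruct runs the parent construction, then combines the DefaultAbilities list with the results of DoGetOtherDefaultAbilities, an empty hook that derived scripts can optionally override.
; The combined list becomes the ability owner params, added to the entity handle with the configured AbilitiesReplication setting.
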(fn `DoConstruct`
  (params (InHandle :type "Ck_Handle Structure (by ref)") (InOptionalParams :type "InstancedStruct Structure (by ref)"))
  (locals (L_DefaultAbilities :type "Array of Ck_Ability_Script_PDA Class Reference"))
  (`parent.DoConstruct` InHandle InOptionalParams)
  (bind _output_get (set `local.L_DefaultAbilities` (`self.DefaultAbilities`)))
  (`KismetArrayLibrary.Array_Append` _output_get (`self.DoGetOtherDefaultAbilities`))
  (`Ck_Utils_AbilityOwner_UE.Add` InHandle (make `Ck_Fragment_AbilityOwner_ParamsData` (`local.L_DefaultAbilities`)) (`self.AbilitiesReplication`))
  (return))

(fn `DoGetOtherDefaultAbilities`
  (returns (OutAbilities :type "Array of Ck_Ability_Script_PDA Class Reference"))
  ;[0 0.2031 1] Optionally Override in the Derived ConstructionScript
  (return))