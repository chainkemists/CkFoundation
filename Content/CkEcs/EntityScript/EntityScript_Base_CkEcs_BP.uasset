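; Base Blueprint for CkEcs entity scripts, supplying shared begin-play, handle lookup and thumbnail behavior.
; On begin play it notifies an optional listener interface, if valid, with the script entity's handle and class.
; GetHandleToUse returns the optional context handle when valid and otherwise falls back to the script's own entity.
; A thumbnail override supplies the EntityScript icon and a dark blue background color.
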(event `self.DoBeginPlay`
  (params (InHandle :type "Ck_Handle Structure"))
  (bind _returnvalue (`Ck_Utils_EntityScript_UE.DoCastChecked` (`self.DoGet_ScriptEntity`)))
  (bind _outinterface (`/CkFoundation/CkCore/FlowControl_CkCore_BPML.ValidateInterface` (`self.EntityScript_Listener (Optional)`))
    (:`IsValid`
      (`/CkFoundation/CkEcs/EntityScript/EntityScript_Base_CkEcs_BPI.OnSpawnedEntityScriptBeginPlay` _outinterface _returnvalue (`Ck_Utils_EntityScript_UE.Get_ScriptClass` _returnvalue)))))

(fn `Get_HandleToUse`
  (returns (OutHandle :type "Ck_Handle Structure"))
  (bind _outhandle (`/CkFoundation/CkEcs/EntityHandle_CkEcs_ML.ValidateEntityHandle` (`self.ContextHandle (Optional)`))
    (:`IsValid`
      (return _outhandle))
    (:`NotValid`
      (return (`self.DoGet_ScriptEntity`)))))

(fn `Get_ThumbnailIconAndColor`
  (returns (OutBackgroundColor :type "LinearColor Structure") (ReturnValue :type "Texture2D Object Reference"))
  (return (struct :`R` 0.028966 :`G` 0.081572 :`B` 0.109375 :`A` 1.0) "/CkFoundation/Textures/Icon_EntityScript_64px.Icon_EntityScript_64px"))