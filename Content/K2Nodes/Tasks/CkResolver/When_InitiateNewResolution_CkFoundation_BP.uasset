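; Blueprint task node that initiates a new resolution on a resolver source and reports its progress through callbacks.
; On activation it sends the request; the returned data bundle gets bindings for phase start, phase complete and all phases complete.
; Bindings use FireIfPayloadInFlightThisFrame, and each event is forwarded to the task's outputs.
; The task deactivates after all phases complete, unbinding its delegates if the bundle handle is valid.
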(event `self.Activate_BP`
  (`Ck_Utils_ResolverSource_UE.Request_InitiateNewResolution` (`self.InResolverSource`) (`self.InRequest`) (delegate `Event_OnNewResolverDataBundle`)))

(event `Event_OnNewResolverDataBundle`
  (params (InSource :type "Ck_Handle_ResolverSource Structure") (InCause :type "Ck_Handle Structure") (InDataBundle :type "Ck_Handle_ResolverDataBundle Structure"))
  (bind _output_get (set `self._DataBundle` InDataBundle))
  (bind _returnvalue (`Ck_Utils_ResolverDataBundle_UE.BindTo_OnPhaseStart` _output_get "FireIfPayloadInFlightThisFrame" "DoNothing" (delegate `Event_OnPhaseStart`)))
  (bind _returnvalue_2 (`Ck_Utils_ResolverDataBundle_UE.BindTo_OnPhaseComplete` _returnvalue "FireIfPayloadInFlightThisFrame" "DoNothing" (delegate `Event_OnPhaseComplete`)))
  (bind _returnvalue_3 (`Ck_Utils_ResolverDataBundle_UE.BindTo_OnAllPhasesComplete` _returnvalue_2 "FireIfPayloadInFlightThisFrame" "DoNothing" (delegate `Event_OnAllPhasesComplete`)))
  (`self.OnNewDataBundle` _returnvalue_3))

(event `Event_OnPhaseStart`
  (params (InDataBundle :type "Ck_Handle_ResolverDataBundle Structure") (InPhase :type "GameplayTag Structure"))
  (`self.OnPhaseStart` InDataBundle InPhase))

(event `Event_OnPhaseComplete`
  (params (InDataBundle :type "Ck_Handle_ResolverDataBundle Structure") (InPhase :type "GameplayTag Structure") (InPayload :type "Ck_Payload_ResolverDataBundle_Resolved Structure"))
  (`self.OnPhaseComplete` InDataBundle InPhase InPayload))

(event `Event_OnAllPhasesComplete`
  (params (InDataBundle :type "Ck_Handle_ResolverDataBundle Structure") (InPayload :type "Ck_Payload_ResolverDataBundle_Resolved Structure"))
  (`self.OnAllPhasesComplete` InDataBundle InPayload)
  (`self.Deactivate`))

(event `self.Deactivate_BP`
  (bind _outhandle (`/CkFoundation/CkEcs/EntityHandle_CkEcs_ML.ValidateEntityHandle` (`self._DataBundle`))
    (:`IsValid`
      (`Ck_Utils_ResolverSource_UE.UnbindFrom_OnNewResolverDataBundle` (`self.InResolverSource`) (delegate `Event_OnNewResolverDataBundle`))
      (bind _returnvalue (`Ck_Utils_ResolverDataBundle_UE.UnbindFrom_OnPhaseStart` _outhandle (delegate `Event_OnPhaseStart`)))
      (bind _returnvalue_2 (`Ck_Utils_ResolverDataBundle_UE.UnbindFrom_OnPhaseComplete` _returnvalue (delegate `Event_OnPhaseComplete`)))
      (`Ck_Utils_ResolverDataBundle_UE.UnbindFrom_OnAllPhasesComplete` _returnvalue_2 (delegate `Event_OnAllPhasesComplete`)))))