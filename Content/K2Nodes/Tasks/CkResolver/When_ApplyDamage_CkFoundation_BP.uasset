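; Blueprint task node that applies damage from an Instigator to a Target through the CkResolver system, failing if either is invalid.
; It runs the DefaultResolutions bundles in sequence, storing the HitResult on each new damage bundle.
; Each completed resolution's metadata and final value seed the next as tags and a BaseValue Add modifier.
; It broadcasts each phase completion, then the fully resolved damage once the chain ends.
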(event `self.Activate_BP`
  (`Ck_Utils_EcsEnsure_UE.EnsureMsgf_IsValid` (`self.Instigator`) (`|FormatText` self "Invalid Instigator passed to [{self}]")
    (:`Valid`
      (`Ck_Utils_EcsEnsure_UE.EnsureMsgf_IsValid` (`self.Target`) (`|FormatText` self "Invalid Target passed to [{self}]")
        (:`Valid`
          (`self.InitiateNewResolution` (`self.InitialMetadata`) (`self.InitialModifierOperations`)))
        (:`Invalid`
          (`self.OnFailed`)
          (`self.Deactivate`))))
    (:`Invalid`
      (`self.OnFailed`)
      (`self.Deactivate`))))

(event `InitiateNewResolution`
  (params (` Initial Metadata` :type "Array of Ck_ResolverDataBundle_MetadataOperation_Conditional Structure (by ref)") (` Initial Modifier Operations` :type "Array of Ck_ResolverDataBundle_ModifierOperation_Conditional Structure (by ref)"))
  (bind _output (`self.Get_NextResolution` ` Initial Metadata` ` Initial Modifier Operations`)
    (:`Valid`
      (bind (_taskobject _onnewdatabundle_indatabundle _onphasestart_indatabundle _onphasestart_inphase _onphasecomplete_indatabundle _onphasecomplete_inphase _onphasecomplete_inpayload _onallphasescomplete_indatabundle _onallphasescomplete_inpayload) (`|Blueprint_Template` (`self.Instigator`) _output :!label _label)
        (:`then`
          (`self.DoRequest_AddTaskToDeactivateOnDeactivate` _taskobject))
        (:`OnNewDataBundle`
          (`/CkFoundation/CkResolver/Damage_CkFoundation_FL.[Ck][Damage] Request_StoreHitResultOnDamageBundle` _onnewdatabundle_indatabundle (`self.HitResult`)))
        (:`OnPhaseComplete`
          (`self.Event_OnDamagePhaseComplete` _onphasecomplete_inphase _onphasecomplete_inpayload))
        (:`OnAllPhasesComplete`
          (`|ExecutionSequence`
            (:`then_0`
              (goto _label :!via `Deactivate`))
            (:`then_1`
              (if (`KismetArrayLibrary.Array_IsValidIndex` (`self._DefaultResolutions`) (`self._NextResolution`))
                (bind (_outmetadata _outmodifieroperations) (`self.Convert_PayLoadToOperations` _onallphasescomplete_inpayload))
                (`self.InitiateNewResolution` _outmetadata _outmodifieroperations)
                (else
                  (`self.Event_OnDamageFullyResolved` _onallphasescomplete_inpayload))))))))))

(event `Event_OnDamagePhaseComplete`
  (params (InPhase :type "GameplayTag Structure") (InResolvedPayload :type "Ck_Payload_ResolverDataBundle_Resolved Structure"))
  (`self.OnDamagePhaseComplete` InPhase InResolvedPayload (`self.HitResult`)))

(event `Event_OnDamageFullyResolved`
  (params (InResolvedPayload :type "Ck_Payload_ResolverDataBundle_Resolved Structure"))
  (`self.OnDamageFullyResolved` InResolvedPayload (`self.HitResult`)))

(fn `Convert_PayLoadToOperations`
  (params (InPayload :type "Ck_Payload_ResolverDataBundle_Resolved Structure (by ref)"))
  (returns (OutMetadata :type "Array of Ck_ResolverDataBundle_MetadataOperation_Conditional Structure") (OutModifierOperations :type "Array of Ck_ResolverDataBundle_ModifierOperation_Conditional Structure"))
  (bind (__databundle __instigator __target __resolvercause __causer __finalvalue __metadata) (break `Ck_Payload_ResolverDataBundle_Resolved` InPayload))
  (return (`|MakeArray` (make `Ck_ResolverDataBundle_MetadataOperation_Conditional` (struct :`RequireTags` (struct) :`IgnoreTags` (struct) :`TagQuery` (struct)) (make `Ck_ResolverDataBundle_MetadataOperation` __metadata))) (`|MakeArray` (make `Ck_ResolverDataBundle_ModifierOperation_Conditional` (struct :`RequireTags` (struct) :`IgnoreTags` (struct) :`TagQuery` (struct)) (make `Ck_ResolverDataBundle_ModifierOperation` "BaseValue" "Add" __finalvalue)))))

(fn `Get_DefaultResolutions`
  (returns (_Resolutions :type "Array of GameplayTag Structure"))
  (return (`self._DefaultResolutions`)))

(fn `Get_NextResolution`
  (params (` Initial Metadata` :type "Array of Ck_ResolverDataBundle_MetadataOperation_Conditional Structure") (` Initial Modifier Operations` :type "Array of Ck_ResolverDataBundle_ModifierOperation_Conditional Structure"))
  (returns (Output :type "Ck_Request_ResolverSource_InitiateNewResolution Structure (by ref)") (OutValidOrNot :type "ECk_ValidInvalid Enum"))
  (locals (L_InitialMetadata :type "Array of Ck_ResolverDataBundle_MetadataOperation_Conditional Structure") (L_InitialModifierOperations :type "Array of Ck_ResolverDataBundle_ModifierOperation_Conditional Structure"))
  (bind _output (`/CkFoundation/CkCore/Container/Container_CkCore_ML.Array_GetValidatedIndex` (`self._DefaultResolutions`) (`self._NextResolution`))
    (:`IsValid`
      (`/Engine/EditorBlueprintResources/StandardMacros.IncrementInt` (`self._NextResolution`)
        (:`  `
          (bind _ck_request_resolversource_initiatenewresolution (make `Ck_Request_ResolverSource_InitiateNewResolution` _output (`self.Target`) (`self.Causer`) ` Initial Metadata` ` Initial Modifier Operations`))
          (return _ck_request_resolversource_initiatenewresolution "Valid"))))
    (:`NotValid`
      (return _ck_request_resolversource_initiatenewresolution "Invalid"))))

(fn `Get_NodeDescription_BP`
  (returns (ReturnValue :type String))
  (locals (L_Description :type "Array of String"))
  (for _array_element (`self._DefaultResolutions`)
    (`KismetArrayLibrary.Array_Add` (`local.L_Description`) (`/CkFoundation/CkCore/Debug/Utils_Debug_CkCore_FL.[Ck] Get_GameplayTag_DebugString` _array_element)))
  (return (`KismetStringLibrary.JoinStringArray` (`local.L_Description`) " \n")))