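; Blueprint async task node that waits for new resolver data bundles on a resolver target and relays their progress through its output events.
; On activation it listens for new bundles, stores each one, binds to its phase-complete and all-phases-complete events, then reports the bundle.
; Bindings also fire for payloads already in flight that frame.
; Deactivation unbinds from the target and from only the last stored bundle, if still valid.
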(event `self.Activate_BP`
  (`parent.Activate_BP`)
  (`Ck_Utils_ResolverTarget_UE.BindTo_OnNewResolverDataBundle` (`self.InResolverTarget`) "FireIfPayloadInFlightThisFrame" "DoNothing" (delegate `Event_OnNewResolverDataBundle`)))

(event `Event_OnNewResolverDataBundle`
  (params (InTarget :type "Ck_Handle_ResolverTarget Structure") (InDataBundle :type "Ck_Handle_ResolverDataBundle Structure"))
  (bind _output_get (set `self._DataBundle` InDataBundle))
  (bind _returnvalue (`Ck_Utils_ResolverDataBundle_UE.BindTo_OnPhaseComplete` _output_get "FireIfPayloadInFlightThisFrame" "DoNothing" (delegate `Event_OnPhaseComplete`)))
  (bind _returnvalue_2 (`Ck_Utils_ResolverDataBundle_UE.BindTo_OnAllPhasesComplete` _returnvalue "FireIfPayloadInFlightThisFrame" "DoNothing" (delegate `Event_OnAllPhasesComplete`)))
  (`self.OnNewDataBundle` _returnvalue_2))

(event `Event_OnPhaseComplete`
  (params (InDataBundle :type "Ck_Handle_ResolverDataBundle Structure") (InPhase :type "GameplayTag Structure") (InPayload :type "Ck_Payload_ResolverDataBundle_Resolved Structure"))
  (`self.OnPhaseComplete` InDataBundle InPhase InPayload))

(event `Event_OnAllPhasesComplete`
  (params (InDataBundle :type "Ck_Handle_ResolverDataBundle Structure") (InPayload :type "Ck_Payload_ResolverDataBundle_Resolved Structure"))
  (`self.OnAllPhasesComplete` InDataBundle InPayload))

(event `self.Deactivate_BP`
  (`parent.Deactivate_BP`)
  (`Ck_Utils_ResolverTarget_UE.UnbindFrom_OnNewResolverDataBundle` (`self.InResolverTarget`) (delegate `Event_OnNewResolverDataBundle`))
  (bind _outhandle (`/CkFoundation/CkEcs/EntityHandle_CkEcs_ML.ValidateEntityHandle` (`self._DataBundle`))
    (:`IsValid`
      (bind _returnvalue (`Ck_Utils_ResolverDataBundle_UE.UnbindFrom_OnPhaseComplete` _outhandle (delegate `Event_OnPhaseComplete`)))
      (`Ck_Utils_ResolverDataBundle_UE.UnbindFrom_OnAllPhasesComplete` _returnvalue (delegate `Event_OnAllPhasesComplete`)))))