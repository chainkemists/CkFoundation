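; Blueprint task that waits for new aggro to be added to an AggroOwner entity in the Ck aggro system.
; On activation it binds to the owner's new-aggro event, also firing for payloads already in flight that frame, and relays owner and new aggro through its NewAggroAdded output.
; Deactivation unbinds the listener.
; The status string shows the owner entity, or flags it as invalid.
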(event `self.Activate_BP`
  (`parent.Activate_BP`)
  (`Ck_Utils_AggroOwner_UE.BindTo_OnNewAggroAdded` (`self.AggroOwner`) "FireIfPayloadInFlightThisFrame" "DoNothing" (delegate `OnNewAggroAdded`)))

(event `OnNewAggroAdded`
  (params (InAggroOwner :type "Ck_Handle_AggroOwner Structure") (InNewAggro :type "Ck_Handle_Aggro Structure"))
  (`self.NewAggroAdded` InAggroOwner InNewAggro))

(event `self.Deactivate_BP`
  (`parent.Deactivate_BP`)
  (`Ck_Utils_AggroOwner_UE.UnbindFrom_OnNewAggroAdded` (`self.AggroOwner`) (`|CreateDelegate` :!event `OnNewAggroAdded`)))

(fn `Get_StatusString_BP`
  (returns (ReturnValue :type String))
  (`/CkFoundation/CkEcs/EntityHandle_CkEcs_ML.ValidateEntityHandle` (`self.AggroOwner`)
    (:`IsValid`
      (return (`Ck_Utils_Handle_UE.Conv_HandleToString` (`self.AggroOwner`))))
    (:`NotValid`
      (return "Invalid AggroOwner Entity"))))