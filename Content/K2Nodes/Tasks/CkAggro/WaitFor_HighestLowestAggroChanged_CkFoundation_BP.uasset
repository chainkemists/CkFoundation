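; Blueprint task that watches an aggro owner and fires delegates whenever its highest or lowest aggro changes.
; On activation it starts a score-attribute listener task for each existing and newly added aggro, each set to deactivate with the parent task.
; Activation, listener startup and score changes re-sort the aggros, broadcasting only when an end entry differs from the cached handle.
; Deactivation unbinds the new-aggro event.
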(event `self.Activate_BP`
  (`parent.Activate_BP`)
  (`Ck_Utils_Aggro_UE.BindTo_OnNewAggroAdded` (`self.AggroOwner`) "FireIfPayloadInFlightThisFrame" "DoNothing" (delegate `OnNewAggroAdded`))
  (bind _returnvalue (`Ck_Utils_Aggro_UE.ForEach_Aggro` (`self.AggroOwner`)))
  (for _array_element _returnvalue
    (`self.ListenForAggroScoreUpdated` _array_element))
  (`self.BroadcastDelegates`))

(event `ListenForAggroScoreUpdated`
  (params (InAggroHandle :type "Ck_Handle_Aggro Structure"))
  ;[1 0 0.2578] ListenForAggroScoreUpdated
  (bind _taskobject (`|Blueprint_Template` (`Ck_Utils_Handle_UE.Get_RawHandle` InAggroHandle) (struct :`TagName` "FloatAttribute.Aggro.Score"))
    (:`then`
      (`self.DoRequest_AddTaskToDeactivateOnDeactivate` _taskobject)
      (`self.BroadcastDelegates`))
    (:`AttributeChanged`
      (`self.BroadcastDelegates`))))

(event `OnNewAggroAdded`
  (params (InAggroOwner :type "Ck_Handle Structure") (InNewAggro :type "Ck_Handle_Aggro Structure"))
  (`self.ListenForAggroScoreUpdated` InNewAggro))

(event `BroadcastDelegates`
  ;[1 0.3047 0] BroadcastDelegates
  (bind _returnvalue (`Ck_Utils_Aggro_UE.ForEach_Aggro_Sorted` (`self.AggroOwner`) (struct) "SmallestToLargest"))
  (`|ExecutionSequence`
    (:`then_0`
      (bind _output (`/CkFoundation/CkCore/Container/Container_CkCore_ML.Array_GetFirstElementValidated` _returnvalue)
        (:`IsValid`
          (bind _outhandle (`/CkFoundation/CkEcs/EntityHandle_CkEcs_ML.ValidateEntityHandle` _output)
            (:`IsValid`
              (if (`Ck_Utils_Handle_UE.IsNotEqual` _outhandle (`self._CurrentLowestAggro`))
                (bind _output_get (set `self._CurrentLowestAggro` _outhandle))
                (`self.NewLowestAggro` _output_get)))))))
    (:`then_1`
      (bind _output_2 (`/CkFoundation/CkCore/Container/Container_CkCore_ML.Array_GetLastElementValidated` _returnvalue)
        (:`IsValid`
          (bind _outhandle_2 (`/CkFoundation/CkEcs/EntityHandle_CkEcs_ML.ValidateEntityHandle` _output_2)
            (:`IsValid`
              (if (`Ck_Utils_Handle_UE.IsNotEqual` _outhandle_2 (`self._CurrentHighestAggro`))
                (bind _output_get_2 (set `self._CurrentHighestAggro` _outhandle_2))
                (`self.NewHighestAggro` _output_get_2)))))))))

(event `self.Deactivate_BP`
  (`parent.Deactivate_BP`)
  (`Ck_Utils_Aggro_UE.UnbindFrom_OnNewAggroAdded` (`self.AggroOwner`) (`|CreateDelegate` :!event `OnNewAggroAdded`)))