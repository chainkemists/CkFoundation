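; WaitFor_AggroChanged_BP is a latent task node in CkAggro that waits for aggro changes on an aggro owner entity.
; On activation it binds to the owner's OnAggroChanged signal, also firing for a payload already in flight, and unbinds on deactivation.
; Each change is re-broadcast through the task's OnAggroChanged output with the owner, previous and new aggro.
; Its status string shows the owner entity, or flags it as invalid.
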(event `self.Activate_BP`
  (`parent.Activate_BP`)
  (`Ck_Utils_AggroOwner_UE.BindTo_OnAggroChanged` (`self.AggroOwner`) "FireIfPayloadInFlight" "DoNothing" (delegate `Event_OnAggroChanged`)))

(event `Event_OnAggroChanged`
  (params (InAggroOwner :type "Ck_Handle_AggroOwner Structure") (InPrevAggro :type "Ck_Handle_Aggro Structure") (InNewAggro :type "Ck_Handle_Aggro Structure"))
  (`self.OnAggroChanged` InAggroOwner InPrevAggro InNewAggro))

(event `self.Deactivate_BP`
  (`parent.Deactivate_BP`)
  (`Ck_Utils_AggroOwner_UE.UnbindFrom_OnAggroChanged` (`self.AggroOwner`) (delegate `Event_OnAggroChanged`)))

(fn `Get_StatusString_BP`
  (returns (ReturnValue :type String))
  (`/CkFoundation/CkEcs/EntityHandle_CkEcs_ML.ValidateEntityHandle` (`self.AggroOwner`)
    (:`IsValid`
      (return (`Ck_Utils_Handle_UE.Conv_HandleToString` (`self.AggroOwner`))))
    (:`NotValid`
      (return "Invalid AggroOwner Entity"))))