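; Latent CkFoundation task that repeatedly rotates an entity's owning actor toward a target entity, deactivating if the entity check fails.
; A looping timer at TickRate applies a look-at rotation and broadcasts each update.
; The look-at is recomputed only for pawns, whose controller-rotation flags are overridden while active and restored on deactivation.
; The yaw, pitch and roll overrides all read the yaw setting.
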(event `self.Activate_BP`
  (`parent.Activate_BP`)
  (bind _output_get (set `self.EntityActor` (`Ck_Utils_OwningActor_UE.Get_EntityOwningActor` (`self.EntityWithActorOrPawn`))))
  (bind _aspawn (cast `Pawn` _output_get)
    (:`then`
      (bind _output_get_2 (set `self.MaybePawn` _aspawn))
      (`self.DoStoreControllerRotations` _output_get_2))
    (:`CastFailed`
      _))
  (`Ck_Utils_Ensure_UE.EnsureMsgf` (`Ck_Utils_AbilityOwner_UE.Has` (`self.EntityWithActorOrPawn`)) (`|FormatText` "Unable to RotateTorwards since Handle [{handle}] does NOT have an Owning Actor" (`Ck_Utils_Handle_UE.Conv_HandleToString` (`self.EntityWithActorOrPawn`)))
    (:`Valid`
      (bind _taskobject (`|Blueprint_Template` (`self.TickRate`) "NewEnumerator1" true)
        (:`then`
          (`self.DoRequest_AddTaskToDeactivateOnDeactivate` _taskobject))
        (:`OnTimerEvent`
          (bind _maybepawn (`self.MaybePawn`)
            (:`then`
              (`self.DoSetControllerRotation_Yaw` _maybepawn)
              (`self.DoSetControllerRotation_Pitch` _maybepawn)
              (`self.DoSetControllerRotation_Roll` _maybepawn)
              (bind _output_get_3 (set `self.NewLookAtRotation` (`KismetMathLibrary.FindLookAtRotation` (`Ck_Utils_Transform_UE.Get_EntityCurrentLocation` (`Ck_Utils_Transform_UE.DoCastChecked` (`self.EntityWithActorOrPawn`))) (`Ck_Utils_Transform_UE.Get_EntityCurrentLocation` (`Ck_Utils_Transform_UE.DoCastChecked` (`self.TargetEntity`)))))))
            (:`else`
              _))
          (`Actor.K2_SetActorRotation` (`self.EntityActor`) _output_get_3 false)
          (`self.OnUpdateRotation` (`self.EntityWithActorOrPawn`) (`self.TargetEntity`) (`self.NewLookAtRotation`)))))
    (:`Invalid`
      (`self.Deactivate`))))

(event `self.Deactivate_BP`
  (`parent.Deactivate_BP`)
  (bind _entityactor (`self.EntityActor`)
    (:`then`
      (bind _aspawn (cast `Pawn` _entityactor))
      (`self.DoRestoreStoreControllerRotations` _aspawn))
    (:`else`)))

(fn `DoRestoreStoreControllerRotations`
  (params (InPawn :type "Pawn Object Reference"))
  (set `Pawn.bUseControllerRotationYaw` (`self.Prev_ControllerRotation_Yaw`) InPawn)
  (set `Pawn.bUseControllerRotationPitch` (`self.Prev_ControllerRotation_Pitch`) InPawn)
  (set `Pawn.bUseControllerRotationRoll` (`self.Prev_ControllerRotation_Roll`) InPawn))

(fn `DoSetControllerRotation_Pitch`
  (params (InPawn :type "Pawn Object Reference"))
  (switch `ECk_EnableDisable` (`self.ControllerRotation_Yaw`)
    (:`Enable`
      (set `Pawn.bUseControllerRotationPitch` true InPawn))
    (:`Disable`
      (set `Pawn.bUseControllerRotationPitch` false InPawn))))

(fn `DoSetControllerRotation_Roll`
  (params (InPawn :type "Pawn Object Reference"))
  (switch `ECk_EnableDisable` (`self.ControllerRotation_Yaw`)
    (:`Enable`
      (set `Pawn.bUseControllerRotationRoll` true InPawn))
    (:`Disable`
      (set `Pawn.bUseControllerRotationRoll` false InPawn))))

(fn `DoSetControllerRotation_Yaw`
  (params (InPawn :type "Pawn Object Reference"))
  (switch `ECk_EnableDisable` (`self.ControllerRotation_Yaw`)
    (:`Enable`
      (set `Pawn.bUseControllerRotationYaw` true InPawn))
    (:`Disable`
      (set `Pawn.bUseControllerRotationYaw` false InPawn))))

(fn `DoStoreControllerRotations`
  (params (InPawn :type "Pawn Object Reference"))
  (set `self.Prev_ControllerRotation_Yaw` (`Pawn.bUseControllerRotationYaw` InPawn))
  (set `self.Prev_ControllerRotation_Pitch` (`Pawn.bUseControllerRotationPitch` InPawn))
  (set `self.Prev_ControllerRotation_Roll` (`Pawn.bUseControllerRotationRoll` InPawn)))