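; A Blueprint task that requests a replicated actor spawn through the CkFoundation actor modifier and waits for the result.
; On activation it forwards its owner or world, class, transform, collision handling, names, labels and optional payload to the spawn request.
; When the spawn callback fires, it passes the spawned actor and payload to OnActorSpawned and deactivates itself, making it a one-shot latent wrapper.
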(event `self.Activate_BP`
  (`parent.Activate_BP`)
  (`/CkFoundation/CkActor/Utils_CkActor_FL.[Ck][ActorModifier] Request Spawn Actor (Replicated)` (`self.OwnerOrWorld`) (`self.ActorClass`) (`self.SpawnTransform`) (`self.CollisionHandling`) (`self.OptionalPayload`) (delegate `ActorSpawned`) (`self.NonUniqueName`) (`self.EditorOnlyLabel`)))

(event `ActorSpawned`
  (params (InActorSpawned :type "Actor Object Reference") (InOptionalPayload :type "InstancedStruct Structure (by ref)"))
  (`self.OnActorSpawned` InActorSpawned InOptionalPayload)
  (`self.Deactivate`))