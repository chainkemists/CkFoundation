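; TaskForge node that moves an entity's owning actor in a straight line toward a goal target entity at a set speed.
; On activation it validates inputs, caches either side as a Character, and starts a looping timer.
; Each tick re-reads both locations, applies Character-based offsets, and sets actor location without sweep, clamping the step at the acceptance radius.
; It broadcasts each location update, then signals goal reached and deactivates.
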(event `self.Activate_BP`
  (`parent.Activate_BP`)
  (`Ck_Utils_Ensure_UE.EnsureMsgf` (`/CkFoundation/CkCore/Math/Math_CkCore_ML.>0 (float)` (`self.MovementSpeed`)) (`|FormatText` self "Unable to perform [{self}] since the MovementSpeed is [{speed}]" (`self.MovementSpeed`))
    (:`Valid`
      (`Ck_Utils_Ensure_UE.EnsureMsgf` (`Ck_Utils_OwningActor_UE.Has` (`self.EntityWithActor`)) (`|FormatText` self "Unable to perform [{self}] since Handle [{handle}] does NOT have an Owning Actor" (`Ck_Utils_Handle_UE.Conv_HandleToString` (`self.EntityWithActor`)))
        (:`Valid`
          (bind _output_get (set `self._EntityActor` (`Ck_Utils_OwningActor_UE.Get_EntityOwningActor` (`self.EntityWithActor`))))
          (bind _ascharacter (cast `Character` _output_get)
            (:`then`
              (set `self._MaybeEntityAsCharacter` _ascharacter))
            (:`CastFailed`
              _))
          (`Ck_Utils_Ensure_UE.EnsureMsgf_IsValid` (`self._EntityActor`) (`|FormatText` self "Unable to perform [{self}] since Handle [{handle}] does NOT have a valid OwningActor" (`Ck_Utils_Handle_UE.Conv_HandleToString` (`self.EntityWithActor`)))
            (:`Valid`
              (`Ck_Utils_EcsEnsure_UE.EnsureMsgf_IsValid` (`self.GoalTargetPoint`) (`|FormatText` self "Unable to perform [{self}] since the GoalTargetPoint is INVALID")
                (:`Valid`
                  (if (`Ck_Utils_OwningActor_UE.Has` (`self.GoalTargetPoint`))
                    (bind _ascharacter_2 (cast `Character` (`Ck_Utils_OwningActor_UE.Get_EntityOwningActor` (`self.GoalTargetPoint`)))
                      (:`then`
                        (set `self._MaybeGoalTargetAsCharacter` _ascharacter_2))
                      (:`CastFailed`
                        _)))
                  (bind (_taskobject _ontimerstarted_outtimerentity _ontimerevent_outtimerentity _ontimerevent_outtimerchrono _ontimerevent_outdeltat) (`|TaskForge_K2Node` (struct :`TagName` "Timer.Actor.MoveTo") (`self.TickRate`) "NewEnumerator1" true)
                    (:`OnTimerEvent`
                      (`self.DoPerformMoveTo` (`Ck_Utils_Time_UE.Make_FromSeconds` _ontimerevent_outdeltat)))))
                (:`Invalid`
                  (`self.Deactivate`))))
            (:`Invalid`
              (`self.Deactivate`))))
        (:`Invalid`
          (`self.Deactivate`))))
    (:`Invalid`
      (`self.Deactivate`))))

(event `self.Deactivate_BP`
  (`parent.Deactivate_BP`))

(fn `DoGet_IsWithinAcceptanceRadius`
  (params (V1 :type "Vector Structure") (V2 :type "Vector Structure"))
  (returns (OutIsWithinAcceptanceRadius :type Boolean) (Distance :type "Float (double-precision)"))
  (locals (L_DistanceToGoal :type "Float (double-precision)" :default 0.0))
  (bind _output_get (set `local.L_DistanceToGoal` (`KismetMathLibrary.Vector_Distance` V1 V2)))
  (return (<= (`local.L_DistanceToGoal`) (`self.AcceptanceRadius`)) _output_get))

(fn `DoPerformMoveTo`
  (params (InDeltaT :type "Ck_Time Structure"))
  (locals (L_MaxDistanceToMove :type "Float (double-precision)") (L_EntityCurrentLoc :type "Vector Structure" :default (0.0 0.0 0.0)) (L_GoalCurrentLoc :type "Vector Structure" :default (0.0 0.0 0.0)) (L_DistanceToGoal :type "Float (double-precision)" :default 0.0) (L_DistanceToGoal_MinusAcceptanceRadius :type "Float (double-precision)") (L_MoveToLocation :type "Vector Structure" :default (0.0 0.0 0.0)))
  (bind _returnvalue__direction (break `Ck_DirectionAndLength` (`Ck_Utils_Vector3_UE.Get_DirectionAndLengthBetweenVectors` (`local.L_GoalCurrentLoc`) (`local.L_EntityCurrentLoc`))))
  (`|ExecutionSequence`
    (:`then_0`
      (set `local.L_MaxDistanceToMove` (* (`._Seconds` (break `Ck_Time` (`local.InDeltaT`))) (`self.MovementSpeed`)))
      (set `local.L_EntityCurrentLoc` (`Ck_Utils_Transform_UE.Get_EntityCurrentLocation` (`Ck_Utils_Transform_UE.DoCastChecked` (`self.EntityWithActor`))))
      (set `local.L_GoalCurrentLoc` (`Ck_Utils_Transform_UE.Get_EntityCurrentLocation` (`self.GoalTargetPoint`))))
    (:`then_1`
      (bind __maybeentityascharacter (`self._MaybeEntityAsCharacter`)
        (:`then`
          (set `local.L_EntityCurrentLoc` (- __maybeentityascharacter (`local.L_EntityCurrentLoc`))))
        (:`else`)))
    (:`then_2`
      (bind __maybegoaltargetascharacter (`self._MaybeGoalTargetAsCharacter`)
        (:`then`
          (set `local.L_GoalCurrentLoc` (- __maybegoaltargetascharacter (`local.L_GoalCurrentLoc`))))
        (:`else`)))
    (:`then_3`
      (if (`self.DoGet_IsWithinAcceptanceRadius` (`local.L_EntityCurrentLoc`) (`local.L_GoalCurrentLoc`))
        (`self.OnReachedGoal` (`self.EntityWithActor`) (`self.GoalTargetPoint`) :!label _label)
        (`self.Deactivate`)
        (return)
        (else
          (bind _output_get (set `local.L_DistanceToGoal` (`KismetMathLibrary.Vector_Distance` (`local.L_EntityCurrentLoc`) (`local.L_GoalCurrentLoc`))))
          (bind _output_get_2 (set `local.L_DistanceToGoal_MinusAcceptanceRadius` (- _output_get (`self.AcceptanceRadius`))))
          (if (`KismetMathLibrary.NearlyEqual_FloatFloat` _output_get_2 0.0 1.0)
            (goto _label)
            (else
              (set `local.L_MoveToLocation` (`Ck_Utils_Vector3_UE.Get_LocationFromOriginInDirection` (`local.L_EntityCurrentLoc`) _returnvalue__direction (`KismetMathLibrary.FMin` (`local.L_MaxDistanceToMove`) (`local.L_DistanceToGoal_MinusAcceptanceRadius`))))
              (bind __maybeentityascharacter_2 (`self._MaybeEntityAsCharacter`)
                (:`then`
                  (set `local.L_MoveToLocation` (+ __maybeentityascharacter_2 (`local.L_MoveToLocation`)))
                  (set `local.L_GoalCurrentLoc` (+ __maybeentityascharacter_2 (`local.L_GoalCurrentLoc`))))
                (:`else`
                  _))
              (`Actor.K2_SetActorLocation` (`self._EntityActor`) (`local.L_MoveToLocation`) false false)
              (`self.OnUpdateLocation` (`self.EntityWithActor`) (`self.GoalTargetPoint`) (`local.L_MoveToLocation`))
              (if (`self.DoGet_IsWithinAcceptanceRadius` (`local.L_MoveToLocation`) (`local.L_GoalCurrentLoc`))
                (`self.OnReachedGoal` (`self.EntityWithActor`) (`self.GoalTargetPoint`))
                (`self.Deactivate`)
                (else
                  (return))))))))))