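; Latent task Blueprint node from CkFoundation that requests adding an actor component and waits until it has been added.
; On activation it sends a CkActorModifier add-component request with the component, parent, attachment socket and type, uniqueness and optional payload.
; When the added callback fires, it forwards the owner, new component and payload to its output delegate, then deactivates itself.
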(event `self.Activate_BP`
  (`parent.Activate_BP`)
  (`/CkFoundation/CkActor/Utils_CkActor_FL.[Ck][ActorModifier] Request Add Actor Component` (`self.ComponentToAdd`) (`self.ParentComponent`) (`self.OptionalPayload`) (delegate `ComponentAdded`) (`self.IsUnique`) (`self.AttachmentSocket`) (`self.AttachmentType`)))

(event `ComponentAdded`
  (params (InOwner :type "Actor Object Reference") (InActorComponentAdded :type "ActorComponent Object Reference") (InOptionalPayload :type "InstancedStruct Structure (by ref)"))
  (`self.OnComponentAdded` InOwner InActorComponentAdded InOptionalPayload)
  (`self.Deactivate`))