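; Task node that reports movement mode changes on the Character that owns a given Entity.
; On activation it uses ensures to validate the Entity's owning Actor, Character cast and CharacterMovement component, then binds to the movement-mode-changed delegate and immediately outputs the current modes.
; Each change event forwards current and previous standard and custom modes with the Entity and Character.
; Deactivation unbinds the delegate if the Character is still valid.
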(event `self.Deactivate_BP`
  (`parent.Deactivate_BP`)
  (`/Engine/EditorBlueprintResources/StandardMacros.IsValid` (`self._Character`)
    (:`Is Valid`
      (remove `Character.MovementModeChangedDelegate` (`self._Character`) (delegate `Event_OnMovementModeChanged`)))))

(event `Event_OnMovementModeChanged`
  (params (Character :type "Character Object Reference") (PrevMovementMode :type "EMovementMode Enum" :default "MOVE_None") (PreviousCustomMode :type Byte))
  (bind _charactermovement (`Character.CharacterMovement` Character))
  (`self.OnMovementModeChanged` (`self.EntityWithActorMovementComponent`) Character (`CharacterMovementComponent.MovementMode` _charactermovement) (`CharacterMovementComponent.CustomMovementMode` _charactermovement) PrevMovementMode PreviousCustomMode))

(event `self.Activate_BP`
  (bind _entitywithactormovementcomponent (`self.EntityWithActorMovementComponent`))
  (`parent.Activate_BP`)
  (`Ck_Utils_Ensure_UE.EnsureMsgf` (`Ck_Utils_OwningActor_UE.Has` _entitywithactormovementcomponent) (`|FormatText` "Unable to Bind to MovementMode of Entity [{Entity}] since it does NOT have an Actor" (`KismetTextLibrary.Conv_TextToString` (`Ck_Utils_Handle_UE.Conv_HandleToText` (`self.EntityWithActorMovementComponent`))))
    (:`Valid`
      (bind _ascharacter (cast `Character` (`Ck_Utils_OwningActor_UE.Get_EntityOwningActor` _entitywithactormovementcomponent))
        (:`then`
          (bind _output_get (set `self._Character` _ascharacter))
          (`Ck_Utils_Ensure_UE.EnsureMsgf_IsValid` (`Character.CharacterMovement` (`self._Character`)) (`|FormatText` "Unable to Bind to MovementMode of Entity [{Entity}] with Actor [{Actor}] since the Actor, which is a Character, does NOT have a CharacterMovement component" (`Ck_Utils_Handle_UE.Conv_HandleToText` (`self.EntityWithActorMovementComponent`)) (`self._Character`))
            (:`Valid`
              (add `Character.MovementModeChangedDelegate` _output_get (delegate `Event_OnMovementModeChanged`))
              (`self.Exec` (`self.EntityWithActorMovementComponent`) (`self._Character`) (`CharacterMovementComponent.MovementMode` (`Character.CharacterMovement` (`self._Character`))) (`CharacterMovementComponent.CustomMovementMode` (`Character.CharacterMovement` (`self._Character`)))))))
        (:`CastFailed`
          (`Ck_Utils_Ensure_UE.TriggerEnsure` (`|FormatText` "Unable to Bind to MovementMode of Entity [{Entity}] with Actor [{Actor}] since the Actor is NOT a " (`Ck_Utils_Handle_UE.Conv_HandleToText` (`self.EntityWithActorMovementComponent`)) (`self._Character`))))))))