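; Task Blueprint that notifies when a supplied Actor has begun play.
; On activation in game, it ensures the Actor is valid, then polls once per tick through a gate until HasBegunPlay is true.
; It then fires OnActorBegunPlay with that Actor and deactivates itself, or just deactivates if the Actor is or becomes invalid.
; Deactivation closes the gate, which stops any pending polling.
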(event `self.Activate_BP`
  (`parent.Activate_BP`)
  (if (`Ck_Utils_Game_UE.Get_IsInGame` false)
    (`Ck_Utils_Ensure_UE.EnsureMsgf_IsValid` (`self.Actor`) (`|FormatText` self "Invalid Actor supplied to [{self}]")
      (:`Valid`
        (`/Engine/EditorBlueprintResources/StandardMacros.Gate` false :!label _label
          (:`Exit`
            (bind _actor (`self.Actor`)
              (:`then`
                (if (`Ck_Utils_Actor_UE.Get_HasBegunPlay` _actor)
                  (`self.OnActorBegunPlay` (`self.Actor`))
                  (`self.Deactivate`)
                  (else
                    (`KismetSystemLibrary.DelayUntilNextTick`)
                    (goto _label))))
              (:`else`
                (`self.Deactivate`))))))
      (:`Invalid`
        (`self.Deactivate`)))))

(event `self.Deactivate_BP`
  (`parent.Deactivate_BP`)
  (goto _label :!via `Close`))