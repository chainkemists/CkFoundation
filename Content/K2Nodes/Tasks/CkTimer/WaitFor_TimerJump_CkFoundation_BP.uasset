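; Latent task node that waits for a CkFoundation Timer entity to jump and reports it to the calling graph.
; On activation it ensures the Timer handle is valid, then binds to the timer's OnJump with a configurable binding policy.
; Each jump forwards the handle, chrono, delta time, direction and amount through CallTimerJump.
; On deactivation it unbinds if the handle is still valid.
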(event `self.Activate_BP`
  (`parent.Activate_BP`)
  (`Ck_Utils_Ensure_UE.EnsureMsgf` (`Ck_Utils_Handle_UE.Get_IsValid` (`self.TimerEntity`)) (`|FormatText` self "Invalid Timer handle supplied to [{self}]")
    (:`Valid`
      (`Ck_Utils_Timer_UE.BindTo_OnJump` (`self.TimerEntity`) (`self.BindingPolicy`) (`|CreateDelegate` :!event `OnTimerJump`)))))

(event `OnTimerJump`
  (params (InHandle :type "Ck_Handle_Timer Structure") (InChrono :type "Ck_Chrono Structure") (InDeltaT :type "Ck_Time Structure") (InJumpDirection :type "ECk_Timer_JumpDirection Enum" :default "Forwards") (InJumpAmount :type "Ck_Time Structure"))
  (`self.TimerJump` InHandle InChrono InDeltaT InJumpDirection InJumpAmount))

(event `self.Deactivate_BP`
  (`parent.Deactivate_BP`)
  (`/CkFoundation/CkEcs/EntityHandle_CkEcs_ML.ValidateEntityHandle` (`self.TimerEntity`)
    (:`IsValid`
      (`Ck_Utils_Timer_UE.UnbindFrom_OnJump` (`self.TimerEntity`) (`|CreateDelegate` :!event `OnTimerJump`)))))