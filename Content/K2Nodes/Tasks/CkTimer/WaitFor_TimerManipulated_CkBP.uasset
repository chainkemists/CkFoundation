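; Async task node that waits for a chosen manipulation (reset, complete, stop, pause or resume) of a Ck timer entity.
; On activation it binds to the matching timer delegate using the configured binding policy, and each handler forwards the timer entity and chrono through a single OnTimerManipulated output.
; On deactivation it unbinds that delegate, provided the timer entity handle is still valid.
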(event `OnTimerDone`
  (params (InHandle :type "Ck_Handle Structure") (InChrono :type "Ck_Chrono Structure"))
  ;[1 0 0.1875] Timer Events
  (`self.OnTimerManipulated` InHandle InChrono))

(event `self.Activate_BP`
  ;[1 0 0.8906] Activate
  (`parent.Activate_BP`)
  (switch `ECk_Timer_Manipulate` (`self.TimerManipulation`)
    (:`Reset`
      (`Ck_Utils_Timer_UE.BindTo_OnTimerReset` (`self.TimerEntity`) (`self.BindingPolicy`) (`|CreateDelegate` :!event `OnTimerReset`)))
    (:`Complete`
      (`Ck_Utils_Timer_UE.BindTo_OnTimerDone` (`self.TimerEntity`) (`self.BindingPolicy`) (`|CreateDelegate` :!event `OnTimerDone`)))
    (:`Stop`
      (`Ck_Utils_Timer_UE.BindTo_OnTimerStop` (`self.TimerEntity`) (`self.BindingPolicy`) (`|CreateDelegate` :!event `OnTimerStop`)))
    (:`Pause`
      (`Ck_Utils_Timer_UE.BindTo_OnTimerPause` (`self.TimerEntity`) (`self.BindingPolicy`) (`|CreateDelegate` :!event `OnTimerPause`)))
    (:`Resume`
      (`Ck_Utils_Timer_UE.BindTo_OnTimerResume` (`self.TimerEntity`) (`self.BindingPolicy`) (`|CreateDelegate` :!event `OnTimerResume`)))))

(event `OnTimerStop`
  (params (InHandle :type "Ck_Handle Structure") (InChrono :type "Ck_Chrono Structure"))
  ;[1 0 0.1875] Timer Events
  (`self.OnTimerManipulated` InHandle InChrono))

(event `OnTimerResume`
  (params (InHandle :type "Ck_Handle Structure") (InChrono :type "Ck_Chrono Structure"))
  ;[1 0 0.1875] Timer Events
  (`self.OnTimerManipulated` InHandle InChrono))

(event `OnTimerPause`
  (params (InHandle :type "Ck_Handle Structure") (InChrono :type "Ck_Chrono Structure"))
  ;[1 0 0.1875] Timer Events
  (`self.OnTimerManipulated` InHandle InChrono))

(event `OnTimerReset`
  (params (InHandle :type "Ck_Handle Structure") (InChrono :type "Ck_Chrono Structure"))
  ;[1 0 0.1875] Timer Events
  (`self.OnTimerManipulated` InHandle InChrono))

(event `self.Deactivate_BP`
  ;[1 0.3281 0] Deactivate
  (`parent.Deactivate_BP`)
  (`/CkFoundation/CkEcs/BPML_CkEcs_EntityHandle.ValidateEntityHandle` (`self.TimerEntity`)
    (:`IsValid`
      (switch `ECk_Timer_Manipulate` (`self.TimerManipulation`)
        (:`Reset`
          (`Ck_Utils_Timer_UE.UnbindFrom_OnTimerReset` (`self.TimerEntity`) (`|CreateDelegate` :!event `OnTimerReset`)))
        (:`Complete`
          (`Ck_Utils_Timer_UE.UnbindFrom_OnTimerDone` (`self.TimerEntity`) (`|CreateDelegate` :!event `OnTimerDone`)))
        (:`Stop`
          (`Ck_Utils_Timer_UE.UnbindFrom_OnTimerStop` (`self.TimerEntity`) (`|CreateDelegate` :!event `OnTimerStop`)))
        (:`Pause`
          (`Ck_Utils_Timer_UE.UnbindFrom_OnTimerPause` (`self.TimerEntity`) (`|CreateDelegate` :!event `OnTimerPause`)))
        (:`Resume`
          (`Ck_Utils_Timer_UE.UnbindFrom_OnTimerResume` (`self.TimerEntity`) (`|CreateDelegate` :!event `OnTimerResume`)))))))