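; Blueprint task that, going by its name, waits for a timer to stop, with the timer identified by name on an owner entity.
; On activation it resolves the timer entity from the owner and name tag, then hands off to the parent task's activation only if valid.
; A failed lookup triggers an ensure reporting the name, owner and task, while deactivation simply defers to the parent.
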(event `self.Activate_BP`
  (set `self.TimerEntity` (`Ck_Utils_Timer_UE.TryGet_Timer` (`self.TimerOwnerEntity`) (`self.TimerName`)))
  (`Ck_Utils_Ensure_UE.EnsureMsgf` (`Ck_Utils_Handle_UE.Get_IsValid` (`self.TimerEntity`)) (`|FormatText` self "Could NOT find Timer  with Name [{name}] in Entity  [{owner}] in [{self}]" (`BlueprintGameplayTagLibrary.GetTagName` (`self.TimerName`)) (`Ck_Utils_Handle_UE.Conv_HandleToText` (`self.TimerOwnerEntity`)))
    (:`Valid`
      (`parent.Activate_BP`))))

(event `self.Deactivate_BP`
  (`parent.Deactivate_BP`))