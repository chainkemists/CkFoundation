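; A TaskForge task node that creates and runs a CkFoundation timer, optionally looping and with a randomized start delay.
; On activation a temporary delay timer on a transient entity runs first if needed, then the main timer starts on its own entity and reports start and update events, including the rolled delay.
; Looping timers are checked for a custom name.
; Deactivation unbinds and destroys both timers and their entities; status text shows delay progress.
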(event `self.Activate_BP`
  (bind _timername (`self.TimerName`))
  (if (`self.Looping`)
    (`Ck_Utils_Ensure_UE.EnsureMsgf` (and (`BlueprintGameplayTagLibrary.IsGameplayTagValid` _timername) (not (`BlueprintGameplayTagLibrary.MatchesTag` _timername (struct :`TagName` "Timer.WaitForNewTimerTask") true))) (`|FormatText` "Timer found in [{outer}] is LOOPING and does NOT have a name" (`KismetSystemLibrary.GetOuterObject` self))
      (:`Valid`
        _)
      (:`Invalid`
        _)))
  (bind _output_get (set `self.RandomStartingVariance` (+ (`self.StartDelay`) (`Ck_Utils_FloatRange_UE.Get_RandomValueInRange` (`self.StartDelayVariance`)))))
  (if (`/CkFoundation/CkCore/Math/Math_CkCore_ML.>0 (float)` _output_get)
    (bind _returnvalue (`Ck_Utils_EntityLifetime_UE.Request_CreateEntity_TransientOwner`))
    (bind _output_get_2 (set `self._EntityWithStartDelayTimer` _returnvalue))
    (bind _outnewtimer (`/CkFoundation/CkTimer/Utils_CkTimer_FL.[Ck][Timer] Add New Timer` (struct :`TagName` "Timer.WaitForNewTimerTaskStartDelay") _output_get_2 (`self.RandomStartingVariance`) "PauseOnDone" "Running"))
    (set `self._StartDelayTimer` _outnewtimer)
    (bind (_taskobject _timerdone_outtimerentity) (`|TaskForge_K2Node` (`self._StartDelayTimer`))
      (:`TimerDone`
        (`Ck_Utils_EntityLifetime_UE.Request_DestroyEntity` _timerdone_outtimerentity))))
  (bind _returnvalue_2 (`Ck_Utils_EntityLifetime_UE.Request_CreateEntity_TransientOwner`))
  (bind _output_get_3 (set `self._EntityWithTimer` _returnvalue_2))
  (bind _outnewtimer_2 (`/CkFoundation/CkTimer/Utils_CkTimer_FL.[Ck][Timer] Add New Timer` (`self.TimerName`) _output_get_3 (`self.Time`) (select `bool` (`self.Looping`) :`false` "PauseOnDone" :`true` "ResetOnDone" :!type "ECk_Timer_Behavior Enum") "Running"))
  (bind _output_get_4 (set `self.TimerEntity` _outnewtimer_2))
  (`self.OnTimerStarted` _output_get_4)
  (add `self.TimerManipulated` (delegate `OnTimerManipulated`))
  (`parent.Activate_BP`))

(event `OnTimerManipulated` :!signature `self.TimerManipulated`
  (params (OutTimerEntity :type "Ck_Handle_Timer Structure") (OutTimerChrono :type "Ck_Chrono Structure") (InDeltaT :type "Ck_Time Structure") (OutEventType :type "/CkFoundation/K2Nodes/Tasks/CkTimer/EventType_Timer_CkFoundation_E Enum" :default "NewEnumerator1"))
  (`self.OnTimerEvent` OutTimerEntity OutTimerChrono (`._Seconds` (break `Ck_Time` InDeltaT)) (`self.RandomStartingVariance`)))

(event `self.Deactivate_BP`
  (`parent.Deactivate_BP`)
  (remove `self.TimerManipulated` (`|CreateDelegate` :!event `OnTimerManipulated`))
  (`Ck_Utils_EntityLifetime_UE.Request_DestroyEntity` (`self._StartDelayTimer`))
  (`Ck_Utils_EntityLifetime_UE.Request_DestroyEntity` (`self.TimerEntity`))
  (`Ck_Utils_EntityLifetime_UE.Request_DestroyEntity` (`self._EntityWithStartDelayTimer`))
  (`Ck_Utils_EntityLifetime_UE.Request_DestroyEntity` (`self._EntityWithTimer`)))

(fn `Get_StatusString_BP`
  (returns (ReturnValue :type String))
  (`/CkFoundation/CkEcs/EntityHandle_CkEcs_ML.ValidateEntityHandle` (`self._StartDelayTimer`)
    (:`IsValid`
      (return (`KismetTextLibrary.Conv_TextToString` (`|FormatText` "{owner} \n{timer} \nDelay: {delay}" (`Ck_Utils_Handle_UE.Conv_HandleToString` (`Ck_Utils_EntityLifetime_UE.Get_LifetimeOwner` (`self.TimerEntity`))) (`Ck_Utils_Handle_UE.Conv_HandleToString` (`self.TimerEntity`)) (`self.Get_FormatTimerProgress` (`self._StartDelayTimer`))))))
    (:`NotValid`
      (bind _returnvalue (`parent.Get_StatusString_BP`))
      (return _returnvalue))))