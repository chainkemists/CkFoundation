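; Latent task Blueprint that waits for a Ck timer entity to deplete.
; On activation it binds to the timer's depleted event, with a policy that also fires if a payload is already in flight this frame.
; Each depletion calls OnTimerDepleted with the timer entity and its chrono.
; Deactivation unbinds the delegate only if the timer entity handle is still valid.
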(event `self.Activate_BP`
  ;[1 0 0.8906] Activate
  (`parent.Activate_BP`)
  (`Ck_Utils_Timer_UE.BindTo_OnTimerDepleted` (`self.TimerEntity`) "FireIfPayloadInFlightThisFrame" (delegate `TimerDepleted`)))

(event `TimerDepleted`
  (params (InHandle :type "Ck_Handle Structure") (InChrono :type "Ck_Chrono Structure"))
  (`self.OnTimerDepleted` InHandle InChrono))

(event `self.Deactivate_BP`
  ;[1 0.3281 0] Deactivate
  (`parent.Deactivate_BP`)
  (`/CkFoundation/CkEcs/BPML_CkEcs_EntityHandle.ValidateEntityHandle` (`self.TimerEntity`)
    (:`IsValid`
      (`Ck_Utils_Timer_UE.UnbindFrom_OnTimerDepleted` (`self.TimerEntity`) (`|CreateDelegate` :!event `TimerDepleted`)))))