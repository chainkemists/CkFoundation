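; Latent task node that waits for one chosen CkTimer event type on a timer entity and broadcasts TimerManipulated with handle, chrono and delta time.
; Activation ensures the timer is valid, then binds only the delegate matching EventType using the supplied binding policy.
; Deactivation unbinds every timer event if the handle is still valid.
; The Jump handler reports its event type as Reset and drops jump direction and amount.
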(event `self.Activate_BP`
  ;[1 0 0.8906] Activate
  (`parent.Activate_BP`)
  (`Ck_Utils_Ensure_UE.EnsureMsgf` (`Ck_Utils_Handle_UE.Get_IsValid` (`self.TimerEntity`)) (`|FormatText` self "Invalid Timer handle supplied to [{self}]")
    (:`Valid`
      (switch `/CkFoundation/K2Nodes/Tasks/CkTimer/EventType_Timer_CkFoundation_E` (`self.EventType`)
        (:`NewEnumerator1`
          ;;[1 0 0.3984] OnDone
          (`Ck_Utils_Timer_UE.BindTo_OnDone` (`self.TimerEntity`) (`self.BindingPolicy`) (`|CreateDelegate` :!event `OnTimerDone`)))
        (:`NewEnumerator0`
          ;;[0.9922 0 1] OnDepleted
          (`Ck_Utils_Timer_UE.BindTo_OnDepleted` (`self.TimerEntity`) (`self.BindingPolicy`) (`|CreateDelegate` :!event `OnTimerDepleted`)))
        (:`NewEnumerator2`
          ;;[0 1 0.01562] OnPause
          (`Ck_Utils_Timer_UE.BindTo_OnPause` (`self.TimerEntity`) (`self.BindingPolicy`) (`|CreateDelegate` :!event `OnTimerPause`)))
        (:`NewEnumerator3`
          ;;[1 0 0.2578] OnReset
          (`Ck_Utils_Timer_UE.BindTo_OnReset` (`self.TimerEntity`) (`self.BindingPolicy`) (`|CreateDelegate` :!event `OnTimerReset`)))
        (:`NewEnumerator4`
          ;;[0 0.3437 1] OnResume
          (`Ck_Utils_Timer_UE.BindTo_OnResume` (`self.TimerEntity`) (`self.BindingPolicy`) (`|CreateDelegate` :!event `OnTimerResume`)))
        (:`NewEnumerator5`
          ;;[1 0 0.9609] OnStop
          (`Ck_Utils_Timer_UE.BindTo_OnStop` (`self.TimerEntity`) (`self.BindingPolicy`) (`|CreateDelegate` :!event `OnTimerStop`)))
        (:`NewEnumerator6`
          ;;[0 0.6953 1] OnUpdate
          (`Ck_Utils_Timer_UE.BindTo_OnUpdate` (`self.TimerEntity`) (`self.BindingPolicy`) (`|CreateDelegate` :!event `OnTimerUpdate`)))
        (:`NewEnumerator7`
          ;;[0 0.6953 1] OnJump
          (`Ck_Utils_Timer_UE.BindTo_OnJump` (`self.TimerEntity`) (`self.BindingPolicy`) (`|CreateDelegate` :!event `OnTimerJump`)))))))

(event `OnTimerUpdate`
  (params (InHandle :type "Ck_Handle_Timer Structure") (InChrono :type "Ck_Chrono Structure") (InDeltaT :type "Ck_Time Structure"))
  ;[1 0 0.1875] Timer Events
  (`self.TimerManipulated` InHandle InChrono InDeltaT "NewEnumerator6"))

(event `OnTimerDepleted`
  (params (InHandle :type "Ck_Handle_Timer Structure") (InChrono :type "Ck_Chrono Structure") (InDeltaT :type "Ck_Time Structure"))
  ;[1 0 0.1875] Timer Events
  (`self.TimerManipulated` InHandle InChrono InDeltaT "NewEnumerator0"))

(event `OnTimerDone`
  (params (InHandle :type "Ck_Handle_Timer Structure") (InChrono :type "Ck_Chrono Structure") (InDeltaT :type "Ck_Time Structure"))
  ;[1 0 0.1875] Timer Events
  (`self.TimerManipulated` InHandle InChrono InDeltaT "NewEnumerator1"))

(event `OnTimerStop`
  (params (InHandle :type "Ck_Handle_Timer Structure") (InChrono :type "Ck_Chrono Structure") (InDeltaT :type "Ck_Time Structure"))
  ;[1 0 0.1875] Timer Events
  (`self.TimerManipulated` InHandle InChrono InDeltaT "NewEnumerator5"))

(event `OnTimerResume`
  (params (InHandle :type "Ck_Handle_Timer Structure") (InChrono :type "Ck_Chrono Structure") (InDeltaT :type "Ck_Time Structure"))
  ;[1 0 0.1875] Timer Events
  (`self.TimerManipulated` InHandle InChrono InDeltaT "NewEnumerator4"))

(event `OnTimerPause`
  (params (InHandle :type "Ck_Handle_Timer Structure") (InChrono :type "Ck_Chrono Structure") (InDeltaT :type "Ck_Time Structure"))
  ;[1 0 0.1875] Timer Events
  (`self.TimerManipulated` InHandle InChrono InDeltaT "NewEnumerator2"))

(event `OnTimerReset`
  (params (InHandle :type "Ck_Handle_Timer Structure") (InChrono :type "Ck_Chrono Structure") (InDeltaT :type "Ck_Time Structure"))
  ;[1 0 0.1875] Timer Events
  (`self.TimerManipulated` InHandle InChrono InDeltaT "NewEnumerator3"))

(event `OnTimerJump`
  (params (InHandle :type "Ck_Handle_Timer Structure") (InChrono :type "Ck_Chrono Structure") (InDeltaT :type "Ck_Time Structure") (InJumpDirection :type "ECk_Timer_JumpDirection Enum" :default "Forwards") (InJumpAmount :type "Ck_Time Structure"))
  ;[1 0 0.1875] Timer Events
  (`self.TimerManipulated` InHandle InChrono InDeltaT "NewEnumerator3"))

(event `self.Deactivate_BP`
  ;[1 0.3281 0] Deactivate
  (`parent.Deactivate_BP`)
  (`/CkFoundation/CkEcs/EntityHandle_CkEcs_ML.ValidateEntityHandle` (`self.TimerEntity`)
    (:`IsValid`
      (`|ExecutionSequence`
        (:`then_0`
          ;;[0.9688 0 1] OnReset
          (`Ck_Utils_Timer_UE.UnbindFrom_OnReset` (`self.TimerEntity`) (`|CreateDelegate` :!event `OnTimerReset`)))
        (:`then_1`
          ;;[0 0.6484 1] OnDone
          (`Ck_Utils_Timer_UE.UnbindFrom_OnDone` (`self.TimerEntity`) (`|CreateDelegate` :!event `OnTimerDone`)))
        (:`then_2`
          ;;[1 0 0.4453] OnStop
          (`Ck_Utils_Timer_UE.UnbindFrom_OnStop` (`self.TimerEntity`) (`|CreateDelegate` :!event `OnTimerStop`)))
        (:`then_3`
          ;;[1 0.8672 0] OnPause
          (`Ck_Utils_Timer_UE.UnbindFrom_OnPause` (`self.TimerEntity`) (`|CreateDelegate` :!event `OnTimerPause`)))
        (:`then_4`
          ;;[1 0.3281 0] OnResume
          (`Ck_Utils_Timer_UE.UnbindFrom_OnResume` (`self.TimerEntity`) (`|CreateDelegate` :!event `OnTimerResume`)))
        (:`then_5`
          ;;[0.03125 0 1] OnDepleted
          (`Ck_Utils_Timer_UE.UnbindFrom_OnDepleted` (`self.TimerEntity`) (`|CreateDelegate` :!event `OnTimerDepleted`)))
        (:`then_6`
          ;;[0.3828 1 0] OnUpdate
          (`Ck_Utils_Timer_UE.UnbindFrom_OnUpdate` (`self.TimerEntity`) (`|CreateDelegate` :!event `OnTimerUpdate`)))
        (:`then_7`
          ;;[1 0 0.4453] OnJump
          (`Ck_Utils_Timer_UE.UnbindFrom_OnJump` (`self.TimerEntity`) (`|CreateDelegate` :!event `OnTimerJump`)))))))