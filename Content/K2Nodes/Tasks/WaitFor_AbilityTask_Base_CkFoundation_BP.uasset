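; Base Blueprint task node in CkFoundation for wait-for tasks that can be tied to the lifetime of an optional ability.
; On activation it binds to that ability's deactivated event when the handle is valid, also firing for a deactivation already in flight this frame.
; When the ability ends, the task deactivates itself, and its own deactivation removes the binding.
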(event `self.Activate_BP`
  (bind _optionalabilityhandle (`self.OptionalAbilityHandle`))
  (`parent.Activate_BP`)
  (`/CkFoundation/CkEcs/EntityHandle_CkEcs_ML.ValidateEntityHandle` _optionalabilityhandle
    (:`IsValid`
      (if (`Ck_Utils_Ability_UE.Has` _optionalabilityhandle)
        (`Ck_Utils_Ability_UE.BindTo_OnAbilityDeactivated` (`self.OptionalAbilityHandle`) "FireIfPayloadInFlightThisFrame" (delegate `OnAbilityEnded`))))))

(event `OnAbilityEnded`
  (params (InAbilityHandle :type "Ck_Handle Structure"))
  (`self.Deactivate`))

(event `self.Deactivate_BP`
  (bind _optionalabilityhandle (`self.OptionalAbilityHandle`))
  (`parent.Deactivate_BP`)
  (`/CkFoundation/CkEcs/EntityHandle_CkEcs_ML.ValidateEntityHandle` _optionalabilityhandle
    (:`IsValid`
      (if (`Ck_Utils_Ability_UE.Has` _optionalabilityhandle)
        (`Ck_Utils_Ability_UE.UnbindFrom_OnAbilityDeactivated` (`self.OptionalAbilityHandle`) (delegate `OnAbilityEnded`))))))