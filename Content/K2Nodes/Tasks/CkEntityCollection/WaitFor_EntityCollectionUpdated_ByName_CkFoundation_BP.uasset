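; A CkFoundation task Blueprint for waiting on updates to an Entity Collection identified by name on an owner entity.
; On activation it looks up the collection handle from the owner entity and name tag, then ensures that handle is valid.
; Only a valid handle continues to the parent activation, which presumably does the waiting; a failed lookup reports the missing name and owner.
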(event `self.Activate_BP`
  (set `self.EntityCollectionHandle` (`Ck_Utils_EntityCollection_UE.TryGet_EntityCollection` (`self.EntityCollectionOwnerEntity`) (`self.EntityCollectionName`)))
  (`Ck_Utils_Ensure_UE.EnsureMsgf` (`Ck_Utils_Handle_UE.Get_IsValid` (`self.EntityCollectionHandle`)) (`|FormatText` self "Could NOT find Entity Collection with Name [{name}] in Entity [{owner}] in [{self}]" (`BlueprintGameplayTagLibrary.GetTagName` (`self.EntityCollectionName`)) (`Ck_Utils_Handle_UE.Conv_HandleToText` (`self.EntityCollectionOwnerEntity`)))
    (:`Valid`
      (`parent.Activate_BP`))))