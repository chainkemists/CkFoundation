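; Blueprint async task node that waits for updates to a CkFoundation entity collection and rebroadcasts them.
; On activation it ensures the collection handle is valid and binds to its collection-updated event, then forwards previous and current contents plus added and removed entities through its output delegate.
; Deactivation unbinds if the handle is still valid, and a status string reports the collection's lifetime owner and handle.
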(event `self.Activate_BP`
  (`parent.Activate_BP`)
  (`Ck_Utils_Ensure_UE.EnsureMsgf` (`Ck_Utils_Handle_UE.Get_IsValid` (`self.EntityCollectionHandle`)) (`|FormatText` self "Invalid Entity Collection handle supplied to [{self}]")
    (:`Valid`
      (`Ck_Utils_EntityCollection_UE.BindTo_OnCollectionUpdated` (`self.EntityCollectionHandle`) (delegate `OnEntityCollectionUpdated`)))))

(event `OnEntityCollectionUpdated`
  (params (InEntityCollection :type "Ck_Handle_EntityCollection Structure") (InPreviousContent :type "Ck_EntityCollection_Content Structure (by ref)") (InCurrentContent :type "Ck_EntityCollection_Content Structure (by ref)") (InEntitiesAdded :type "Array of Ck_Handle Structure (by ref)") (InEntitiesRemoved :type "Array of Ck_Handle Structure (by ref)"))
  (`self.CollectionUpdated` InEntityCollection (`._EntitiesInCollection` (break `Ck_EntityCollection_Content` InPreviousContent)) (`._EntitiesInCollection` (break `Ck_EntityCollection_Content` InCurrentContent)) InEntitiesAdded InEntitiesRemoved))

(event `self.Deactivate_BP`
  (`parent.Deactivate_BP`)
  (bind _outhandle (`/CkFoundation/CkEcs/EntityHandle_CkEcs_ML.ValidateEntityHandle` (`self.EntityCollectionHandle`))
    (:`IsValid`
      (`Ck_Utils_EntityCollection_UE.UnbindFrom_OnCollectionUpdated` _outhandle (`|CreateDelegate` :!event `OnEntityCollectionUpdated`)))))

(fn `Get_StatusString_BP`
  (returns (ReturnValue :type String))
  (`/CkFoundation/CkEcs/EntityHandle_CkEcs_ML.ValidateEntityHandle` (`self.EntityCollectionHandle`)
    (:`IsValid`
      (return (`KismetTextLibrary.Conv_TextToString` (`|FormatText` "{owner} \n{collection}" (`Ck_Utils_Handle_UE.Conv_HandleToString` (`Ck_Utils_EntityLifetime_UE.Get_LifetimeOwner` (`self.EntityCollectionHandle`))) (`Ck_Utils_Handle_UE.Conv_HandleToString` (`self.EntityCollectionHandle`))))))
    (:`NotValid`
      (return "Invalid EntityCollection Entity"))))