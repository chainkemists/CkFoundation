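; Blueprint task in CkFoundation that waits for begin and end overlap events on a supplied sensor entity handle.
; Activation ensures the handle is valid, then binds to both overlap signals with a policy that also fires for payloads already in flight that frame.
; Each handler re-broadcasts the owner handle, sensor handle and overlap payload through the task's output delegates.
; Deactivation unbinds both if the handle is still valid.
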(event `self.Activate_BP`
  (`parent.Activate_BP`)
  (`Ck_Utils_Ensure_UE.EnsureMsgf` (`Ck_Utils_Handle_UE.Get_IsValid` (`self.SensorHandle`)) (`|FormatText` self "Invalid Sensor handle supplied to [{self}]")
    (:`Valid`
      (bind _returnvalue (`Ck_Utils_Sensor_UE.BindTo_OnBeginOverlap` (`self.SensorHandle`) "FireIfPayloadInFlightThisFrame" (delegate `OnSensor_BeginOverlap`)))
      (`Ck_Utils_Sensor_UE.BindTo_OnEndOverlap` _returnvalue "FireIfPayloadInFlightThisFrame" (delegate `OnSensor_EndOverlap`)))))

(event `OnSensor_BeginOverlap`
  (params (InHandle :type "Ck_Handle Structure") (InPayload :type "Ck_Sensor_Payload_OnBeginOverlap Structure"))
  (`self.SensorBeginOverlap` InHandle (`self.SensorHandle`) InPayload))

(event `OnSensor_EndOverlap`
  (params (InHandle :type "Ck_Handle Structure") (InPayload :type "Ck_Sensor_Payload_OnEndOverlap Structure"))
  (`self.SensorEndOverlap` InHandle (`self.SensorHandle`) InPayload))

(event `self.Deactivate_BP`
  (`parent.Deactivate_BP`)
  (bind _outhandle (`/CkFoundation/CkEcs/EntityHandle_CkEcs_ML.ValidateEntityHandle` (`self.SensorHandle`))
    (:`IsValid`
      (bind _returnvalue (`Ck_Utils_Sensor_UE.UnbindFrom_OnBeginOverlap` _outhandle (`|CreateDelegate` :!event `OnSensor_BeginOverlap`)))
      (`Ck_Utils_Sensor_UE.UnbindFrom_OnEndOverlap` _returnvalue (`|CreateDelegate` :!event `OnSensor_EndOverlap`)))))