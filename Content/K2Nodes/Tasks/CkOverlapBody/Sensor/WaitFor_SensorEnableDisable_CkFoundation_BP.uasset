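; Blueprint async task node that waits for a CkFoundation overlap-body sensor to be enabled or disabled.
; On activation it ensures the sensor handle is valid and binds to its enable/disable event, also firing for a payload already in flight this frame.
; Each event is rebroadcast with owner handle, sensor handle and new state.
; Deactivation unbinds, and the status string shows the sensor's tag name.
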(event `self.Activate_BP`
  (`parent.Activate_BP`)
  (`Ck_Utils_Ensure_UE.EnsureMsgf` (`Ck_Utils_Handle_UE.Get_IsValid` (`self.SensorHandle`)) (`|FormatText` self "Invalid Sensor handle supplied to [{self}]")
    (:`Valid`
      (`Ck_Utils_Sensor_UE.BindTo_OnEnableDisable` (`self.SensorHandle`) "FireIfPayloadInFlightThisFrame" (delegate `OnSensor_EnableDisable`)))))

(event `OnSensor_EnableDisable`
  (params (InHandle :type "Ck_Handle Structure") (InSensorName :type "GameplayTag Structure") (InEnableDisable :type "ECk_EnableDisable Enum" :default "Enable"))
  (`self.SensorEnableDisable` InHandle (`self.SensorHandle`) InEnableDisable))

(event `self.Deactivate_BP`
  (`parent.Deactivate_BP`)
  (bind _outhandle (`/CkFoundation/CkEcs/EntityHandle_CkEcs_ML.ValidateEntityHandle` (`self.SensorHandle`))
    (:`IsValid`
      (`Ck_Utils_Sensor_UE.UnbindFrom_OnEnableDisable` _outhandle (`|CreateDelegate` :!event `OnSensor_EnableDisable`)))))

(fn `Get_StatusString_BP`
  (returns (ReturnValue :type String))
  (bind _outhandle (`/CkFoundation/CkEcs/EntityHandle_CkEcs_ML.ValidateEntityHandle` (`self.SensorHandle`))
    (:`IsValid`
      (return (`KismetStringLibrary.Conv_NameToString` (`BlueprintGameplayTagLibrary.GetTagName` (`Ck_Utils_Sensor_UE.Get_Name` _outhandle)))))
    (:`NotValid`
      (return "Invalid Sensor Entity"))))