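; Blueprint task that, going by its name, waits for an overlap on a Sensor identified by name.
; On activation it looks up the Sensor handle on the owner entity using the given name.
; An ensure reports a missing Sensor with its name and owner, and the parent activation runs only when the handle is valid.
; Deactivation passes straight through to the parent, and this graph contains no overlap handling itself.
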(event `self.Activate_BP`
  (set `self.SensorHandle` (`Ck_Utils_Sensor_UE.TryGet_Sensor` (`self.SensorOwnerEntity`) (`self.SensorName`)))
  (`Ck_Utils_Ensure_UE.EnsureMsgf` (`Ck_Utils_Handle_UE.Get_IsValid` (`self.SensorHandle`)) (`|FormatText` self "Could NOT find Sensor with Name [{name}] in Entity [{owner}] in [{self}]" (`BlueprintGameplayTagLibrary.GetTagName` (`self.SensorName`)) (`Ck_Utils_Handle_UE.Conv_HandleToText` (`self.SensorOwnerEntity`)))
    (:`Valid`
      (`parent.Activate_BP`))))

(event `self.Deactivate_BP`
  (`parent.Deactivate_BP`))