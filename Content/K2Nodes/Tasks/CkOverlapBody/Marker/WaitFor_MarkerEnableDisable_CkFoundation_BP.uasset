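; CkFoundation task node that waits for enable/disable changes on an overlap-body Marker.
; On activation it validates the Marker handle and binds to its enable/disable signal, also firing for a payload already in flight this frame.
; Each signal is relayed through the MarkerEnableDisable dispatcher with owner handle, Marker handle and new state.
; Deactivation unbinds if the handle is still valid; firing does not end the task.
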(event `self.Activate_BP`
  (`parent.Activate_BP`)
  (`Ck_Utils_Ensure_UE.EnsureMsgf` (`Ck_Utils_Handle_UE.Get_IsValid` (`self.MarkerHandle`)) (`|FormatText` self "Invalid Marker handle supplied to [{self}]")
    (:`Valid`
      (`Ck_Utils_Marker_UE.BindTo_OnEnableDisable` (`self.MarkerHandle`) "FireIfPayloadInFlightThisFrame" (delegate `OnMarker_EnableDisable`)))))

(event `OnMarker_EnableDisable`
  (params (InHandle :type "Ck_Handle Structure") (InMarkerName :type "GameplayTag Structure") (InEnableDisable :type "ECk_EnableDisable Enum" :default "Enable"))
  (`self.MarkerEnableDisable` InHandle (`self.MarkerHandle`) InEnableDisable))

(event `self.Deactivate_BP`
  (`parent.Deactivate_BP`)
  (bind _outhandle (`/CkFoundation/CkEcs/EntityHandle_CkEcs_ML.ValidateEntityHandle` (`self.MarkerHandle`))
    (:`IsValid`
      (`Ck_Utils_Marker_UE.UnbindFrom_OnEnableDisable` _outhandle (`|CreateDelegate` :!event `OnMarker_EnableDisable`)))))