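; Blueprint task in the CkOverlapBody marker set that, per its name, waits for a Marker enable/disable, with the Marker identified by name.
; On activation it looks up the named Marker on the owner entity and stores the handle.
; An ensure reports a failed lookup with name and owner, and parent activation runs only for a valid handle.
; Deactivation simply defers to the parent.
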(event `self.Activate_BP`
  (set `self.MarkerHandle` (`Ck_Utils_Marker_UE.TryGet_Marker` (`self.MarkerOwnerEntity`) (`self.MarkerName`)))
  (`Ck_Utils_Ensure_UE.EnsureMsgf` (`Ck_Utils_Handle_UE.Get_IsValid` (`self.MarkerHandle`)) (`|FormatText` self "Could NOT find Marker with Name [{name}] in Entity [{owner}] in [{self}]" (`BlueprintGameplayTagLibrary.GetTagName` (`self.MarkerName`)) (`Ck_Utils_Handle_UE.Conv_HandleToText` (`self.MarkerOwnerEntity`)))
    (:`Valid`
      (`parent.Activate_BP`))))

(event `self.Deactivate_BP`
  (`parent.Deactivate_BP`))