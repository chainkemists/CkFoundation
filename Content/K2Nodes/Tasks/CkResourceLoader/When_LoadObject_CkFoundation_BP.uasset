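; A Blueprint task node, When_LoadObject, that loads a soft object reference through the CkFoundation resource loader.
; On activation it sends a load request on the ECS world subsystem's transient entity, using the node's soft reference and loading policy.
; When loading completes, it broadcasts the loaded object through OnLoadingDone and deactivates itself.
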(event `self.Activate_BP`
  (`parent.Activate_BP`)
  (`Ck_Utils_ResourceLoader_UE.Request_LoadObject` (`Ck_EcsWorld_Subsystem_UE._TransientEntity` (subsystem `Ck_EcsWorld_Subsystem_UE`)) (make `Ck_Request_ResourceLoader_LoadObject` (`self.ObjectReferenceSoft`) (`self.LoadingPolicy`)) (delegate `LoadDone`)))

(event `LoadDone`
  (params (InPayload :type "Ck_Payload_ResourceLoader_OnObjectLoaded Structure"))
  (`self.OnLoadingDone` (`._LoadedObject` (break `Ck_Payload_ResourceLoader_OnObjectLoaded` InPayload)))
  (`self.Deactivate`))