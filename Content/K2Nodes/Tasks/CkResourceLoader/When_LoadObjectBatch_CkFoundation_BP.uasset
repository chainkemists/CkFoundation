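; Blueprint task node that asynchronously loads a batch of soft object references through the Ck resource loader.
; On activation it sends a load-batch request on the given handle with the chosen loading policy.
; When loading completes, it fires a done output with the handle, unique loaded objects and full ordered list, then deactivates itself.
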(event `self.Activate_BP`
  (`Ck_Utils_ResourceLoader_UE.Request_LoadObjectBatch` (`self.In Handle`) (make `Ck_Request_ResourceLoader_LoadObjectBatch` (`self.Object References Soft`) (`self.Loading Policy`)) (delegate `LoadDone`)))

(event `self.Deactivate_BP`)

(event `LoadDone`
  (params (InHandle :type "Ck_Handle Structure") (InPayload :type "Ck_Payload_ResourceLoader_OnObjectBatchLoaded Structure"))
  (bind (__uniqueloadedobjects __allorderedloadedobjects) (break `Ck_ResourceLoader_LoadedObjectBatch` (`._LoadedObjectBatch` (break `Ck_Payload_ResourceLoader_OnObjectBatchLoaded` InPayload))))
  (bind _output_get (set `self._UniqueLoadedObjects` __uniqueloadedobjects))
  (bind _output_get_2 (set `self._AllOrderedLoadedObjects` __allorderedloadedobjects))
  (`self.OnLoadingDone` InHandle _output_get _output_get_2)
  (`self.Deactivate`))