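; Blueprint task that waits on overlap events from a CkSpatialQuery ProbeTrace entity.
; On activation it ensures the handle is valid, then binds to begin, updated and end overlap signals, firing for payloads in flight that frame, and relays each through its own delegates.
; Deactivation unbinds all three if the handle is still valid.
; Its status string shows the probe trace and its lifetime owner, or flags an invalid entity.
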(event `self.Activate_BP`
  (`parent.Activate_BP`)
  (`Ck_Utils_Ensure_UE.EnsureMsgf` (`Ck_Utils_Handle_UE.Get_IsValid` (`self.ProbeTraceHandle`)) (`|FormatText` self "Invalid ProbeTrace handle supplied to [{self}]")
    (:`Valid`
      (bind _returnvalue (`Ck_Utils_Probe_UE.BindTo_OnBeginOverlap_ProbeTrace` (`self.ProbeTraceHandle`) "FireIfPayloadInFlightThisFrame" "DoNothing" (delegate `OnBeginOverlap`)))
      (bind _returnvalue_2 (`Ck_Utils_Probe_UE.BindTo_OnOverlapUpdated_ProbeTrace` _returnvalue "FireIfPayloadInFlightThisFrame" "DoNothing" (delegate `OnOverlapUpdated`)))
      (`Ck_Utils_Probe_UE.BindTo_OnEndOverlap_ProbeTrace` _returnvalue_2 "FireIfPayloadInFlightThisFrame" "DoNothing" (delegate `OnEndOverlap`)))))

(event `OnBeginOverlap`
  (params (InHandle :type "Ck_Handle_ProbeTrace Structure") (InPayload :type "Ck_Probe_Payload_OnBeginOverlap Structure"))
  (`self.BeginOverlap` InHandle InPayload))

(event `OnOverlapUpdated`
  (params (InHandle :type "Ck_Handle_ProbeTrace Structure") (InPayload :type "Ck_Probe_Payload_OnOverlapUpdated Structure"))
  (`self.OverlapUpdated` InHandle InPayload))

(event `OnEndOverlap`
  (params (InHandle :type "Ck_Handle_ProbeTrace Structure") (InPayload :type "Ck_Probe_Payload_OnEndOverlap Structure"))
  (`self.EndOverlap` InHandle InPayload))

(event `self.Deactivate_BP`
  (`parent.Deactivate_BP`)
  (bind _outhandle (`/CkFoundation/CkEcs/EntityHandle_CkEcs_ML.ValidateEntityHandle` (`self.ProbeTraceHandle`))
    (:`IsValid`
      (bind _returnvalue (`Ck_Utils_Probe_UE.UnbindFrom_OnBeginOverlap_ProbeTrace` _outhandle (`|CreateDelegate` :!event `OnBeginOverlap`)))
      (bind _returnvalue_2 (`Ck_Utils_Probe_UE.UnbindFrom_OnOverlapUpdated_ProbeTrace` _returnvalue (`|CreateDelegate` :!event `OnOverlapUpdated`)))
      (`Ck_Utils_Probe_UE.UnbindFrom_OnEndOverlap_ProbeTrace` _returnvalue_2 (`|CreateDelegate` :!event `OnEndOverlap`)))))

(fn `Get_StatusString_BP`
  (returns (ReturnValue :type String))
  (`/CkFoundation/CkEcs/EntityHandle_CkEcs_ML.ValidateEntityHandle` (`self.ProbeTraceHandle`)
    (:`IsValid`
      (return (`KismetTextLibrary.Conv_TextToString` (`|FormatText` "{owner} \n{probe}" (`Ck_Utils_Handle_UE.Conv_HandleToString` (`Ck_Utils_EntityLifetime_UE.Get_LifetimeOwner` (`self.ProbeTraceHandle`))) (`Ck_Utils_Handle_UE.Conv_HandleToString` (`self.ProbeTraceHandle`))))))
    (:`NotValid`
      (return "Invalid Probe Entity"))))