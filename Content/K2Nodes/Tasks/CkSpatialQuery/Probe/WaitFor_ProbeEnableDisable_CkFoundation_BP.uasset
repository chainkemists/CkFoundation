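; Latent task Blueprint from CkFoundation's SpatialQuery probe nodes that reports when a probe is enabled or disabled.
; On activation it validates the probe handle and binds to its enable/disable signal, also firing for payloads in flight this frame.
; Each signal is re-broadcast with handle and state, and the binding persists until deactivation unbinds it.
; The status string shows the probe and its shape type, or flags an invalid entity.
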(event `self.Activate_BP`
  (`parent.Activate_BP`)
  (`Ck_Utils_Ensure_UE.EnsureMsgf` (`Ck_Utils_Handle_UE.Get_IsValid` (`self.ProbeHandle`)) (`|FormatText` self "Invalid Probe handle supplied to [{self}]")
    (:`Valid`
      (`Ck_Utils_Probe_UE.BindTo_OnEnableDisable` (`self.ProbeHandle`) "FireIfPayloadInFlightThisFrame" "DoNothing" (delegate `Event_OnEnableDisable`)))))

(event `Event_OnEnableDisable`
  (params (InHandle :type "Ck_Handle_Probe Structure") (InPayload :type "Ck_Probe_Payload_OnEnableDisable Structure"))
  (`self.OnEnableDisable` InHandle (`._EnableDisable` (break `Ck_Probe_Payload_OnEnableDisable` InPayload))))

(event `self.Deactivate_BP`
  (`parent.Deactivate_BP`)
  (bind _outhandle (`/CkFoundation/CkEcs/EntityHandle_CkEcs_ML.ValidateEntityHandle` (`self.ProbeHandle`))
    (:`IsValid`
      (`Ck_Utils_Probe_UE.UnbindFrom_OnEnableDisable` _outhandle (`|CreateDelegate` :!event `Event_OnEnableDisable`)))))

(fn `Get_StatusString_BP`
  (returns (ReturnValue :type String))
  (bind _outhandle (`/CkFoundation/CkEcs/EntityHandle_CkEcs_ML.ValidateEntityHandle` (`self.ProbeHandle`))
    (:`IsValid`
      (return (`KismetTextLibrary.Conv_TextToString` (`|FormatText` "{probe} \n{value}" (`Ck_Utils_Handle_UE.Conv_HandleToString` (`self.ProbeHandle`)) (`|GetEnumeratorNameAsString` (`Ck_Utils_Shapes_UE.Get_ShapeType` _outhandle))))))
    (:`NotValid`
      (return "Invalid Probe Entity"))))