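; Blueprint task that waits for overlap events on a CkSpatialQuery Probe entity and relays them as Begin, Updated and End callbacks.
; On activation it validates the Probe handle and binds to begin, persisted and end overlap, using a policy that also fires for payloads in flight this frame.
; Deactivation unbinds all three delegates if the handle is still valid.
; Its status string reports the probe's lifetime owner, handle and enabled state.
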(event `self.Activate_BP`
  (`parent.Activate_BP`)
  (`Ck_Utils_Ensure_UE.EnsureMsgf` (`Ck_Utils_Handle_UE.Get_IsValid` (`self.ProbeHandle`)) (`|FormatText` self "Invalid Probe handle supplied to [{self}]")
    (:`Valid`
      (bind _returnvalue (`Ck_Utils_Probe_UE.BindTo_OnBeginOverlap` (`self.ProbeHandle`) "FireIfPayloadInFlightThisFrame" "DoNothing" (delegate `OnBeginOverlap`)))
      (bind _returnvalue_2 (`Ck_Utils_Probe_UE.BindTo_OnOverlapPersisted` _returnvalue "FireIfPayloadInFlightThisFrame" "DoNothing" (delegate `OnOverlapUpdated`)))
      (`Ck_Utils_Probe_UE.BindTo_OnEndOverlap` _returnvalue_2 "FireIfPayloadInFlightThisFrame" "DoNothing" (delegate `OnEndOverlap`)))))

(event `OnOverlapUpdated`
  (params (InHandle :type "Ck_Handle_Probe Structure") (InPayload :type "Ck_Probe_Payload_OnOverlapPersisted Structure"))
  (`self.OverlapUpdated` InHandle InPayload))

(event `OnEndOverlap`
  (params (InHandle :type "Ck_Handle_Probe Structure") (InPayload :type "Ck_Probe_Payload_OnEndOverlap Structure"))
  (`self.EndOverlap` InHandle InPayload))

(event `OnBeginOverlap`
  (params (InHandle :type "Ck_Handle_Probe Structure") (InPayload :type "Ck_Probe_Payload_OnBeginOverlap Structure"))
  (`self.BeginOverlap` InHandle InPayload))

(event `self.Deactivate_BP`
  (`parent.Deactivate_BP`)
  (bind _outhandle (`/CkFoundation/CkEcs/EntityHandle_CkEcs_ML.ValidateEntityHandle` (`self.ProbeHandle`))
    (:`IsValid`
      (bind _returnvalue (`Ck_Utils_Probe_UE.UnbindFrom_OnBeginOverlap` _outhandle (`|CreateDelegate` :!event `OnBeginOverlap`)))
      (bind _returnvalue_2 (`Ck_Utils_Probe_UE.UnbindFrom_OnOverlapPersisted` _returnvalue (`|CreateDelegate` :!event `OnOverlapUpdated`)))
      (`Ck_Utils_Probe_UE.UnbindFrom_OnEndOverlap` _returnvalue_2 (`|CreateDelegate` :!event `OnEndOverlap`)))))

(fn `Get_StatusString_BP`
  (returns (ReturnValue :type String))
  (`/CkFoundation/CkEcs/EntityHandle_CkEcs_ML.ValidateEntityHandle` (`self.ProbeHandle`)
    (:`IsValid`
      (return (`KismetTextLibrary.Conv_TextToString` (`|FormatText` "{owner} \n{probe} \n{status}" (`Ck_Utils_Handle_UE.Conv_HandleToString` (`Ck_Utils_EntityLifetime_UE.Get_LifetimeOwner` (`self.ProbeHandle`))) (`|GetEnumeratorNameAsString` (`Ck_Utils_Probe_UE.Get_IsEnabledDisabled` (`self.ProbeHandle`))) (`Ck_Utils_Handle_UE.Conv_HandleToString` (`self.ProbeHandle`))))))
    (:`NotValid`
      (return "Invalid Probe Entity"))))