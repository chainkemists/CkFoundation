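; Task Blueprint that relays Ck interaction events from an InteractTarget as new-interaction and interaction-finished callbacks.
; On activation it binds to both events, using a policy that also fires for payloads in flight this frame.
; Each handler forwards the target and interaction, with the finished one adding the succeeded/failed result.
; On deactivation it unbinds both handlers if the InteractTarget handle is still valid.
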(event `self.Activate_BP`
  (`parent.Activate_BP`)
  (bind _returnvalue (`Ck_Utils_InteractTarget_UE.BindTo_OnNewInteraction` (`self.InteractTarget`) "FireIfPayloadInFlightThisFrame" "DoNothing" (delegate `Event_OnNewInteraction`)))
  (`Ck_Utils_InteractTarget_UE.BindTo_OnInteractionFinished` _returnvalue "FireIfPayloadInFlightThisFrame" "DoNothing" (delegate `Event_OnInteractionFinished`)))

(event `Event_OnNewInteraction`
  (params (InTarget :type "Ck_Handle_InteractTarget Structure") (InInteraction :type "Ck_Handle_Interaction Structure"))
  (`self.OnNewInteraction` InTarget InInteraction))

(event `Event_OnInteractionFinished`
  (params (InTarget :type "Ck_Handle_InteractTarget Structure") (InInteraction :type "Ck_Handle_Interaction Structure") (SucceededFailed :type "ECk_SucceededFailed Enum" :default "Succeeded"))
  (`self.OnInteractionFinished` InTarget InInteraction SucceededFailed))

(event `self.Deactivate_BP`
  (`parent.Deactivate_BP`)
  (bind _outhandle (`/CkFoundation/CkEcs/EntityHandle_CkEcs_ML.ValidateEntityHandle` (`self.InteractTarget`))
    (:`IsValid`
      (bind _returnvalue (`Ck_Utils_InteractTarget_UE.UnbindFrom_OnNewInteraction` _outhandle (delegate `Event_OnNewInteraction`)))
      (`Ck_Utils_InteractTarget_UE.UnbindFrom_OnInteractionFinished` _returnvalue (delegate `Event_OnInteractionFinished`)))))