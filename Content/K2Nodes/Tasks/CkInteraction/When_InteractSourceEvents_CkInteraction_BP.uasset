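; A Blueprint task node that relays an interact source's interaction events as new-interaction and interaction-finished outputs.
; On activation it binds both events on the InteractSource handle, firing also for payloads already in flight that frame.
; Each handler forwards the source and interaction, with the finished output adding the success or failure result.
; On deactivation it unbinds both, only if the InteractSource entity handle is still valid.
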(event `self.Activate_BP`
  (`parent.Activate_BP`)
  (bind _returnvalue (`Ck_Utils_InteractSource_UE.BindTo_OnNewInteraction` (`self.InteractSource`) "FireIfPayloadInFlightThisFrame" "DoNothing" (delegate `Event_OnNewInteraction`)))
  (`Ck_Utils_InteractSource_UE.BindTo_OnInteractionFinished` _returnvalue "FireIfPayloadInFlightThisFrame" "DoNothing" (delegate `Event_OnInteractionFinished`)))

(event `Event_OnNewInteraction`
  (params (InSource :type "Ck_Handle_InteractSource Structure") (InInteraction :type "Ck_Handle_Interaction Structure"))
  (`self.OnNewInteraction` InSource InInteraction))

(event `Event_OnInteractionFinished`
  (params (InSource :type "Ck_Handle_InteractSource Structure") (InInteraction :type "Ck_Handle_Interaction Structure") (SucceededFailed :type "ECk_SucceededFailed Enum" :default "Succeeded"))
  (`self.OnInteractionFinished` InSource InInteraction SucceededFailed))

(event `self.Deactivate_BP`
  (`parent.Deactivate_BP`)
  (bind _outhandle (`/CkFoundation/CkEcs/EntityHandle_CkEcs_ML.ValidateEntityHandle` (`self.InteractSource`))
    (:`IsValid`
      (bind _returnvalue (`Ck_Utils_InteractSource_UE.UnbindFrom_OnNewInteraction` _outhandle (delegate `Event_OnNewInteraction`)))
      (`Ck_Utils_InteractSource_UE.UnbindFrom_OnInteractionFinished` _returnvalue (delegate `Event_OnInteractionFinished`)))))