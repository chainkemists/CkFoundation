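; Blueprint task node that waits for any of several CkFoundation messages on a handle.
; On activation it binds a broadcast listener for every tag in the message name container, also firing for payloads already in flight that frame.
; Each broadcast is forwarded through the new-message output with its handle, name and payload, repeatedly until deactivation unbinds every listener.
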(event `self.Activate_BP`
  (`parent.Activate_BP`)
  (for _array_element (`BlueprintGameplayTagLibrary.BreakGameplayTagContainer` (`self.InMessageNames`))
    (`Ck_Utils_Messaging_UE.BindTo_OnBroadcast` (`self.InHandle`) _array_element "FireIfPayloadInFlightThisFrame" "DoNothing" (delegate `OnMessageBroadcast`))))

(event `OnMessageBroadcast`
  (params (InHandle :type "Ck_Handle Structure") (InMessageName :type "GameplayTag Structure") (InPayload :type "InstancedStruct Structure"))
  (`self.OnNewMessage` InHandle InMessageName InPayload))

(event `self.Deactivate_BP`
  (`parent.Deactivate_BP`)
  (for _array_element (`BlueprintGameplayTagLibrary.BreakGameplayTagContainer` (`self.InMessageNames`))
    (`Ck_Utils_Messaging_UE.UnbindFrom_OnBroadcast` (`self.InHandle`) _array_element (delegate `OnMessageBroadcast`))))