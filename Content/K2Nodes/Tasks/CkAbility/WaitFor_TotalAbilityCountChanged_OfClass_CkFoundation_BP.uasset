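; Async task Blueprint that, by its name, waits for an ability owner's total count of abilities of a given class to change.
; Activation ensures the Ability Class is valid, then runs the parent activation, or deactivates the task if it is invalid.
; It overrides the parent's ability count getter to return only the count for that class on the owner entity.
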(event `self.Activate_BP`
  (`Ck_Utils_Ensure_UE.EnsureMsgf` (`KismetSystemLibrary.IsValidClass` (`self.AbilityClass`)) (`|FormatText` self "Invalid Ability Class supplied to [{self}]")
    (:`Valid`
      (`parent.Activate_BP`))
    (:`Invalid`
      (`self.Deactivate`))))

(fn `Get_AbilityCount (Override Optional)`
  (returns (ReturnValue :type Integer))
  (return (`Ck_Utils_AbilityOwner_UE.Get_AbilityCount_OfClass` (`self.AbilityOwnerHandle`) (`self.AbilityClass`))))