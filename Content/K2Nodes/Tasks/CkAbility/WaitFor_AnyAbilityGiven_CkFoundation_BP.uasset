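; Task node that notifies whenever any ability is given to an AbilityOwner entity in the CkFoundation ability system.
; On activation it binds to the owner's ability-given signal, also firing for payloads in flight that frame, and re-broadcasts each owner and ability pair.
; An invalid owner handle triggers an ensure and deactivates the task.
; Deactivation unbinds if the handle is still valid, and the status string reports the owner handle.
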(event `self.Activate_BP`
  (`parent.Activate_BP`)
  (`Ck_Utils_Ensure_UE.EnsureMsgf` (`Ck_Utils_Handle_UE.Get_IsValid` (`self.AbilityOwnerHandle`)) (`|FormatText` self "Invalid AbilityOwner Handle provided to [{self}]")
    (:`Valid`
      (`Ck_Utils_AbilityOwner_UE.BindTo_OnAbilityGiven` (`self.AbilityOwnerHandle`) "FireIfPayloadInFlightThisFrame" "DoNothing" (delegate `OnAbilityGiven`)))
    (:`Invalid`
      (`self.Deactivate`))))

(event `OnAbilityGiven`
  (params (InAbilityOwner :type "Ck_Handle_AbilityOwner Structure") (InAbility :type "Ck_Handle_Ability Structure"))
  (`self.AbilityGiven` InAbilityOwner InAbility))

(event `self.Deactivate_BP`
  (`parent.Deactivate_BP`)
  (bind _outhandle (`/CkFoundation/CkEcs/EntityHandle_CkEcs_ML.ValidateEntityHandle` (`self.AbilityOwnerHandle`))
    (:`IsValid`
      (`Ck_Utils_AbilityOwner_UE.UnbindFrom_OnAbilityGiven` _outhandle (`|CreateDelegate` :!event `OnAbilityGiven`)))))

(fn `Get_StatusString_BP`
  (returns (ReturnValue :type String))
  (`/CkFoundation/CkEcs/EntityHandle_CkEcs_ML.ValidateEntityHandle` (`self.AbilityOwnerHandle`)
    (:`IsValid`
      (return (`Ck_Utils_Handle_UE.Conv_HandleToString` (`self.AbilityOwnerHandle`))))
    (:`NotValid`
      (return "Invalid AbilityOwner Entity"))))