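; Ability task that waits for gameplay tags to be removed from an ability owner entity, part of the CkFoundation WaitFor task nodes.
; On activation it binds to the owner's tags-updated signal, also firing for payloads in flight this frame, and unbinds on deactivation.
; When an update carries removed tags, it calls TagsRemoved with the owner, new and previous active tags, and removed tags.
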(event `self.Activate_BP`
  (`parent.Activate_BP`)
  (`Ck_Utils_AbilityOwner_UE.BindTo_OnTagsUpdated` (`self.AbilityOwnerHandle`) "FireIfPayloadInFlightThisFrame" "DoNothing" (delegate `OnTagsRemoved`)))

(event `OnTagsRemoved`
  (params (InHandle :type "Ck_Handle_AbilityOwner Structure") (InPreviousTags :type "GameplayTagContainer Structure (by ref)") (InActiveTags :type "GameplayTagContainer Structure (by ref)") (InTagsRemoved :type "GameplayTagContainer Structure (by ref)") (InTagsAdded :type "GameplayTagContainer Structure (by ref)"))
  (if (`/CkFoundation/CkCore/Math/Math_CkCore_ML.>0int` (`BlueprintGameplayTagLibrary.GetNumGameplayTagsInContainer` InTagsRemoved))
    (`self.TagsRemoved` InHandle InActiveTags InPreviousTags InTagsRemoved)))

(event `self.Deactivate_BP`
  (`parent.Deactivate_BP`)
  (`Ck_Utils_AbilityOwner_UE.UnbindFrom_OnTagsUpdated` (`self.AbilityOwnerHandle`) (delegate `OnTagsRemoved`)))