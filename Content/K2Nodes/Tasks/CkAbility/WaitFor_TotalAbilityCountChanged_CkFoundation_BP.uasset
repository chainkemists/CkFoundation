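; Async task node that reports when the total ability count on an Ability Owner entity changes.
; On activation it validates the handle, fires a "count now" event with the current count, then binds to ability given/revoked and extension added/removed signals.
; Each signal re-reads the count through an overridable getter and broadcasts previous and new values only on change.
; Deactivation unbinds all listeners.
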(event `BindOn_ExtensionRemovedAndAdded`
  ;[0 0 0] BindOn_ExtensionRemovedAndAdded
  (bind _returnvalue (`Ck_Utils_EntityExtension_UE.BindTo_OnExtensionRemoved` (`self.AbilityOwnerHandle`) "FireIfPayloadInFlightThisFrame" "DoNothing" (delegate `OnExtensionRemoved`)))
  (`Ck_Utils_EntityExtension_UE.BindTo_OnExtensionAdded` _returnvalue "FireIfPayloadInFlightThisFrame" "DoNothing" (delegate `OnExtensionAdded`)))

(event `OnExtensionRemoved`
  (params (InExtensionOwner :type "Ck_Handle Structure") (InEntityAsExtension :type "Ck_Handle_EntityExtension Structure"))
  (`self.EvaluateIfAbilityCountChanged`))

(event `OnExtensionAdded`
  (params (InExtensionOwner :type "Ck_Handle Structure") (InEntityAsExtension :type "Ck_Handle_EntityExtension Structure"))
  (`self.EvaluateIfAbilityCountChanged`))

(event `UnbindFrom_ExtensionRemovedAndAdded`
  ;[0 0 0] UnbindFrom_ExtensionRemovedAndAdded
  (bind _returnvalue (`Ck_Utils_EntityExtension_UE.UnbindFrom_OnExtensionRemoved` (`self.AbilityOwnerHandle`) (delegate `OnExtensionRemoved`)))
  (`Ck_Utils_EntityExtension_UE.UnbindFrom_OnExtensionAdded` _returnvalue (delegate `OnExtensionAdded`)))

(event `self.Activate_BP`
  (`parent.Activate_BP`)
  (`Ck_Utils_Ensure_UE.EnsureMsgf` (`Ck_Utils_Handle_UE.Get_IsValid` (`self.AbilityOwnerHandle`)) (`|FormatText` self "Invalid AbilityOwner Handle provided to [{self}]")
    (:`Valid`
      (bind _output_get (set `self._CurrentAbilityCount` (`self.Get_AbilityCount (Override Optional)`)))
      (`self.AbilityCountNow` (`self.AbilityOwnerHandle`) _output_get)
      (`self.BindTo_OnAbilityGivenAndRevoked`)
      (`self.BindOn_ExtensionRemovedAndAdded`))
    (:`Invalid`
      (`self.Deactivate`))))

(event `BindTo_OnAbilityGivenAndRevoked`
  ;[0 0 0] BindTo_OnAbilityGivenAndRevoked
  (bind _returnvalue (`Ck_Utils_AbilityOwner_UE.BindTo_OnAbilityGiven` (`self.AbilityOwnerHandle`) "FireIfPayloadInFlightThisFrame" "DoNothing" (delegate `OnAbilityGiven`)))
  (`Ck_Utils_AbilityOwner_UE.BindTo_OnAbilityRevoked` _returnvalue "FireIfPayloadInFlightThisFrame" "DoNothing" (delegate `OnAbilityRevoked`)))

(event `self.Deactivate_BP`
  (`parent.Deactivate_BP`)
  (`/CkFoundation/CkEcs/EntityHandle_CkEcs_ML.ValidateEntityHandle` (`self.AbilityOwnerHandle`)
    (:`IsValid`
      (`self.UnbindFrom_OnAbilityGivenAndRevoked`)
      (`self.UnbindFrom_ExtensionRemovedAndAdded`))))

(event `OnAbilityRevoked`
  (params (InAbilityOwner :type "Ck_Handle_AbilityOwner Structure") (InAbility :type "Ck_Handle_Ability Structure"))
  (`self.EvaluateIfAbilityCountChanged`))

(event `OnAbilityGiven`
  (params (InAbilityOwner :type "Ck_Handle_AbilityOwner Structure") (InAbility :type "Ck_Handle_Ability Structure"))
  (`self.EvaluateIfAbilityCountChanged`))

(event `UnbindFrom_OnAbilityGivenAndRevoked`
  ;[0 0 0] UnbindFrom_OnAbilityGivenAndRevoked
  (bind _returnvalue (`Ck_Utils_AbilityOwner_UE.UnbindFrom_OnAbilityGiven` (`self.AbilityOwnerHandle`) (`|CreateDelegate` :!event `OnAbilityGiven`)))
  (`Ck_Utils_AbilityOwner_UE.UnbindFrom_OnAbilityRevoked` _returnvalue (`|CreateDelegate` :!event `OnAbilityRevoked`)))

(fn `EvaluateIfAbilityCountChanged`
  (locals (L_NewCount :type Integer :default 0))
  (bind _output_get (set `local.L_NewCount` (`self.Get_AbilityCount (Override Optional)`)))
  (if (!= _output_get (`self._CurrentAbilityCount`))
    (`self.AbilityCountChanged` (`self.AbilityOwnerHandle`) (`self._CurrentAbilityCount`) (`local.L_NewCount`))
    (set `self._CurrentAbilityCount` (`local.L_NewCount`))))

(fn `Get_AbilityCount (Override Optional)`
  (returns (ReturnValue :type Integer))
  (return (`Ck_Utils_AbilityOwner_UE.Get_AbilityCount` (`self.AbilityOwnerHandle`))))

(fn `Get_StatusString_BP`
  (returns (ReturnValue :type String))
  (`/CkFoundation/CkEcs/EntityHandle_CkEcs_ML.ValidateEntityHandle` (`self.AbilityOwnerHandle`)
    (:`IsValid`
      (return (`KismetTextLibrary.Conv_TextToString` (`|FormatText` "{owner} \nTotal Ability Count: {count}" (`Ck_Utils_Handle_UE.Conv_HandleToString` (`self.AbilityOwnerHandle`)) (`self._CurrentAbilityCount`)))))
    (:`NotValid`
      (return "Invalid AbilityOwner Entity"))))