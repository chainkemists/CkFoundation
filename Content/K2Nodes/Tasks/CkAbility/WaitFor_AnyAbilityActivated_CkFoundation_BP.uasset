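; CkFoundation Blueprint task node that waits for any ability to activate on a given ability owner entity.
; On activation it binds to the owner's ability-activated signal, including payloads in flight this frame, or deactivates with an ensure if the handle is invalid.
; Each activation is rebroadcast with owner and ability, as the binding persists after firing.
; Deactivation unbinds if the handle is still valid.
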(event `self.Activate_BP`
  (`parent.Activate_BP`)
  (`Ck_Utils_Ensure_UE.EnsureMsgf` (`Ck_Utils_Handle_UE.Get_IsValid` (`self.AbilityOwnerHandle`)) (`|FormatText` self "Invalid AbilityOwner Handle provided to [{self}]")
    (:`Valid`
      (`Ck_Utils_AbilityOwner_UE.BindTo_OnAbilityActivated` (`self.AbilityOwnerHandle`) "FireIfPayloadInFlightThisFrame" "DoNothing" (delegate `OnAbilityActivated`)))
    (:`Invalid`
      (`self.Deactivate`))))

(event `OnAbilityActivated`
  (params (InAbilityOwner :type "Ck_Handle_AbilityOwner Structure") (InAbility :type "Ck_Handle_Ability Structure"))
  (`self.AbilityActivated` InAbilityOwner InAbility))

(event `self.Deactivate_BP`
  (`parent.Deactivate_BP`)
  (bind _outhandle (`/CkFoundation/CkEcs/EntityHandle_CkEcs_ML.ValidateEntityHandle` (`self.AbilityOwnerHandle`))
    (:`IsValid`
      (`Ck_Utils_AbilityOwner_UE.UnbindFrom_OnAbilityActivated` _outhandle (`|CreateDelegate` :!event `OnAbilityActivated`)))))