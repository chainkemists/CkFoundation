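; Blueprint async task node that waits for specific events on a CkFoundation ability owner.
; On activation it binds to the owner's events, also catching any already in flight that frame, and unbinds on deactivation.
; Each batch is checked against a tag container, and only the first event whose name exactly matches a tag fires the output with the owner handle and event.
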(event `self.Activate_BP`
  (`parent.Activate_BP`)
  (`Ck_Utils_AbilityOwner_UE.BindTo_OnEvents` (`self.AbilityOwnerHandle`) "FireIfPayloadInFlightThisFrame" "DoNothing" (delegate `OnEvent`)))

(event `OnEvent`
  (params (InHandle :type "Ck_Handle_AbilityOwner Structure") (InEvents :type "Array of Ck_AbilityOwner_Event Structure (by ref)"))
  (for _array_element InEvents
    (if (`BlueprintGameplayTagLibrary.HasTag` (`self.TagsToTest`) (`._EventName` (break `Ck_AbilityOwner_Event` _array_element)) true)
      (`self.EventFired` InHandle _array_element)
      (break))))

(event `self.Deactivate_BP`
  (`parent.Deactivate_BP`)
  (`Ck_Utils_AbilityOwner_UE.UnbindFrom_OnEvents` (`self.AbilityOwnerHandle`) (delegate `OnEvent`)))