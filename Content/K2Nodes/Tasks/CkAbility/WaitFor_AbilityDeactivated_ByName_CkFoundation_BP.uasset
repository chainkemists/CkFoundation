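; Blueprint async task node that, going by its name, waits for a named ability to deactivate on an ability owner entity.
; On activation it resolves the ability handle from the owner by name and ensures it is valid, with an error message naming the tag, owner and task.
; The parent task's activation runs only on a valid handle, so the waiting logic is inherited; deactivation simply defers to the parent.
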(event `self.Activate_BP`
  (set `self.AbilityHandle` (`Ck_Utils_AbilityOwner_UE.TryGet_AbilityByName` (`self.AbilityOwnerHandle`) (`self.AbilityName`)))
  (`Ck_Utils_Ensure_UE.EnsureMsgf` (`Ck_Utils_Handle_UE.Get_IsValid` (`self.AbilityHandle`)) (`|FormatText` self "Could NOT find Ability with Name [{name}] in Ability Owner [{owner}] in [{self}]" (`BlueprintGameplayTagLibrary.GetTagName` (`self.AbilityName`)) (`Ck_Utils_Handle_UE.Conv_HandleToText` (`self.AbilityOwnerHandle`)))
    (:`Valid`
      (`parent.Activate_BP`))))

(event `self.Deactivate_BP`
  (`parent.Deactivate_BP`))