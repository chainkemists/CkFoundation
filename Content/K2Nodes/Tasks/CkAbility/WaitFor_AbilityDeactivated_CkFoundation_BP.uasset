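; Blueprint task node that waits for a given Ck ability to deactivate, with separate outcomes for deactivation and for an ability that is already inactive.
; On activation it validates the ability handle, binds to its deactivation signal (also firing for payloads in flight this frame), then reports immediately if the status is Not Active.
; On task deactivation it unbinds if the handle is still valid.
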(event `self.Activate_BP`
  (`parent.Activate_BP`)
  (`Ck_Utils_Ensure_UE.EnsureMsgf` (`Ck_Utils_Handle_UE.Get_IsValid` (`self.AbilityHandle`)) (`|FormatText` self "Invalid Ability Handle provided to [{self}]")
    (:`Valid`
      (bind _returnvalue (`Ck_Utils_Ability_UE.BindTo_OnAbilityDeactivated` (`self.AbilityHandle`) "FireIfPayloadInFlightThisFrame" "DoNothing" (delegate `OnAbilityDeactivated`)))
      (switch `ECk_Ability_Status` (`Ck_Utils_Ability_UE.Get_Status` _returnvalue)
        (:`NotActive`
          (`self.AbilityAlreadyNotActive` _returnvalue))))))

(event `OnAbilityDeactivated`
  (params (InAbilityHandle :type "Ck_Handle_Ability Structure"))
  (`self.AbilityDeactivated` InAbilityHandle))

(event `self.Deactivate_BP`
  (`parent.Deactivate_BP`)
  (bind _outhandle (`/CkFoundation/CkEcs/EntityHandle_CkEcs_ML.ValidateEntityHandle` (`self.AbilityHandle`))
    (:`IsValid`
      (`Ck_Utils_Ability_UE.UnbindFrom_OnAbilityDeactivated` _outhandle (`|CreateDelegate` :!event `OnAbilityDeactivated`)))))