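; A CkFoundation task node that waits for ability owner events and fires EventFired for each one passing its relevant and excluded tag filters.
; With only relevant tags, it binds per tag; otherwise it binds to all events and filters by exact tag match.
; Bindings also catch payloads in flight that frame and persist after firing.
; Deactivation branches on the same lists to call the unbind functions.
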(event `self.Activate_BP`
  (bind __relevanteventslist (`self._RelevantEventsList`))
  (`parent.Activate_BP`)
  (set `self._ExcludedEventsList` (`BlueprintGameplayTagLibrary.BreakGameplayTagContainer` (`self.ExcludedEvents`)))
  (set `self._RelevantEventsList` (`BlueprintGameplayTagLibrary.BreakGameplayTagContainer` (`self.RelevantEvents`)))
  (`/CkFoundation/CkCore/Container/Container_CkCore_ML.Array_IsEmpty_Exec` (`self._ExcludedEventsList`)
    (:`Empty`
      (`/CkFoundation/CkCore/Container/Container_CkCore_ML.Array_IsNotEmpty_Exec` __relevanteventslist
        (:`NotEmpty`
          (for _array_element __relevanteventslist
            (`Ck_Utils_AbilityOwner_UE.BindTo_OnSingleEvent` (`self.AbilityOwnerHandle`) _array_element "FireIfPayloadInFlightThisFrame" "DoNothing" (delegate `OnSingleEvent`))))
        (:`Empty`
          (`Ck_Utils_AbilityOwner_UE.BindTo_OnEvents` (`self.AbilityOwnerHandle`) (`self.RelevantEvents`) (`self.ExcludedEvents`) "FireIfPayloadInFlightThisFrame" "DoNothing" (delegate `OnEvents`) :!label _label))))
    (:`NotEmpty`
      (goto _label))))

(event `OnSingleEvent`
  (params (InHandle :type "Ck_Handle_AbilityOwner Structure") (InEvent :type "Ck_AbilityOwner_Event Structure (by ref)"))
  (`self.EventFired` InHandle InEvent))

(event `OnEvents`
  (params (InHandle :type "Ck_Handle_AbilityOwner Structure") (InEvents :type "Array of Ck_AbilityOwner_Event Structure (by ref)"))
  (for _array_element InEvents
    (bind __eventname (break `Ck_AbilityOwner_Event` _array_element))
    (if (and (or (`KismetArrayLibrary.Array_IsEmpty` (`self._RelevantEventsList`)) (`BlueprintGameplayTagLibrary.HasTag` (`self.RelevantEvents`) __eventname true)) (or (`KismetArrayLibrary.Array_IsEmpty` (`self._ExcludedEventsList`)) (not (`BlueprintGameplayTagLibrary.HasTag` (`self.ExcludedEvents`) __eventname true))))
      (`self.EventFired` InHandle _array_element))))

(event `self.Deactivate_BP`
  (`parent.Deactivate_BP`)
  (`/CkFoundation/CkCore/Container/Container_CkCore_ML.Array_IsEmpty_Exec` (`self._ExcludedEventsList`)
    (:`Empty`
      (bind _outarray (`/CkFoundation/CkCore/Container/Container_CkCore_ML.Array_IsEmpty_Exec` (`self._RelevantEventsList`))
        (:`Empty`
          (for _ _outarray
            (`Ck_Utils_AbilityOwner_UE.UnbindFrom_OnSingleEvent` (`self.AbilityOwnerHandle`) (`|CreateDelegate` :!event `OnSingleEvent`))))
        (:`NotEmpty`
          (`Ck_Utils_AbilityOwner_UE.UnbindFrom_OnEvents` (`self.AbilityOwnerHandle`) (`|CreateDelegate` :!event `OnEvents`) :!label _label_2))))
    (:`NotEmpty`
      (goto _label_2))))