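; Latent task Blueprint that waits for any ability of a given class to be deactivated, in the CkFoundation ability system.
; On activation it ensures the ability class is valid, then runs the parent activation, or deactivates itself if not.
; It overrides the parent's deactivation callback, forwarding only abilities whose script class exactly equals the requested class.
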(event `self.Activate_BP`
  (`Ck_Utils_Ensure_UE.EnsureMsgf` (`KismetSystemLibrary.IsValidClass` (`self.AbilityClass`)) (`|FormatText` self "Invalid Ability Class supplied to [{self}]")
    (:`Valid`
      (`parent.Activate_BP`))
    (:`Invalid`
      (`self.Deactivate`))))

(event `self.OnAbilityDeactivated`
  (params (InAbilityOwner :type "Ck_Handle_AbilityOwner Structure") (InAbility :type "Ck_Handle_Ability Structure"))
  (if (== (`Ck_Utils_Ability_UE.Get_ScriptClass` InAbility) (`self.AbilityClass`))
    (`parent.OnAbilityDeactivated` InAbilityOwner InAbility)))