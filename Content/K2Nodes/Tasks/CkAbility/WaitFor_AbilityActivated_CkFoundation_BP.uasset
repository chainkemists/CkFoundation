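; CkFoundation ability task that waits for a given ability to activate and reports it with the ability handle and activation payload.
; On activation it validates the handle and binds to the activation signal, also firing for a payload already in flight that frame.
; If the ability's status is already Active, it calls a separate AlreadyActive output.
; The binding persists after firing; deactivation unbinds if the handle is still valid.
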(event `self.Activate_BP`
  (`parent.Activate_BP`)
  (`Ck_Utils_Ensure_UE.EnsureMsgf` (`Ck_Utils_Handle_UE.Get_IsValid` (`self.AbilityHandle`)) (`|FormatText` self "Invalid Ability Handle provided to [{self}]")
    (:`Valid`
      (bind _returnvalue (`Ck_Utils_Ability_UE.BindTo_OnAbilityActivated` (`self.AbilityHandle`) "FireIfPayloadInFlightThisFrame" "DoNothing" (delegate `OnAbilityActivated`)))
      (switch `ECk_Ability_Status` (`Ck_Utils_Ability_UE.Get_Status` _returnvalue)
        (:`Active`
          (`self.AbilityAlreadyActive` _returnvalue))))))

(event `OnAbilityActivated`
  (params (InAbilityHandle :type "Ck_Handle_Ability Structure") (InActivationPayload :type "Ck_Ability_Payload_OnActivate Structure (by ref)"))
  (`self.AbilityActivated` InAbilityHandle InActivationPayload))

(event `self.Deactivate_BP`
  (`parent.Deactivate_BP`)
  (bind _outhandle (`/CkFoundation/CkEcs/EntityHandle_CkEcs_ML.ValidateEntityHandle` (`self.AbilityHandle`))
    (:`IsValid`
      (`Ck_Utils_Ability_UE.UnbindFrom_OnAbilityActivated` _outhandle (`|CreateDelegate` :!event `OnAbilityActivated`)))))