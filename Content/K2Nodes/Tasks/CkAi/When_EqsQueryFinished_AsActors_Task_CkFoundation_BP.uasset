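; Async task node that runs an EQS query for a given querier and returns the results as actors through success or failure callbacks.
; On activation it ensures the net mode is not client, since EQS cannot run there, then starts the query and binds to its finished event.
; An invalid query instance, unsuccessful status or failed actor retrieval reports failure.
; The task deactivates after reporting, unbinding from the query.
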(event `self.Activate_BP`
  (`parent.Activate_BP`)
  (`Ck_Utils_Ensure_UE.EnsureMsgf` (not (`Ck_Utils_Net_UE.Get_IsEntityNetMode_Client` (`Ck_EcsWorld_Subsystem_UE._TransientEntity` (subsystem `Ck_EcsWorld_Subsystem_UE`)))) (`|FormatText` "Cannot perform EQS Query [{query}] because EQS Queries cannot run on the CLIENT" (`self.QueryTemplate`))
    (:`Valid`
      (bind _returnvalue (`EnvQueryManager.RunEQSQuery` (`self.QueryTemplate`) (`self.Querier`) (`self.RunMode`)))
      (bind _output_get (set `self._QueryInstance` _returnvalue))
      (`/Engine/EditorBlueprintResources/StandardMacros.IsValid` _output_get
        (:`Is Valid`
          (add `EnvQueryInstanceBlueprintWrapper.OnQueryFinishedEvent` _output_get (delegate `OnEQSQueryFinished`)))
        (:`Is Not Valid`
          (`self.OnFailure` _output_get "Failed")
          (`self.Deactivate`))))
    (:`Invalid`
      (`self.OnFailure` null "Failed")
      (`self.Deactivate`))))

(event `OnEQSQueryFinished`
  (params (QueryInstance :type "EnvQueryInstanceBlueprintWrapper Object Reference") (QueryStatus :type "EEnvQueryStatus Enum" :default "Processing"))
  (if (`|EnumEquality` QueryStatus "Success")
    (bind (_resultactors _returnvalue) (`EnvQueryInstanceBlueprintWrapper.GetQueryResultsAsActors` QueryInstance))
    (if _returnvalue
      (`self.OnSuccess` (`self._QueryInstance`) _resultactors)
      (else
        (`self.OnFailure` (`self._QueryInstance`) QueryStatus :!label _label)))
    (else
      (goto _label)))
  (`self.Deactivate`))

(event `self.Deactivate_BP`
  (`parent.Deactivate_BP`)
  (bind __queryinstance (`self._QueryInstance`)
    (:`then`
      (remove `EnvQueryInstanceBlueprintWrapper.OnQueryFinishedEvent` __queryinstance (`|CreateDelegate` :!event `OnEQSQueryFinished`)))
    (:`else`)))