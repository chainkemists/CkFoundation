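; A Blueprint task node that plays a float curve as a timeline on a CkFoundation ECS timer.
; Activation creates a timer on a transient entity, with duration from the curve's time range and TimeScale.
; Timer updates broadcast current and previous curve values with direction; completion fires OnDone and can deactivate the task, destroying both entities.
; Functions pause or resume the timer forwards, backwards or reversed, and a status string reports progress.
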(event `self.Activate_BP`
  (`parent.Activate_BP`)
  (`Ck_Utils_Ensure_UE.EnsureMsgf` (`Ck_Utils_RuntimeFloatCurve_UE.Get_IsValid` (`self.TimelineCurve`)) (`|FormatText` self "Invalid Timeline Curve supplied to [{self}]")
    (:`Valid`
      (bind _returnvalue (`Ck_Utils_EntityLifetime_UE.Request_CreateEntity_TransientOwner`))
      (set `self._NewEntityForTimer` _returnvalue)
      (bind _returnvalue_2 (`Ck_Utils_Timer_UE.Add` (`self._NewEntityForTimer`) (make `Ck_Fragment_Timer_ParamsData` (struct) (* (`Ck_Utils_Time_UE.Make_FromSeconds` (`._Max` (break `Ck_FloatRange` (`Ck_Utils_RuntimeFloatCurve_UE.Get_TimeRange` (`self.TimelineCurve`))))) (`self.TimeScale`)) "CountUp" "PauseOnDone" (`self.TimerStartingState`))))
      (bind _output_get (set `self._TimerEntity` _returnvalue_2))
      (bind _returnvalue_3 (`Ck_Utils_Timer_UE.BindTo_OnUpdate` _output_get (delegate `OnTimerUpdate`)))
      (`Ck_Utils_Timer_UE.BindTo_OnDone` _returnvalue_3 (delegate `OnTimerDone`)))))

(event `OnTimerDone`
  (params (InHandle :type "Ck_Handle_Timer Structure") (InChrono :type "Ck_Chrono Structure") (InDeltaT :type "Ck_Time Structure"))
  (`self.OnDone` (`Ck_Utils_Timer_UE.Get_CountDirection` InHandle))
  (switch `ECk_TaskDoneBehavior` (`self.TaskDoneBehavior`)
    (:`Deactivate`
      (`self.Deactivate`))))

(event `OnTimerUpdate`
  (params (InHandle :type "Ck_Handle_Timer Structure") (InChrono :type "Ck_Chrono Structure") (InDeltaT :type "Ck_Time Structure"))
  (set `self._PreviousValue` (`self._NewValue`))
  (set `self._NewValue` (`Ck_Utils_RuntimeFloatCurve_UE.Get_ValueAtTime` (`self.TimelineCurve`) (* (`.OutTimeElapsed` (`Ck_Utils_Chrono_UE.Break_Chrono` InChrono)) (`self.TimeScale`))))
  (`self.OnUpdate` (`self._NewValue`) (`self._PreviousValue`) (`Ck_Utils_Timer_UE.Get_CountDirection` InHandle)))

(event `self.Deactivate_BP`
  (`parent.Deactivate_BP`)
  (`|ExecutionSequence`
    (:`then_0`
      (`/CkFoundation/CkEcs/EntityHandle_CkEcs_ML.ValidateEntityHandle` (`self._TimerEntity`)
        (:`IsValid`
          (`Ck_Utils_Timer_UE.UnbindFrom_OnUpdate` (`self._TimerEntity`) (`|CreateDelegate` :!event `OnTimerUpdate`))
          (`Ck_Utils_Timer_UE.UnbindFrom_OnDone` (`self._TimerEntity`) (`|CreateDelegate` :!event `OnTimerDone`)))))
    (:`then_1`
      (`Ck_Utils_EntityLifetime_UE.Request_DestroyEntity` (`self._NewEntityForTimer`))
      (`Ck_Utils_EntityLifetime_UE.Request_DestroyEntity` (`self._TimerEntity`)))))

(fn `Get_StatusString_BP`
  (returns (ReturnValue :type String))
  (`/CkFoundation/CkEcs/EntityHandle_CkEcs_ML.ValidateEntityHandle` (`self._TimerEntity`)
    (:`IsValid`
      (return (`KismetTextLibrary.Conv_TextToString` (`|FormatText` "[{Direction}{state}] Progress: {elapsed} / {goal}" (select `bool` (`self._IsForwards`) :`false` "BACKWARD" :`true` "FORWARD") (select `ECk_Timer_State` (`Ck_Utils_Timer_UE.Get_CurrentState` (`self._TimerEntity`)) :`Paused` " | PAUSED") (`KismetTextLibrary.Conv_DoubleToText` (`/CkFoundation/CkTimer/Utils_CkTimer_FL.[Ck][Timer] Get Time Elapsed` (`self._TimerEntity`)) "HalfToEven" false true 1 324 0 1) (`/CkFoundation/CkTimer/Utils_CkTimer_FL.[Ck][Timer] Get Timer Goal` (`self._TimerEntity`))))))
    (:`NotValid`
      (return ""))))

(fn `Pause`
  (bind _outhandle (`/CkFoundation/CkEcs/EntityHandle_CkEcs_ML.ValidateEntityHandle` (`self._TimerEntity`))
    (:`IsValid`
      (`Ck_Utils_Timer_UE.Request_Pause` _outhandle))))

(fn `ResumeBackwards`
  (bind _outhandle (`/CkFoundation/CkEcs/EntityHandle_CkEcs_ML.ValidateEntityHandle` (`self._TimerEntity`))
    (:`IsValid`
      (`|ExecutionSequence`
        (:`then_0`
          (if (`self._IsForwards`)
            (set `self._IsForwards` false)
            (`Ck_Utils_Timer_UE.Request_ReverseDirection` _outhandle)))
        (:`then_1`
          (`Ck_Utils_Timer_UE.Request_Resume` _outhandle))))))

(fn `ResumeForward`
  (bind _outhandle (`/CkFoundation/CkEcs/EntityHandle_CkEcs_ML.ValidateEntityHandle` (`self._TimerEntity`))
    (:`IsValid`
      (`|ExecutionSequence`
        (:`then_0`
          (if (not (`self._IsForwards`))
            (set `self._IsForwards` true)
            (`Ck_Utils_Timer_UE.Request_ReverseDirection` _outhandle)))
        (:`then_1`
          (`Ck_Utils_Timer_UE.Request_Resume` _outhandle))))))

(fn `ResumeReversed`
  (bind _outhandle (`/CkFoundation/CkEcs/EntityHandle_CkEcs_ML.ValidateEntityHandle` (`self._TimerEntity`))
    (:`IsValid`
      (`|ExecutionSequence`
        (:`then_0`
          (set `self._IsForwards` (not (`self._IsForwards`)))
          (`Ck_Utils_Timer_UE.Request_ReverseDirection` _outhandle))
        (:`then_1`
          (`Ck_Utils_Timer_UE.Request_Resume` _outhandle))))))