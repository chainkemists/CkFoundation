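; Latent Blueprint task that interpolates an Actor's transform toward a goal over a set time, reporting each step rather than applying it directly in this graph.
; A component bitmask selects location, rotation or scale, with unselected parts keeping their initial values.
; A timer on a transient entity drives OnLerped with normalized elapsed time, then fires OnDone and deactivates.
; Invalid Actors or empty masks deactivate early, and deactivation destroys the timer entity.
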(event `self.Activate_BP`
  (`parent.Activate_BP`)
  (`Ck_Utils_Ensure_UE.EnsureMsgf_IsValid` (`self.Actor`) (`|FormatText` self "Invalid Actor supplied to [{self}]")
    (:`Valid`
      (bind _output_get (set `self._InitialTransform` (`Actor.GetTransform` (`self.Actor`))))
      (set `self._GoalLocation` (.location _output_get))
      (set `self._GoalRotation` (.rotation _output_get))
      (set `self._GoalScale` (.scale _output_get))
      (`|ExecutionSequence`
        (:`then_0`
          (bind _output_get_2 (set `self._ShouldLerpLocation` (`self.ShouldLerpTransformComponent` (enumliteral `ECk_TransformComponents` "Location"))))
          (if _output_get_2
            (set `self._GoalLocation` (.location (`self.GoalTransform`)))))
        (:`then_1`
          (bind _output_get_3 (set `self._ShouldLerpRotation` (`self.ShouldLerpTransformComponent` (enumliteral `ECk_TransformComponents` "Rotation"))))
          (if _output_get_3
            (set `self._GoalRotation` (.rotation (`self.GoalTransform`)))))
        (:`then_2`
          (bind _output_get_4 (set `self._ShouldLerpScale` (`self.ShouldLerpTransformComponent` (enumliteral `ECk_TransformComponents` "Scale"))))
          (if _output_get_4
            (set `self._GoalScale` (.scale (`self.GoalTransform`)))))
        (:`then_3`
          (`Ck_Utils_Ensure_UE.EnsureMsgf` (or (`self._ShouldLerpLocation`) (`self._ShouldLerpRotation`) (`self._ShouldLerpScale`)) (`|FormatText` self "Task [{self}] is setup to lerp NO Transform component for Actor [{actor}]" (`self.Actor`))
            (:`Valid`
              (bind _returnvalue (`Ck_Utils_EntityLifetime_UE.Request_CreateEntity_TransientOwner`))
              (bind _output_get_5 (set `self._EntityWithTimers` _returnvalue))
              (bind _outnewtimer (`/CkFoundation/CkTimer/Utils_CkTimer_FL.[Ck][Timer] Add New Timer` (struct) _output_get_5 (`self.LerpTime`) "PauseOnDone" "Running"))
              (bind (_taskobject _timerupdate_outtimerentity _timerupdate_outtimerchrono) (`|Blueprint_Template` _outnewtimer)
                (:`then`
                  (`self.DoRequest_AddTaskToDeactivateOnDeactivate` _taskobject)
                  (bind _taskobject_2 (`|Blueprint_Template` _outnewtimer)
                    (:`then`
                      (`self.DoRequest_AddTaskToDeactivateOnDeactivate` _taskobject_2))
                    (:`TimerDone`
                      (`self.OnDone` (`self.Actor`))
                      (`self.Deactivate`))))
                (:`TimerUpdate`
                  (bind _returnvalue__seconds (break `Ck_Time` (`Ck_Utils_Chrono_UE.Get_TimeElapsed` _timerupdate_outtimerchrono "ZeroToOne")))
                  (`self.OnLerped` (`self.Actor`) (`KismetMathLibrary.TLerp` (`self._InitialTransform`) (`KismetMathLibrary.MakeTransform` (`self._GoalLocation`) (`self._GoalRotation`) (`self._GoalScale`)) _returnvalue__seconds)))))
            (:`Invalid`
              (`self.Deactivate`))))))
    (:`Invalid`
      (`self.Deactivate`))))

(event `self.Deactivate_BP`
  (`parent.Deactivate_BP`)
  (`Ck_Utils_EntityLifetime_UE.Request_DestroyEntity` (`self._EntityWithTimers`)))