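; A CkFoundation task that reports a Controller's initial and changed possessed pawn once that pawn's replication is complete.
; For a valid pawn, each event starts a nested task, registers it to deactivate with this one, and waits for Replication Complete All Dependents.
; It then broadcasts the pawn, re-derived from the entity's owning actor, along with that entity.
; An invalid pawn is broadcast immediately without an entity.
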(event `self.OnPossessedPawnChanged`
  (params (OldPawn :type "Pawn Object Reference") (NewPawn :type "Pawn Object Reference"))
  (`/Engine/EditorBlueprintResources/StandardMacros.IsValid` NewPawn
    (:`Is Valid`
      (bind (_taskobject _onreplicationcomplete_alldependents_outentity) (`|Blueprint_Template` NewPawn)
        (:`then`
          (`self.DoRequest_AddTaskToDeactivateOnDeactivate` _taskobject))
        (:`OnReplicationComplete_AllDependents`
          (bind _aspawn (cast `Pawn` (`Ck_Utils_OwningActor_UE.Get_EntityOwningActor` _onreplicationcomplete_alldependents_outentity)))
          (`self.PossessedPawnChanged (Replication Complete)` (`self.Controller`) OldPawn _aspawn _onreplicationcomplete_alldependents_outentity))))
    (:`Is Not Valid`
      (`self.PossessedPawnChanged (Replication Complete)` (`self.Controller`) OldPawn NewPawn))))

(event `self.OnInitialPossessedPawn`
  (params (InController :type "Controller Object Reference") (InCurrentPawn :type "Pawn Object Reference"))
  (`/Engine/EditorBlueprintResources/StandardMacros.IsValid` InCurrentPawn
    (:`Is Valid`
      (bind (_taskobject _onreplicationcomplete_alldependents_outentity) (`|Blueprint_Template` InCurrentPawn)
        (:`then`
          (`self.DoRequest_AddTaskToDeactivateOnDeactivate` _taskobject))
        (:`OnReplicationComplete_AllDependents`
          (bind _aspawn (cast `Pawn` (`Ck_Utils_OwningActor_UE.Get_EntityOwningActor` _onreplicationcomplete_alldependents_outentity)))
          (`self.InitialPossessedPawn (Replication Complete)` (`self.Controller`) _aspawn _onreplicationcomplete_alldependents_outentity))))
    (:`Is Not Valid`
      (`self.InitialPossessedPawn (Replication Complete)` (`self.Controller`) InCurrentPawn))))