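; Blueprint task node that waits for a Controller's possessed pawn to change and reports each change with the old and new pawn.
; On activation it validates the Controller, deactivating if invalid, then binds to OnPossessedPawnChanged and immediately reports the currently controlled pawn through a separate InitialPossessedPawn output.
; It stays active across changes and unbinds from the Controller on deactivation if that is still valid.
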(event `self.Activate_BP`
  (`parent.Activate_BP`)
  (`Ck_Utils_Ensure_UE.EnsureMsgf_IsValid` (`self.Controller`) (`|FormatText` self "Invalid Controller supplied to [{self}]")
    (:`Valid`
      (add `Controller.OnPossessedPawnChanged` (`self.Controller`) (delegate `OnPossessedPawnChanged`))
      (`self.OnInitialPossessedPawn` (`self.Controller`) (`Controller.K2_GetPawn` (`self.Controller`))))
    (:`Invalid`
      (`self.Deactivate`))))

(event `OnPossessedPawnChanged`
  (params (OldPawn :type "Pawn Object Reference") (NewPawn :type "Pawn Object Reference"))
  (`self.PossessedPawnChanged` (`self.Controller`) OldPawn NewPawn))

(event `OnInitialPossessedPawn`
  (params (InController :type "Controller Object Reference") (InCurrentPawn :type "Pawn Object Reference"))
  (`self.InitialPossessedPawn` InController InCurrentPawn))

(event `self.Deactivate_BP`
  (`parent.Deactivate_BP`)
  (bind _controller (`self.Controller`)
    (:`then`
      (remove `Controller.OnPossessedPawnChanged` _controller (`|CreateDelegate` :!event `OnPossessedPawnChanged`)))
    (:`else`)))