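; Blueprint task node that waits on a RaySense entity and relays its trace hits through the task's OnTraceHit output.
; On activation it binds to the entity's hit signal, or deactivates with an ensure message if the handle is invalid.
; The binding also fires for a payload already in flight this frame and does nothing after firing, so hits can repeat.
; Deactivation unbinds if the handle is still valid.
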(event `self.Activate_BP`
  (`parent.Activate_BP`)
  (`Ck_Utils_EcsEnsure_UE.EnsureMsgf_IsValid` (`self.RaySense`) (`|FormatText` self "Invalid RaySense entity supplied to [{self}]")
    (:`Valid`
      (`Ck_Utils_RaySense_UE.BindTo_OnTraceHit` (`self.RaySense`) "FireIfPayloadInFlightThisFrame" "DoNothing" (delegate `OnRaySenseTraceHit`)))
    (:`Invalid`
      (`self.Deactivate`))))

(event `OnRaySenseTraceHit`
  (params (InHandle :type "Ck_Handle_RaySense Structure") (InHitResult :type "Ck_RaySense_HitResult Structure"))
  (`self.OnTraceHit` InHandle InHitResult))

(event `self.Deactivate_BP`
  (`parent.Deactivate_BP`)
  (bind _outhandle (`/CkFoundation/CkEcs/EntityHandle_CkEcs_ML.ValidateEntityHandle` (`self.RaySense`))
    (:`IsValid`
      (`Ck_Utils_RaySense_UE.UnbindFrom_OnTraceHit` _outhandle (`|CreateDelegate` :!event `OnRaySenseTraceHit`)))))