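; Blueprint task node that waits for a target actor's ECS entity replication to complete, firing events for the entity and for all its dependents.
; After the actor begins play, it binds replication promises immediately if the EntityBridge component reports completion, or waits on that component's delegate.
; Without a bridge component it signals NotEcsReady and deactivates.
; It also deactivates once all dependents finish, unbinding the delegate.
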(event `self.Activate_BP`
  (`parent.Activate_BP`)
  (`Ck_Utils_Ensure_UE.EnsureMsgf_IsValid` (`self.TargetActor`) (`|FormatText` self "Invalid Target Actor supplied to [{self}] ")
    (:`Valid`
      (bind (_taskobject _onactorbegunplay_outactor) (`|Blueprint_Template` (`self.TargetActor`))
        (:`then`
          (`self.DoRequest_AddTaskToDeactivateOnDeactivate` _taskobject))
        (:`OnActorBegunPlay`
          (set `self._EntityBridgeComp` (`Actor.GetComponentByClass` _onactorbegunplay_outactor "/Script/CkEntityBridge.Ck_EntityBridge_ActorComponent_UE"))
          (`/Engine/EditorBlueprintResources/StandardMacros.IsValid` (`self._EntityBridgeComp`)
            (:`Is Valid`
              (if (`Ck_EntityBridge_ActorComponent_UE.Get_IsReplicationComplete` (`self._EntityBridgeComp`))
                (`self.BindToReplicationComplete_Promises` (`Ck_Utils_OwningActor_UE.Get_ActorEntityHandle` (`self.TargetActor`)))
                (else
                  (add `Ck_EntityBridge_ActorComponent_UE._OnReplicationComplete_MC` (`self._EntityBridgeComp`) (delegate `EntityBridge_ReplicationComplete`)))))
            (:`Is Not Valid`
              (`self.NotEcsReady`)
              (`self.Deactivate`))))))
    (:`Invalid`
      (`self.Deactivate`))))

(event `BindToReplicationComplete_Promises`
  (params (InEntity :type "Ck_Handle Structure"))
  ;[0.9688 1 0] BindToReplicationComplete_Promises
  (`Ck_Utils_EntityReplicationDriver_UE.Promise_OnReplicationComplete` InEntity (`|CreateDelegate` :!event `ReplicationComplete`))
  (`Ck_Utils_EntityReplicationDriver_UE.Promise_OnReplicationCompleteAllDependents` InEntity (`|CreateDelegate` :!event `ReplicationComplete_AllDependents`)))

(event `EntityBridge_ReplicationComplete`
  (params (InEntity :type "Ck_Handle Structure"))
  (bind _outhandle (`/CkFoundation/CkEcs/EntityHandle_CkEcs_ML.ValidateEntityHandle` InEntity)
    (:`IsValid`
      (`self.BindToReplicationComplete_Promises` _outhandle))))

(event `self.Deactivate_BP`
  (`parent.Deactivate_BP`)
  (bind __entitybridgecomp (`self._EntityBridgeComp`)
    (:`then`
      (remove `Ck_EntityBridge_ActorComponent_UE._OnReplicationComplete_MC` __entitybridgecomp (`|CreateDelegate` :!event `EntityBridge_ReplicationComplete`)))
    (:`else`)))

(event `ReplicationComplete`
  (params (InHandle :type "Ck_Handle Structure"))
  ;[0.6172 0 1] ReplicationComplete
  (`self.OnReplicationComplete` InHandle))

(event `ReplicationComplete_AllDependents`
  (params (InHandle :type "Ck_Handle Structure"))
  ;[1 0 0.375] ReplicationComplete_AllDependents
  (`self.OnReplicationComplete_AllDependents` InHandle)
  (`self.Deactivate`))