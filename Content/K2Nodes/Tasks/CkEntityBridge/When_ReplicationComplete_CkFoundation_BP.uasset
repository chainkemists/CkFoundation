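; Blueprint task node in CkFoundation's entity bridge that notifies callers when a target entity finishes replicating.
; On activation it ensures the target handle is valid, warning that Actors may be calling too early and should use OnReplicationComplete instead of BeginPlay.
; It then registers two promises, one for the entity and one for all its dependents, each firing its matching output event.
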(event `self.Activate_BP`
  (`parent.Activate_BP`)
  (`Ck_Utils_Ensure_UE.EnsureMsgf` (`Ck_Utils_Handle_UE.Get_Handle_IsValid` (`self.TargetEntity`)) (`|FormatText` self "Invalid Target Entity supplied to [{self}]. \n \nIf this is used in an Actor, was this called too early ? OnReplicationComplete event should be used over BeginPlay ")
    (:`Valid`
      (`Ck_Utils_EntityReplicationDriver_UE.Promise_OnReplicationComplete` (`self.TargetEntity`) (delegate `ReplicationComplete`))
      (`Ck_Utils_EntityReplicationDriver_UE.Promise_OnReplicationCompleteAllDependents` (`self.TargetEntity`) (delegate `ReplicationComplete_AllDependents`)))))

(event `ReplicationComplete`
  (params (InHandle :type "Ck_Handle Structure"))
  (`self.OnReplicationComplete`))

(event `ReplicationComplete_AllDependents`
  (params (InHandle :type "Ck_Handle Structure"))
  (`self.OnReplicationComplete_AllDependents`))