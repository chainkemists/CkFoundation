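; Latent Blueprint task node that waits for status changes on a CkFoundation Objective handle.
; On activation it validates the handle, binds to its status-changed delegate and immediately fires the status-now output with the current status.
; Each later change is forwarded to the status-changed output, and deactivation unbinds if the handle is still valid.
; A status string reports the lifetime owner, objective and status.
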(event `self.Activate_BP`
  (`parent.Activate_BP`)
  (`Ck_Utils_Ensure_UE.EnsureMsgf` (`Ck_Utils_Handle_UE.Get_IsValid` (`self.ObjectiveHandle`)) (`|FormatText` self "Invalid Objective handle supplied to [{self}]")
    (:`Valid`
      (`Ck_Utils_Objective_UE.BindTo_OnStatusChanged` (`self.ObjectiveHandle`) (delegate `OnObjective_StatusChanged`))
      (`self.ObjectiveStatusNow` (`self.ObjectiveHandle`) (`Ck_Utils_Objective_UE.Get_Status` (`self.ObjectiveHandle`))))))

(event `OnObjective_StatusChanged`
  (params (InObjective :type "Ck_Handle_Objective Structure") (InNewStatus :type "ECk_ObjectiveStatus Enum" :default "NotStarted"))
  (`self.ObjectiveStatusChanged` InObjective InNewStatus))

(event `self.Deactivate_BP`
  (`parent.Deactivate_BP`)
  (bind _outhandle (`/CkFoundation/CkEcs/EntityHandle_CkEcs_ML.ValidateEntityHandle` (`self.ObjectiveHandle`))
    (:`IsValid`
      (`Ck_Utils_Objective_UE.UnbindFrom_OnStatusChanged` _outhandle (`|CreateDelegate` :!event `OnObjective_StatusChanged`)))))

(fn `Get_StatusString_BP`
  (returns (ReturnValue :type String))
  (`/CkFoundation/CkEcs/EntityHandle_CkEcs_ML.ValidateEntityHandle` (`self.ObjectiveHandle`)
    (:`IsValid`
      (return (`KismetTextLibrary.Conv_TextToString` (`|FormatText` "{owner} \n{objective} \n{status}" (`Ck_Utils_Handle_UE.Conv_HandleToString` (`Ck_Utils_EntityLifetime_UE.Get_LifetimeOwner` (`self.ObjectiveHandle`))) (`Ck_Utils_Handle_UE.Conv_HandleToString` (`self.ObjectiveHandle`)) (`|GetEnumeratorNameAsString` (`Ck_Utils_Objective_UE.Get_Status` (`self.ObjectiveHandle`)))))))
    (:`NotValid`
      (return "Invalid Sensor Entity"))))