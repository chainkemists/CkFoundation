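; Blueprint task node that waits for progress updates on a CkFoundation Objective and relays them through ObjectiveProgressUpdated.
; On activation it ensures the handle is valid and binds to progress changes, also firing for a payload in flight this frame.
; Each update forwards objective, metadata, and old and new progress; deactivation unbinds if the handle is valid.
; Its status string shows the objective's lifetime owner, handle and status.
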(event `self.Activate_BP`
  (`parent.Activate_BP`)
  (`Ck_Utils_Ensure_UE.EnsureMsgf` (`Ck_Utils_Handle_UE.Get_IsValid` (`self.ObjectiveHandle`)) (`|FormatText` self "Invalid Objective handle supplied to [{self}]")
    (:`Valid`
      (`Ck_Utils_Objective_UE.BindTo_OnProgressChanged` (`self.ObjectiveHandle`) "FireIfPayloadInFlightThisFrame" "DoNothing" (delegate `OnObjective_ProgressUpdated`)))))

(event `OnObjective_ProgressUpdated`
  (params (InObjective :type "Ck_Handle_Objective Structure") (InMetaData :type "GameplayTag Structure") (InOldProgress :type Integer) (InNewProgress :type Integer))
  (`self.ObjectiveProgressUpdated` InObjective InMetaData InOldProgress InNewProgress))

(event `self.Deactivate_BP`
  (`parent.Deactivate_BP`)
  (bind _outhandle (`/CkFoundation/CkEcs/EntityHandle_CkEcs_ML.ValidateEntityHandle` (`self.ObjectiveHandle`))
    (:`IsValid`
      (`Ck_Utils_Objective_UE.UnbindFrom_OnProgressChanged` _outhandle (`|CreateDelegate` :!event `OnObjective_ProgressUpdated`)))))

(fn `Get_StatusString_BP`
  (returns (ReturnValue :type String))
  (`/CkFoundation/CkEcs/EntityHandle_CkEcs_ML.ValidateEntityHandle` (`self.ObjectiveHandle`)
    (:`IsValid`
      (return (`KismetTextLibrary.Conv_TextToString` (`|FormatText` "{owner} \n{objective} \n{status}" (`Ck_Utils_Handle_UE.Conv_HandleToString` (`Ck_Utils_EntityLifetime_UE.Get_LifetimeOwner` (`self.ObjectiveHandle`))) (`Ck_Utils_Handle_UE.Conv_HandleToString` (`self.ObjectiveHandle`)) (`|GetEnumeratorNameAsString` (`Ck_Utils_Objective_UE.Get_Status` (`self.ObjectiveHandle`)))))))
    (:`NotValid`
      (return "Invalid Sensor Entity"))))