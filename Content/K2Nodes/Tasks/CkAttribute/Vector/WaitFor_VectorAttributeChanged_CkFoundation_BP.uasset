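; Blueprint async task node that waits for changes to a Vector attribute on an entity, for the Ck attribute system.
; On activation it ensures the attribute handle is valid, then binds to value changes, also firing for a change already in flight that frame.
; Each change is relayed with owner, attribute and current and previous base and final values.
; Deactivation unbinds, and the status string shows the attribute's label.
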(event `self.Activate_BP`
  (`parent.Activate_BP`)
  (`Ck_Utils_Ensure_UE.EnsureMsgf` (`Ck_Utils_Handle_UE.Get_IsValid` (`self.AttributeHandle`)) (`|FormatText` self "Invalid Vector Attribute handle supplied to [{self}]")
    (:`Valid`
      (`Ck_Utils_VectorAttribute_UE.BindTo_OnValueChanged` (`self.AttributeHandle`) (`self.AttributeComponent`) "FireIfPayloadInFlightThisFrame" "DoNothing" (delegate `OnAttributeChanged`)))))

(event `OnAttributeChanged`
  (params (InAttributeOwnerEntity :type "Ck_Handle Structure") (InPayload :type "Ck_Payload_VectorAttribute_OnValueChanged Structure"))
  (bind (__attributeentity __basevalue __finalvalue __basevalue_previous __finalvalue_previous) (break `Ck_Payload_VectorAttribute_OnValueChanged` InPayload))
  (`self.AttributeChanged` InAttributeOwnerEntity __attributeentity __basevalue __finalvalue __basevalue_previous __finalvalue_previous))

(event `self.Deactivate_BP`
  (`parent.Deactivate_BP`)
  (bind _outhandle (`/CkFoundation/CkEcs/EntityHandle_CkEcs_ML.ValidateEntityHandle` (`self.AttributeHandle`))
    (:`IsValid`
      (`Ck_Utils_VectorAttribute_UE.UnbindFrom_OnValueChanged` _outhandle (`self.AttributeComponent`) (`|CreateDelegate` :!event `OnAttributeChanged`)))))

(fn `Get_StatusString_BP`
  (returns (ReturnValue :type String))
  (bind _outhandle (`/CkFoundation/CkEcs/EntityHandle_CkEcs_ML.ValidateEntityHandle` (`self.AttributeHandle`))
    (:`IsValid`
      (return (`KismetStringLibrary.Conv_NameToString` (`BlueprintGameplayTagLibrary.GetTagName` (`Ck_Utils_GameplayLabel_UE.Get_Label` _outhandle)))))
    (:`NotValid`
      (return "Invalid VectorAttribute Entity"))))