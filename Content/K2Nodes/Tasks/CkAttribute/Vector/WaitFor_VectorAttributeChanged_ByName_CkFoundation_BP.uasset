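; Async task node that watches a named Vector attribute on an entity and reports changes to one component's base and final values.
; On binding it fires AttributeNow with current values, then relays each change with previous values as AttributeChanged.
; ExtensionAwareness selects a one-time lookup with an ensure, or retries on extension added (and removed, when repeating), firing AttributeDoesNotExist on failure.
; Deactivation unbinds delegates, and a status string reports binding state.
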(event `BindToOnValueChanged`
  (params (InAttribute :type "Ck_Handle_VectorAttribute Structure (by ref)"))
  (bind _returnvalue (`Ck_Utils_VectorAttribute_UE.BindTo_OnValueChanged` InAttribute (`self.AttributeComponent`) "FireIfPayloadInFlightThisFrame" "DoNothing" (delegate `OnAttributeChanged`)))
  (`self.AttributeNow` (`Ck_Utils_EntityLifetime_UE.Get_LifetimeOwner` _returnvalue) _returnvalue (`Ck_Utils_VectorAttribute_UE.Get_BaseValue` _returnvalue (`self.AttributeComponent`)) (`Ck_Utils_VectorAttribute_UE.Get_FinalValue` _returnvalue (`self.AttributeComponent`))))

(event `OnAttributeChanged`
  (params (InAttributeOwnerEntity :type "Ck_Handle Structure") (InPayload :type "Ck_Payload_VectorAttribute_OnValueChanged Structure"))
  (bind (__attributeentity __basevalue __finalvalue __basevalue_previous __finalvalue_previous) (break `Ck_Payload_VectorAttribute_OnValueChanged` InPayload))
  (`self.AttributeChanged` InAttributeOwnerEntity __attributeentity __basevalue __finalvalue __basevalue_previous __finalvalue_previous))

(event `UnbindFromOnValueChanged`
  (params (InAttribute :type "Ck_Handle_VectorAttribute Structure (by ref)"))
  (`Ck_Utils_VectorAttribute_UE.UnbindFrom_OnValueChanged` InAttribute (`self.AttributeComponent`) (delegate `OnAttributeChanged`)))

(event `TryToBindToHandle`
  (bind _outhandle (`/CkFoundation/CkEcs/EntityHandle_CkEcs_ML.ValidateEntityHandle` (`self._AttributeHandle`))
    (:`IsValid`
      (`self.UnbindFromOnValueChanged` _outhandle))
    (:`NotValid`
      _))
  (bind _output_get (set `self._AttributeHandle` (`Ck_Utils_VectorAttribute_UE.TryGet` (`self.AttributeOwnerEntity`) (`self.AttributeName`))))
  (bind _outhandle_2 (`/CkFoundation/CkEcs/EntityHandle_CkEcs_ML.ValidateEntityHandle` _output_get)
    (:`IsValid`
      (`self.BindToOnValueChanged` _outhandle_2)
      (switch `ECk_ExtensionAwareness` (`self.ExtensionAwareness`)
        (:`WaitAndBind_OnFirstAvailable`
          (`Ck_Utils_EntityExtension_UE.UnbindFrom_OnExtensionAdded` (`self.AttributeOwnerEntity`) (`|CreateDelegate` :!event `OnExtensionAdded`)))))
    (:`NotValid`
      (`self.AttributeDoesNotExist` (`self.AttributeName`)))))

(event `self.Activate_BP`
  (`parent.Activate_BP`)
  (switch `ECk_ExtensionAwareness` (`self.ExtensionAwareness`)
    (:`None`
      (set `self._AttributeHandle` (`Ck_Utils_VectorAttribute_UE.TryGet` (`self.AttributeOwnerEntity`) (`self.AttributeName`)))
      (`Ck_Utils_Ensure_UE.EnsureMsgf` (`Ck_Utils_Handle_UE.Get_IsValid` (`self._AttributeHandle`)) (`|FormatText` self "Could NOT find Float Attribute with Name [{name}] in Entity [{owner}] in [{self}]" (`BlueprintGameplayTagLibrary.GetTagName` (`self.AttributeName`)) (`Ck_Utils_Handle_UE.Conv_HandleToText` (`self.AttributeOwnerEntity`)))
        (:`Valid`
          (`self.BindToOnValueChanged` (`self._AttributeHandle`)))))
    (:`WaitAndBind_OnFirstAvailable`
      (`self.BindOn_ExtensionAdded`))
    (:`WaitAndBind_Repeatedly`
      (`self.BindOn_ExtensionRemovedAndAdded`))))

(event `BindOn_ExtensionAdded`
  ;[0 0 0] BindOn_ExtensionAdded
  (`Ck_Utils_EntityExtension_UE.BindTo_OnExtensionAdded` (`self.AttributeOwnerEntity`) "FireIfPayloadInFlightThisFrame" "DoNothing" (delegate `OnExtensionAdded`))
  (`self.TryToBindToHandle`))

(event `self.Deactivate_BP`
  (`parent.Deactivate_BP`)
  (`|ExecutionSequence`
    (:`then_0`
      (bind _outhandle (`/CkFoundation/CkEcs/EntityHandle_CkEcs_ML.ValidateEntityHandle` (`self._AttributeHandle`))
        (:`IsValid`
          (`self.UnbindFromOnValueChanged` _outhandle))))
    (:`then_1`
      (switch `ECk_ExtensionAwareness` (`self.ExtensionAwareness`)
        (:`WaitAndBind_OnFirstAvailable`
          _)
        (:`WaitAndBind_Repeatedly`
          _))
      (`Ck_Utils_EntityExtension_UE.UnbindFrom_OnExtensionAdded` (`self.AttributeOwnerEntity`) (`|CreateDelegate` :!event `OnExtensionAdded`))
      (`Ck_Utils_EntityExtension_UE.UnbindFrom_OnExtensionRemoved` (`self.AttributeOwnerEntity`) (`|CreateDelegate` :!event `OnExtensionRemoved`)))))

(event `OnExtensionAdded`
  (params (InExtensionOwner :type "Ck_Handle Structure") (InEntityAsExtension :type "Ck_Handle_EntityExtension Structure"))
  (`self.TryToBindToHandle`))

(event `BindOn_ExtensionRemovedAndAdded`
  ;[0 0 0] BindOn_ExtensionRemoved
  (`Ck_Utils_EntityExtension_UE.BindTo_OnExtensionRemoved` (`self.AttributeOwnerEntity`) "FireIfPayloadInFlightThisFrame" "DoNothing" (delegate `OnExtensionRemoved`))
  (`self.BindOn_ExtensionAdded`))

(event `OnExtensionRemoved`
  (params (InExtensionOwner :type "Ck_Handle Structure") (InEntityAsExtension :type "Ck_Handle_EntityExtension Structure"))
  (`self.TryToBindToHandle`))

(fn `Get_StatusString_BP`
  (returns (ReturnValue :type String))
  (`/CkFoundation/CkEcs/EntityHandle_CkEcs_ML.ValidateEntityHandle` (`self.AttributeOwnerEntity`)
    (:`IsValid`
      (`/CkFoundation/CkEcs/EntityHandle_CkEcs_ML.ValidateEntityHandle` (`self._AttributeHandle`)
        (:`IsValid`
          (return (`KismetTextLibrary.Conv_TextToString` (`|FormatText` "{owner} \n{attribute} \n{comp}: {val}" (`Ck_Utils_Handle_UE.Conv_HandleToString` (`self.AttributeOwnerEntity`)) (`Ck_Utils_Handle_UE.Conv_HandleToString` (`self._AttributeHandle`)) (`|GetEnumeratorNameAsString` (`self.AttributeComponent`)) (`KismetStringLibrary.Conv_VectorToString` (`Ck_Utils_VectorAttribute_UE.Get_FinalValue` (`self._AttributeHandle`) (`self.AttributeComponent`)))))))
        (:`NotValid`
          (switch `ECk_ExtensionAwareness` (`self.ExtensionAwareness`)
            (:`None`
              (return (`KismetTextLibrary.Conv_TextToString` (`|FormatText` "{owner} \nAttribute [{attribute}] not found!" (`Ck_Utils_Handle_UE.Conv_HandleToString` (`self.AttributeOwnerEntity`)) (`BlueprintGameplayTagLibrary.GetTagName` (`self.AttributeName`))))))
            (:`WaitAndBind_OnFirstAvailable`
              _)
            (:`WaitAndBind_Repeatedly`
              _))
          (return (`KismetTextLibrary.Conv_TextToString` (`|FormatText` "{owner} \nWaiting to bind on [{attribute}]..." (`Ck_Utils_Handle_UE.Conv_HandleToString` (`self.AttributeOwnerEntity`)) (`BlueprintGameplayTagLibrary.GetTagName` (`self.AttributeName`))))))))
    (:`NotValid`
      (return "Invalid AttributeOwner"))))