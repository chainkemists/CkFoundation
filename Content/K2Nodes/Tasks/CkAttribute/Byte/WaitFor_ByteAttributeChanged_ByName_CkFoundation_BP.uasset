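; Task Blueprint for waiting on a change to a Byte Attribute that is identified by name on an owner entity.
; On activation it resolves the attribute handle from the owner entity and name tag, then ensures it is valid.
; Only a valid handle passes on to the parent activation, and a failed lookup reports the name and owner.
; Deactivation simply defers to the parent.
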(event `self.Activate_BP`
  (set `self.AttributeHandle` (`Ck_Utils_ByteAttribute_UE.TryGet` (`self.AttributeOwnerEntity`) (`self.AttributeName`)))
  (`Ck_Utils_Ensure_UE.EnsureMsgf` (`Ck_Utils_Handle_UE.Get_IsValid` (`self.AttributeHandle`)) (`|FormatText` self "Could NOT find Byte Attribute with Name [{name}] in Entity [{owner}] in [{self}]" (`BlueprintGameplayTagLibrary.GetTagName` (`self.AttributeName`)) (`Ck_Utils_Handle_UE.Conv_HandleToText` (`self.AttributeOwnerEntity`)))
    (:`Valid`
      (`parent.Activate_BP`))))

(event `self.Deactivate_BP`
  (`parent.Deactivate_BP`))