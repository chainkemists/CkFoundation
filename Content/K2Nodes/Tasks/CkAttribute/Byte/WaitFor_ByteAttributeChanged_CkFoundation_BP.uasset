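; Blueprint task node from CkFoundation that reports value changes on a Byte attribute.
; On activation it ensures the attribute handle is valid and binds to value changes for the given component, also firing for a payload in flight this frame.
; Each change is relayed through AttributeChanged with the owner, attribute handle, base value and final value.
; Deactivation unbinds if the handle is still valid.
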(event `self.Activate_BP`
  (`parent.Activate_BP`)
  (`Ck_Utils_Ensure_UE.EnsureMsgf` (`Ck_Utils_Handle_UE.Get_IsValid` (`self.AttributeHandle`)) (`|FormatText` self "Invalid Byte Attribute handle supplied to [{self}]")
    (:`Valid`
      (`Ck_Utils_ByteAttribute_UE.BindTo_OnValueChanged` (`self.AttributeHandle`) (`self.AttributeComponent`) "FireIfPayloadInFlightThisFrame" "DoNothing" (delegate `OnAttributeChanged`)))))

(event `OnAttributeChanged`
  (params (InAttributeOwnerEntity :type "Ck_Handle Structure") (InPayload :type "Ck_Payload_ByteAttribute_OnValueChanged Structure"))
  (bind (__attributeentity __basevalue __finalvalue) (break `Ck_Payload_ByteAttribute_OnValueChanged` InPayload))
  (`self.AttributeChanged` InAttributeOwnerEntity __attributeentity __basevalue __finalvalue))

(event `self.Deactivate_BP`
  (`parent.Deactivate_BP`)
  (bind _outhandle (`/CkFoundation/CkEcs/EntityHandle_CkEcs_ML.ValidateEntityHandle` (`self.AttributeHandle`))
    (:`IsValid`
      (`Ck_Utils_ByteAttribute_UE.UnbindFrom_OnValueChanged` _outhandle (`self.AttributeComponent`) (`|CreateDelegate` :!event `OnAttributeChanged`)))))