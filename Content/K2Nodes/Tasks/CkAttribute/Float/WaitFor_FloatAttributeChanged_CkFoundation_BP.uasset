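; Blueprint async task node that waits for changes to a component of a float attribute and re-broadcasts each change.
; On activation it ensures the attribute handle is valid and binds to its value-changed delegate, also firing for payloads already in flight that frame.
; Each change forwards the owner, attribute, and current and previous base and final values; deactivation unbinds.
; A status string reports owner, attribute, component and final value.
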(event `self.Activate_BP`
  (`parent.Activate_BP`)
  (`Ck_Utils_Ensure_UE.EnsureMsgf` (`Ck_Utils_Handle_UE.Get_IsValid` (`self.AttributeHandle`)) (`|FormatText` self "Invalid Float Attribute handle supplied to [{self}]")
    (:`Valid`
      (`Ck_Utils_FloatAttribute_UE.BindTo_OnValueChanged` (`self.AttributeHandle`) (`self.AttributeComponent`) "FireIfPayloadInFlightThisFrame" "DoNothing" (delegate `OnAttributeChanged`)))))

(event `OnAttributeChanged`
  (params (InAttributeOwnerEntity :type "Ck_Handle Structure") (InPayload :type "Ck_Payload_FloatAttribute_OnValueChanged Structure"))
  (bind (__attributeentity __basevalue __finalvalue __basevalue_previous __finalvalue_previous) (break `Ck_Payload_FloatAttribute_OnValueChanged` InPayload))
  (`self.AttributeChanged` InAttributeOwnerEntity __attributeentity __basevalue __finalvalue __basevalue_previous __finalvalue_previous))

(event `self.Deactivate_BP`
  (`parent.Deactivate_BP`)
  (bind _outhandle (`/CkFoundation/CkEcs/EntityHandle_CkEcs_ML.ValidateEntityHandle` (`self.AttributeHandle`))
    (:`IsValid`
      (`Ck_Utils_FloatAttribute_UE.UnbindFrom_OnValueChanged` _outhandle (`self.AttributeComponent`) (`|CreateDelegate` :!event `OnAttributeChanged`)))))

(fn `Get_StatusString_BP`
  (returns (ReturnValue :type String))
  (`/CkFoundation/CkEcs/EntityHandle_CkEcs_ML.ValidateEntityHandle` (`self.AttributeHandle`)
    (:`IsValid`
      (return (`KismetTextLibrary.Conv_TextToString` (`|FormatText` "{owner} \n{attribute} \n{comp}: {val}" (`Ck_Utils_Handle_UE.Conv_HandleToString` (`Ck_Utils_EntityLifetime_UE.Get_LifetimeOwner` (`self.AttributeHandle`))) (`Ck_Utils_Handle_UE.Conv_HandleToString` (`self.AttributeHandle`)) (`|GetEnumeratorNameAsString` (`self.AttributeComponent`)) (`Ck_Utils_FloatAttribute_UE.Get_FinalValue` (`self.AttributeHandle`) (`self.AttributeComponent`))))))
    (:`NotValid`
      (return "Invalid Attribute Entity"))))