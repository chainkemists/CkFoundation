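; Blueprint task node that watches a CkFoundation float attribute and reports its Current-to-Max ratio as it changes.
; On activation it ensures a valid handle with a Max component, broadcasts the initial ratio, then binds to changes on both components.
; Either change recomputes Current / Max and broadcasts it with the previous value.
; Deactivation unbinds, and a status string shows owner, attribute and values.
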(event `self.Activate_BP`
  (`parent.Activate_BP`)
  (`Ck_Utils_Ensure_UE.EnsureMsgf` (`Ck_Utils_Handle_UE.Get_IsValid` (`self.AttributeHandle`)) (`|FormatText` self "Invalid Float Attribute handle supplied to [{self}]")
    (:`Valid`
      (`Ck_Utils_Ensure_UE.EnsureMsgf` (`Ck_Utils_FloatAttribute_UE.Has_Component` (`self.AttributeHandle`) "Max") (`|FormatText` self "Float Attribute [{entity}] supplied to [{self}] does NOT have a MAX component" (`Ck_Utils_Handle_UE.Conv_HandleToText` (`self.AttributeHandle`)))
        (:`Valid`
          (`|ExecutionSequence`
            (:`then_0`
              (set `self._Current` (`Ck_Utils_FloatAttribute_UE.Get_FinalValue` (`self.AttributeHandle`)))
              (set `self._Max` (`Ck_Utils_FloatAttribute_UE.Get_FinalValue` (`self.AttributeHandle`) "Max"))
              (`self.DoNotifyInitialAttributeValue`))
            (:`then_1`
              (`Ck_Utils_FloatAttribute_UE.BindTo_OnValueChanged` (`self.AttributeHandle`) "Current" "FireIfPayloadInFlightThisFrame" "DoNothing" (delegate `OnAttributeChanged_Current`))
              (`Ck_Utils_FloatAttribute_UE.BindTo_OnValueChanged` (`self.AttributeHandle`) "Max" "FireIfPayloadInFlightThisFrame" "DoNothing" (delegate `OnAttributeChanged_Max`)))))))))

(event `OnAttributeChanged_Max`
  (params (InAttributeOwnerEntity :type "Ck_Handle Structure") (InPayload :type "Ck_Payload_FloatAttribute_OnValueChanged Structure"))
  (bind (__attributeentity __basevalue __finalvalue) (break `Ck_Payload_FloatAttribute_OnValueChanged` InPayload))
  (set `self._Max` __finalvalue)
  (`self.DoNotifyAttributeChanged` InAttributeOwnerEntity __attributeentity))

(event `OnAttributeChanged_Current`
  (params (InAttributeOwnerEntity :type "Ck_Handle Structure") (InPayload :type "Ck_Payload_FloatAttribute_OnValueChanged Structure"))
  (bind (__attributeentity __basevalue __finalvalue) (break `Ck_Payload_FloatAttribute_OnValueChanged` InPayload))
  (set `self._Current` __finalvalue)
  (`self.DoNotifyAttributeChanged` InAttributeOwnerEntity __attributeentity))

(event `self.Deactivate_BP`
  (`parent.Deactivate_BP`)
  (`/CkFoundation/CkEcs/EntityHandle_CkEcs_ML.ValidateEntityHandle` (`self.AttributeHandle`)
    (:`IsValid`
      (`|ExecutionSequence`
        (:`then_0`
          (`Ck_Utils_FloatAttribute_UE.UnbindFrom_OnValueChanged` (`self.AttributeHandle`) "Current" (`|CreateDelegate` :!event `OnAttributeChanged_Current`)))
        (:`then_1`
          (if (`Ck_Utils_FloatAttribute_UE.Has_Component` (`self.AttributeHandle`) "Max")
            (`Ck_Utils_FloatAttribute_UE.UnbindFrom_OnValueChanged` (`self.AttributeHandle`) "Max" (`|CreateDelegate` :!event `OnAttributeChanged_Max`))))))))

(fn `DoNotifyAttributeChanged`
  (params (AttributeOwnerHandle :type "Ck_Handle Structure") (AtributeHandle :type "Ck_Handle_FloatAttribute Structure"))
  (set `self._Value%_Previous` (`self._Value%`))
  (set `self._Value%` (/ (`self._Current`) (`self._Max`)))
  (`self.AttributeValueChanged` AttributeOwnerHandle AtributeHandle (`self._Value%`) (`self._Value%_Previous`)))

(fn `DoNotifyInitialAttributeValue`
  (bind _output_get (set `self._Value%` (/ (`self._Current`) (`self._Max`))))
  (set `self._Value%_Previous` _output_get)
  (`self.InitialAttributeValue` (`self._Value%`)))

(fn `Get_StatusString_BP`
  (returns (ReturnValue :type String))
  (`/CkFoundation/CkEcs/EntityHandle_CkEcs_ML.ValidateEntityHandle` (`self.AttributeHandle`)
    (:`IsValid`
      (return (`KismetTextLibrary.Conv_TextToString` (`|FormatText` "{owner} \n{attribute} \n{cur} / {max} [{percent}%]" (`Ck_Utils_Handle_UE.Conv_HandleToString` (`Ck_Utils_EntityLifetime_UE.Get_LifetimeOwner` (`self.AttributeHandle`))) (`Ck_Utils_Handle_UE.Conv_HandleToString` (`self.AttributeHandle`)) (`self._Current`) (`self._Max`) (`self._Value%`)))))
    (:`NotValid`
      (return "Invalid Attribute Entity"))))