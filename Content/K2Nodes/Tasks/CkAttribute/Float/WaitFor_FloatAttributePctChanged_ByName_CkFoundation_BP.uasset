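; Task Blueprint that waits for a percentage change in a Float Attribute identified by name on an owner entity.
; On activation, it resolves the attribute handle from the owner entity and name, then ensures the handle is valid.
; Only a valid handle passes on to the parent activation, which carries the wait logic; a failed lookup reports the name, owner and task.
; Deactivation simply defers to the parent.
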(event `self.Activate_BP`
  (set `self.AttributeHandle` (`Ck_Utils_FloatAttribute_UE.TryGet` (`self.AttributeOwnerEntity`) (`self.AttributeName`)))
  (`Ck_Utils_Ensure_UE.EnsureMsgf` (`Ck_Utils_Handle_UE.Get_IsValid` (`self.AttributeHandle`)) (`|FormatText` self "Could NOT find Float Attribute with Name [{name}] in Entity [{owner}] in [{self}]" (`BlueprintGameplayTagLibrary.GetTagName` (`self.AttributeName`)) (`Ck_Utils_Handle_UE.Conv_HandleToText` (`self.AttributeOwnerEntity`)))
    (:`Valid`
      (`parent.Activate_BP`))))

(event `self.Deactivate_BP`
  (`parent.Deactivate_BP`))