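; Task Forge Blueprint task that exposes the lifetime of a CkEcs entity script as constructed and destroyed callbacks.
; On activation it wraps a pending entity script in a Task Forge node and, once constructed, stores the handle and fires the constructed callback.
; It then binds to that entity's destroy signal, including payloads in flight that frame, to fire the destroyed callback and deactivate itself.
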(event `self.Activate_BP`
  (`parent.Activate_BP`)
  (bind (_taskobject _onconstructed_outentityscripthandle) (`|TaskForge_K2Node` (`self.PendingEntityScript`))
    (:`OnConstructed`
      (bind _output_get (set `self._EntityScriptHandle` _onconstructed_outentityscripthandle))
      (`self.OnConstructed` _output_get)
      (`Ck_Utils_EntityLifetime_UE.BindTo_OnDestroy` (`self._EntityScriptHandle`) "FireIfPayloadInFlightThisFrame" (delegate `OnEntityDestroyed`)))))

(event `OnEntityDestroyed`
  (params (InHandle :type "Ck_Handle Structure"))
  (`self.OnDestroyed` (`self._EntityScriptHandle`))
  (`self.Deactivate`))