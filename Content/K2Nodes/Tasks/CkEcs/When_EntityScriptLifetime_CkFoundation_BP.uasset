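; Blueprint async task node that tracks the lifetime of an ECS entity script, exposing Constructed and Destroyed callbacks.
; On activation it runs a nested template task on the pending entity script, registered to deactivate along with this one.
; Once constructed, it fires OnConstructed with the handle and binds to entity destruction, including payloads in flight that frame.
; On destruction it fires OnDestroyed and deactivates itself.
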(event `self.Activate_BP`
  (`parent.Activate_BP`)
  (bind (_taskobject _onconstructed_outentityscripthandle) (`|Blueprint_Template` (`self.PendingEntityScript`))
    (:`then`
      (`self.DoRequest_AddTaskToDeactivateOnDeactivate` _taskobject))
    (:`OnConstructed`
      (bind _output_get (set `self._EntityScriptHandle` _onconstructed_outentityscripthandle))
      (`self.OnConstructed` _output_get)
      (`Ck_Utils_EntityLifetime_UE.BindTo_OnDestroy` (`self._EntityScriptHandle`) "FireIfPayloadInFlightThisFrame" (delegate `OnEntityDestroyed`)))))

(event `OnEntityDestroyed`
  (params (InHandle :type "Ck_Handle Structure"))
  (`self.OnDestroyed` (`self._EntityScriptHandle`))
  (`self.Deactivate`))