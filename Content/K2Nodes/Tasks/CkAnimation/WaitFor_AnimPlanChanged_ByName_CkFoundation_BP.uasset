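; Task Blueprint that waits for an AnimPlan change, with the AnimPlan looked up by goal name on an owner entity.
; On activation it resolves the AnimPlan entity from the owner and goal tag, then hands off to the parent activation.
; An ensure reports a failed lookup with the goal, owner and context, and the task deactivates instead of waiting.
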(event `self.Activate_BP`
  (set `self.AnimPlanEntity` (`Ck_Utils_AnimPlan_UE.TryGet_AnimPlan` (`self.AnimPlanOwner`) (`self.AnimPlanGoal`)))
  (`Ck_Utils_EcsEnsure_UE.EnsureMsgf_IsValid` (`self.AnimPlanEntity`) (`|FormatText` self "Failed to find AnimPlan [{name}] on Owner [{owner}]. Context: [{self}]" (`BlueprintGameplayTagLibrary.GetTagName` (`self.AnimPlanGoal`)) (`Ck_Utils_Handle_UE.Conv_HandleToText` (`self.AnimPlanOwner`)))
    (:`Valid`
      (`parent.Activate_BP`))
    (:`Invalid`
      (`self.Deactivate`))))