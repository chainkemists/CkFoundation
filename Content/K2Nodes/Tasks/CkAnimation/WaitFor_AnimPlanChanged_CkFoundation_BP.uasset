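; Blueprint task node in CkFoundation that reports goal changes on an AnimPlan entity.
; On activation it binds to the entity's goal-changed signal, also firing for a payload in flight that frame, or raises an ensure and deactivates if the handle is invalid.
; Each change passes the handle and previous and new plan states to PlanChanged without ending the task.
; Deactivation unbinds if the entity is still valid.
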(event `self.Activate_BP`
  (`parent.Activate_BP`)
  (`Ck_Utils_EcsEnsure_UE.EnsureMsgf_IsValid` (`self.AnimPlanEntity`) (`|FormatText` self "Invalid AnimPLan Entity supplied to [{self}]")
    (:`Valid`
      (`Ck_Utils_AnimPlan_UE.BindTo_OnGoalChanged` (`self.AnimPlanEntity`) "FireIfPayloadInFlightThisFrame" "DoNothing" (delegate `OnPlanChanged`)))
    (:`Invalid`
      (`self.Deactivate`))))

(event `OnPlanChanged`
  (params (InHandle :type "Ck_Handle_AnimPlan Structure") (InPreviousPlanState :type "Ck_AnimPlan_State Structure (by ref)") (InNewPlanState :type "Ck_AnimPlan_State Structure (by ref)"))
  (`self.PlanChanged` InHandle InPreviousPlanState InNewPlanState))

(event `self.Deactivate_BP`
  (`parent.Deactivate_BP`)
  (bind _outhandle (`/CkFoundation/CkEcs/EntityHandle_CkEcs_ML.ValidateEntityHandle` (`self.AnimPlanEntity`))
    (:`IsValid`
      (`Ck_Utils_AnimPlan_UE.UnbindFrom_OnGoalChanged` _outhandle (`|CreateDelegate` :!event `OnPlanChanged`)))))