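; Blueprint async task node that plays an animation montage on a skeletal mesh and relays completed, blend out, interrupted and notify events, deactivating on the terminal ones.
; Before playing, it checks skeleton compatibility and mesh ticking, including dedicated-server tick outside clients.
; It can force disabled tick settings on while active and reverts only those it changed on deactivation.
; Otherwise it reports failure, with an optional ensure.
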(event `self.Activate_BP`
  (`parent.Activate_BP`)
  (if (`Ck_Utils_Animation_UE.DoesMontageMatchMeshSkeleton` (`self.Montage to Play`) (`self.In Skeletal Mesh Component`))
    (if (or (`|EnumEquality` (`Ck_Utils_Net_UE.Get_NetMode` (`self.In Skeletal Mesh Component`)) "Client") (`Ck_Utils_ActorComponent_UE.Get_AllowTickOnDedicatedServer` (`self.In Skeletal Mesh Component`)))
      (if (`ActorComponent.IsComponentTickEnabled` (`self.In Skeletal Mesh Component`)) :!label _label
        (bind _notifyname (`|PlayMontage` (`self.In Skeletal Mesh Component`) (`self.Montage to Play`) (`self.Play Rate`) (`self.Starting Position`) (`self.Starting Section`) :!label _label_2)
          (:`OnCompleted`
            (`self.OnCompleted`)
            (`self.Deactivate`))
          (:`OnBlendOut`
            (`self.OnBlendedOut`)
            (`self.Deactivate`))
          (:`OnInterrupted`
            (`self.OnInterrupted`)
            (`self.Deactivate`))
          (:`OnNotifyBegin`
            (`self.OnNotifyBegin` _notifyname))
          (:`OnNotifyEnd`
            (`self.OnNotifyEnd` _notifyname)))
        (elif (`self.ForceMeshToTickWhileActive`)
          (`ActorComponent.SetComponentTickEnabled` (`self.In Skeletal Mesh Component`) true)
          (set `self._SetMeshTickEnabled` true)
          (goto _label_2)
          (else
            (`Ck_Utils_Ensure_UE.EnsureMsgf` (not (`self.EnsureOnFail`)) "Skeletal mesh tick is NOT enabled!"
              (:`Valid`
                _)
              (:`Invalid`
                _))
            (`self.OnFailed`)
            (`self.Deactivate`))))
      (elif (`self.ForceMeshToTickWhileActive`)
        (`Ck_Utils_ActorComponent_UE.Set_AllowTickOnDedicatedServer` (`self.In Skeletal Mesh Component`) true)
        (set `self._SetMeshAllowTickOnDedicatedServer` true)
        (goto _label)
        (else
          (`Ck_Utils_Ensure_UE.EnsureMsgf` (not (`self.EnsureOnFail`)) "Skeletal mesh tick is NOT enabled on server!"
            (:`Valid`
              _)
            (:`Invalid`
              _))
          (`self.OnFailed`)
          (`self.Deactivate`))))
    (else
      (`Ck_Utils_Ensure_UE.EnsureMsgf` (not (`self.EnsureOnFail`)) "Skeletal from montage and mesh do NOT match!"
        (:`Valid`
          _)
        (:`Invalid`
          _))
      (`self.OnFailed`)
      (`self.Deactivate`))))

(event `self.Deactivate_BP`
  (`parent.Deactivate_BP`)
  (`|ExecutionSequence`
    (:`then_0`
      (if (`self._SetMeshAllowTickOnDedicatedServer`)
        (`Ck_Utils_ActorComponent_UE.Set_AllowTickOnDedicatedServer` (`self.In Skeletal Mesh Component`))))
    (:`then_1`
      (if (`self._SetMeshTickEnabled`)
        (`ActorComponent.SetComponentTickEnabled` (`self.In Skeletal Mesh Component`) false)))))