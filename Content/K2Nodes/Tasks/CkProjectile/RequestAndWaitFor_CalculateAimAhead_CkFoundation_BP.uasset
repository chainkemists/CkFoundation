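; Async task Blueprint that requests a projectile aim-ahead calculation from CkProjectile and waits for the result.
; On activation it passes the aim policy, projectile start location and speed, target location and velocity, and an optional payload to the request.
; The callback fires OnSucceeded with the aim point and payload, or OnFailed with only the payload, then deactivates the task.
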(event `self.Activate_BP`
  (`parent.Activate_BP`)
  (`/CkFoundation/CkProjectile/Utils_CkProjectile_FL.[Ck][Projectile] Request Calculate Aim Ahead` (`self.AimAheadPolicy`) (`self.ProjectileStartingLoc`) (`self.ProjectileSpeed`) (`self.TargetLoc`) (`self.TargetVel`) (`self.OptionalPayload`) (delegate `OnAimAheadCalculated`)))

(event `OnAimAheadCalculated`
  (params (InSuccessFailed :type "ECk_SucceededFailed Enum" :default "Succeeded") (InTargetAimPoint :type "Vector Structure (by ref)") (InOptionalPayload :type "InstancedStruct Structure (by ref)"))
  (switch `ECk_SucceededFailed` InSuccessFailed
    (:`Succeeded`
      (`self.OnSucceeded` InTargetAimPoint InOptionalPayload))
    (:`Failed`
      (`self.OnFailed` InOptionalPayload)))
  (`self.Deactivate`))