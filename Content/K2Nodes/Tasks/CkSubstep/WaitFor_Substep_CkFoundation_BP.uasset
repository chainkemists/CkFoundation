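; Blueprint task node that waits on a CkFoundation substep handle and relays its first-update, per-step update and frame-end signals.
; On activation it binds all three, firing for payloads already in flight this frame, and forwards each event with its delta times, plus step number for updates.
; The frame-end binding unbinds after firing, while the other two persist until deactivation removes all three.
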(event `self.Activate_BP`
  (`parent.Activate_BP`)
  (bind _returnvalue (`Ck_Utils_Substep_UE.BindTo_OnFirstUpdate` (`self.SubstepHandle`) "FireIfPayloadInFlightThisFrame" "DoNothing" (delegate `Event_OnFirstUpdate`)))
  (bind _returnvalue_2 (`Ck_Utils_Substep_UE.BindTo_OnUpdate` _returnvalue "FireIfPayloadInFlightThisFrame" "DoNothing" (delegate `Event_OnUpdate`)))
  (`Ck_Utils_Substep_UE.BindTo_OnFrameEnd` _returnvalue_2 "FireIfPayloadInFlightThisFrame" "Unbind" (delegate `Event_OnFrameEnd`)))

(event `Event_OnFirstUpdate`
  (params (InHandle :type "Ck_Handle_Substep Structure") (InFrameDeltaT :type "Ck_Time Structure"))
  (`self.OnFirstUpdate` InHandle InFrameDeltaT))

(event `Event_OnUpdate`
  (params (InHandle :type "Ck_Handle_Substep Structure") (InSubstepDeltaT :type "Ck_Time Structure") (InStepNumber :type Integer) (InFrameDeltaT :type "Ck_Time Structure"))
  (`self.OnUpdate` InHandle InSubstepDeltaT InStepNumber InFrameDeltaT))

(event `Event_OnFrameEnd`
  (params (InHandle :type "Ck_Handle_Substep Structure") (InFrameDeltaT :type "Ck_Time Structure"))
  (`self.OnFrameEnd` InHandle InFrameDeltaT))

(event `self.Deactivate_BP`
  (`parent.Deactivate_BP`)
  (bind _returnvalue (`Ck_Utils_Substep_UE.UnbindFrom_OnFirstUpdate` (`self.SubstepHandle`) (`|CreateDelegate` :!event `Event_OnFirstUpdate`)))
  (bind _returnvalue_2 (`Ck_Utils_Substep_UE.UnbindFrom_OnUpdate` _returnvalue (`|CreateDelegate` :!event `Event_OnUpdate`)))
  (`Ck_Utils_Substep_UE.UnbindFrom_OnFrameEnd` _returnvalue_2 (`|CreateDelegate` :!event `Event_OnFrameEnd`)))