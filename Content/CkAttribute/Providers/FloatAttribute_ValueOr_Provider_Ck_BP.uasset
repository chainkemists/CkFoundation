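; A float provider Blueprint that supplies a named attribute's value from an entity, with a fallback when the attribute is absent.
; It resolves the optional input handle to itself or its parent, then tries to get the attribute there.
; A GetValueOr branch returns the base or final value of the configured attribute component according to the value category, or the ValueOr default if the attribute is invalid.
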(fn `Get_Value`
  (params (InOptionalHandle :type "Ck_Handle Structure"))
  (returns (ReturnValue :type "Float (single-precision)"))
  (locals (L_EntityToUse :type "Ck_Handle Structure") (L_Attribute :type "Ck_Handle_FloatAttribute Structure"))
  (bind _outentity (`/CkFoundation/CkAttribute/Attribute_CkAttribute_ML.Get_EntityOrParent` (`self.SelfOrParent`) InOptionalHandle))
  (bind _output_get (set `local.L_EntityToUse` _outentity))
  (set `local.L_Attribute` (`Ck_Utils_FloatAttribute_UE.TryGet` (`local.L_EntityToUse`) (`self.AttributeName`)))
  (`/CkFoundation/CkAttribute/Attribute_CkAttribute_ML.Get_ValueOr` _output_get (`self.AttributeName`) (`self.SelfOrParent`) (`self.ValueCategory`) (`Ck_Utils_Handle_UE.Get_IsValid` (`local.L_Attribute`))
    (:`BaseValue`
      (return (`Ck_Utils_FloatAttribute_UE.Get_BaseValue` (`local.L_Attribute`) (`self.AttributeComponent`))))
    (:`FinalValue`
      (return (`Ck_Utils_FloatAttribute_UE.Get_FinalValue` (`local.L_Attribute`) (`self.AttributeComponent`))))
    (:`DefaultValue`
      (return (`self.ValueOr`)))))