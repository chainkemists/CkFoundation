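; A value provider Blueprint that reads a named meter attribute from an entity, with a fallback value when it cannot.
; Get_Value resolves the optional handle to the entity or its parent, according to the SelfOrParent setting.
; A shared GetValueOr node takes an attribute presence check and the value category, then branches to return the base value, final value or ValueOr default.
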(fn `Get_Value`
  (params (InOptionalHandle :type "Ck_Handle Structure"))
  (returns (ReturnValue :type "Ck_Meter Structure"))
  (locals (L_EntityToUse :type "Ck_Handle Structure"))
  (bind _outentity (`/CkFoundation/CkAttribute/Attribute_CkAttribute_ML.Get_EntityOrParent` (`self.SelfOrParent`) InOptionalHandle))
  (bind _output_get (set `local.L_EntityToUse` _outentity))
  (`/CkFoundation/CkAttribute/Attribute_CkAttribute_ML.Get_ValueOr` _output_get (`self.AttributeName`) (`self.SelfOrParent`) (`self.ValueCategory`) (`Ck_Utils_MeterAttribute_UE.Has` (struct) (`self.AttributeName`))
    (:`BaseValue`
      (return (`Ck_Utils_MeterAttribute_UE.Get_BaseValue` (struct) (`self.AttributeName`))))
    (:`FinalValue`
      (return (`Ck_Utils_MeterAttribute_UE.Get_FinalValue` (struct) (`self.AttributeName`))))
    (:`DefaultValue`
      (return (`self.ValueOr`)))))