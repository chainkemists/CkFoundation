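; Base CkAbility Blueprint that activates or deactivates an ability through events, automatically, or both, based on its trigger policy.
; When given, event policies listen on the ability owner for activation and deactivation tags, with deactivation taking precedence.
; Activation forwards the event's context and data as payload.
; Automatic policies request activation whenever tags update on the owner, or on the ability if it is an AbilityOwner, where matching activation settings exist.
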(event `self.DoOnGiveAbility`
  (params (InOptionalPayload :type "Ck_Ability_Payload_OnGranted Structure (by ref)"))
  (`parent.DoOnGiveAbility` InOptionalPayload)
  (switch `ECk_Ability_ActivationTrigger_Policy` (`self.ActivationTriggerPolicy`)
    (:`TriggeredByEvent`
      (`BlueprintGameplayTagLibrary.AppendGameplayTagContainers` (`self._AllTriggers`) (`self.ActivationTriggers`) :!label _label)
      (`BlueprintGameplayTagLibrary.AppendGameplayTagContainers` (`self._AllTriggers`) (`self.DeactivationTriggers`))
      (if (`KismetArrayLibrary.Array_IsNotEmpty` (`BlueprintGameplayTagLibrary.BreakGameplayTagContainer` (`self._AllTriggers`)))
        (bind (_taskobject _eventfired_outabilityownerhandle _eventfired_outevent) (`|Blueprint_Template` (`self.DoGet_AbilityOwnerEntity`) (`self._AllTriggers`))
          (:`EventFired`
            (`self.TryActivateOrDeactivateOnEvent` _eventfired_outevent)))))
    (:`TriggeredAutomatically`
      (`|ExecutionSequence` :!label _label_2
        (:`then_0`
          (if (`self.DoGet_HasAnyActivationSettings_OnOwner`)
            (`|Blueprint_Template` (`self.DoGet_AbilityOwnerEntity`)
              (:`TagsUpdated`
                (`self.DoRequest_ActivateAbility` (struct))))))
        (:`then_1`
          ;[0 1 0.4844] It's VALID to NOT be an AbilityOwner
          (bind _returnvalue (`Ck_Utils_AbilityOwner_UE.DoCast` (`self.DoGet_AbilityEntity`))
            (:`Succeeded`
              (if (`self.DoGet_HasAnyActivationSettings_OnSelf`)
                (`|Blueprint_Template` _returnvalue
                  (:`TagsUpdated`
                    (`self.DoRequest_ActivateAbility` (struct))))))))))
    (:`TriggeredByEventOrAutomatically`
      (`|ExecutionSequence`
        (:`then_0`
          (goto _label))
        (:`then_1`
          (goto _label_2))))))

(fn `DoGet_HasAnyActivationSettings_OnOwner`
  (returns (OutResult :type Boolean))
  (bind (__granttagsonabilityowner __cancelledbytagsonabilityowner __requiredtagsonabilityowner __blockedbytagsonabilityowner) (break `Ck_Ability_ActivationSettings_OnOwner` (`._ActivationSettingsOnOwner` (break `Ck_Ability_ActivationSettings` (`Ck_Utils_Ability_UE.Get_ActivationSettings` (`self.DoGet_AbilityEntity`))))))
  (return (`/CkFoundation/CkCore/Math/Math_CkCore_ML.>0 (int)` (+ (`BlueprintGameplayTagLibrary.GetNumGameplayTagsInContainer` __cancelledbytagsonabilityowner) (`BlueprintGameplayTagLibrary.GetNumGameplayTagsInContainer` __requiredtagsonabilityowner) (`BlueprintGameplayTagLibrary.GetNumGameplayTagsInContainer` __blockedbytagsonabilityowner)))))

(fn `DoGet_HasAnyActivationSettings_OnSelf`
  (returns (OutResult :type Boolean))
  (bind (__cancelledbytagsonself __blockedbytagsonself) (break `Ck_Ability_ActivationSettings_OnSelf` (`._ActivationSettingsOnSelf` (break `Ck_Ability_ActivationSettings` (`Ck_Utils_Ability_UE.Get_ActivationSettings` (`self.DoGet_AbilityEntity`))))))
  (return (`/CkFoundation/CkCore/Math/Math_CkCore_ML.>0 (int)` (+ (`BlueprintGameplayTagLibrary.GetNumGameplayTagsInContainer` __cancelledbytagsonself) (`BlueprintGameplayTagLibrary.GetNumGameplayTagsInContainer` __blockedbytagsonself)))))

(fn `TryActivateOrDeactivateOnEvent`
  (params (InEvent :type "Ck_AbilityOwner_Event Structure"))
  (locals (L_AbilityOwnerEvent :type "Ck_AbilityOwner_Event Structure"))
  (bind (__eventname __contextentity __eventdata) (break `Ck_AbilityOwner_Event` (`local.L_AbilityOwnerEvent`)))
  (set `local.L_AbilityOwnerEvent` InEvent)
  (if (`BlueprintGameplayTagLibrary.HasTag` (`self.DeactivationTriggers`) (`._EventName` (break `Ck_AbilityOwner_Event` (`local.L_AbilityOwnerEvent`))) true)
    (`self.DoRequest_DeactivateAbility`)
    (elif (`BlueprintGameplayTagLibrary.HasTag` (`self.ActivationTriggers`) (`._EventName` (break `Ck_AbilityOwner_Event` (`local.L_AbilityOwnerEvent`))) true)
      (`self.DoRequest_ActivateAbility` (make `Ck_Ability_Payload_OnActivate` __contextentity __eventdata))
      (else
        (bind _returnvalue (`Ck_Utils_AbilityOwner_UE.DoCast` (`self.DoGet_AbilityEntity`))
          (:`Succeeded`
            (`self.DoOnAbilityNotActivated` (make `Ck_Ability_NotActivated_Info` "RequirementsNotMet_OnSelf" (`Ck_Utils_AbilityOwner_UE.Get_ActiveTags` (`self.DoGet_AbilityOwnerEntity`)) (`Ck_Utils_AbilityOwner_UE.Get_ActiveTags` _returnvalue)))))))))