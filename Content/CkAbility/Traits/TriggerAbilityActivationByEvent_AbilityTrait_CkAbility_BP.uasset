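; Ability trait that, when its owning ability is given, sets up activation by event, automatically or both, per its trigger policy.
; Event mode listens on the ability owner for trigger tags, checking deactivation first and passing event context and data into activation.
; Automatic mode requests activation on tag updates from the owner, and from the ability if it is itself an owner, wherever relevant activation tag settings exist.
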(event `self.DoOnOwningAbilityGiven`
  (params (InAbility :type "Ck_Handle_Ability Structure") (InAbilityOwner :type "Ck_Handle_AbilityOwner Structure"))
  (bind __alltriggers (`self._AllTriggers`))
  (`parent.DoOnOwningAbilityGiven` InAbility InAbilityOwner)
  (switch `ECk_Ability_ActivationTrigger_Policy` (`self.ActivationTriggerPolicy`)
    (:`TriggeredByEvent`
      (`BlueprintGameplayTagLibrary.AppendGameplayTagContainers` (`self._AllTriggers`) (`self.ActivationTriggers`) :!label _label)
      (`BlueprintGameplayTagLibrary.AppendGameplayTagContainers` (`self._AllTriggers`) (`self.DeactivationTriggers`))
      (bind (_taskobject _eventfired_outabilityownerhandle _eventfired_outevent) (`|Blueprint_Template` (`self.DoGet_OwningAbilityOwnerEntity`) __alltriggers __alltriggers)
        (:`EventFired`
          (`self.TryActivateOrDeactivateOnEvent` _eventfired_outevent))))
    (:`TriggeredAutomatically`
      (`|ExecutionSequence` :!label _label_2
        (:`then_0`
          (if (`self.DoGet_HasAnyActivationSettings_OnOwningAbilityOwner`)
            (`|Blueprint_Template` (`self.DoGet_OwningAbilityOwnerEntity`)
              (:`TagsUpdated`
                (`self.DoRequest_ActivateOwningAbility` (struct))))))
        (:`then_1`
          ;[0 1 0.4844] It's VALID to NOT be an AbilityOwner
          (bind _returnvalue (`Ck_Utils_AbilityOwner_UE.DoCast` (`self.DoGet_OwningAbilityEntity`))
            (:`Succeeded`
              (if (`self.DoGet_HasAnyActivationSettings_OnOwningAbility`)
                (`|Blueprint_Template` _returnvalue
                  (:`TagsUpdated`
                    (`self.DoRequest_ActivateOwningAbility` (struct))))))))))
    (:`TriggeredByEventOrAutomatically`
      (`|ExecutionSequence`
        (:`then_0`
          (goto _label))
        (:`then_1`
          (goto _label_2))))))

(event `self.DoOnOwningAbilityRevoked`
  (params (InAbility :type "Ck_Handle_Ability Structure") (InAbilityOwner :type "Ck_Handle_AbilityOwner Structure"))
  (`parent.DoOnOwningAbilityRevoked` InAbility InAbilityOwner))

(fn `DoGet_HasAnyActivationSettings_OnOwningAbility`
  (returns (OutResult :type Boolean))
  (bind (__cancelledbytagsonself __blockedbytagsonself) (break `Ck_Ability_ActivationSettings_OnSelf` (`._ActivationSettingsOnSelf` (break `Ck_Ability_ActivationSettings` (`Ck_Utils_Ability_UE.Get_ActivationSettings` (`self.DoGet_OwningAbilityEntity`))))))
  (return (`/CkFoundation/CkCore/Math/Math_CkCore_ML.>0 (int)` (+ (`BlueprintGameplayTagLibrary.GetNumGameplayTagsInContainer` __cancelledbytagsonself) (`BlueprintGameplayTagLibrary.GetNumGameplayTagsInContainer` __blockedbytagsonself)))))

(fn `DoGet_HasAnyActivationSettings_OnOwningAbilityOwner`
  (returns (OutResult :type Boolean))
  (bind (__granttagsonabilityowner __cancelledbytagsonabilityowner __requiredtagsonabilityowner __blockedbytagsonabilityowner) (break `Ck_Ability_ActivationSettings_OnOwner` (`._ActivationSettingsOnOwner` (break `Ck_Ability_ActivationSettings` (`Ck_Utils_Ability_UE.Get_ActivationSettings` (`self.DoGet_OwningAbilityEntity`))))))
  (return (`/CkFoundation/CkCore/Math/Math_CkCore_ML.>0 (int)` (+ (`BlueprintGameplayTagLibrary.GetNumGameplayTagsInContainer` __cancelledbytagsonabilityowner) (`BlueprintGameplayTagLibrary.GetNumGameplayTagsInContainer` __requiredtagsonabilityowner) (`BlueprintGameplayTagLibrary.GetNumGameplayTagsInContainer` __blockedbytagsonabilityowner)))))

(fn `TryActivateOrDeactivateOnEvent`
  (params (InEvent :type "Ck_AbilityOwner_Event Structure"))
  (locals (L_AbilityOwnerEvent :type "Ck_AbilityOwner_Event Structure"))
  (bind (__eventname __contextentity __eventdata) (break `Ck_AbilityOwner_Event` (`local.L_AbilityOwnerEvent`)))
  (set `local.L_AbilityOwnerEvent` InEvent)
  (if (`BlueprintGameplayTagLibrary.HasTag` (`self.DeactivationTriggers`) (`._EventName` (break `Ck_AbilityOwner_Event` (`local.L_AbilityOwnerEvent`))) true)
    (`self.DoRequest_DeactivateOwningAbility`)
    (elif (`BlueprintGameplayTagLibrary.HasTag` (`self.ActivationTriggers`) (`._EventName` (break `Ck_AbilityOwner_Event` (`local.L_AbilityOwnerEvent`))) true)
      (`self.DoRequest_ActivateOwningAbility` (make `Ck_Ability_Payload_OnActivate` __contextentity __eventdata)))))