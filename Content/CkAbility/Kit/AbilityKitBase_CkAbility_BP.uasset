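; Base Blueprint for ability kits: abilities registered as entity extensions of their owner that can hold sub-abilities.
; Construct and give add the extension and revoke removes it.
; Give also fires ensures on blocking, cost or cooldown sub-abilities, which kits do not support.
; Activation forwards the owner's ability events to the kit under an all, all-except or specific-tags policy, and syncs relevant owner tags.
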(event `Check Condition Subabilities`
  ;[0 0 0] Check that there are no conditional subabilities since we don't support using blocking tags on abilities that are an extension
  (bind _returnvalue (`Ck_Utils_AbilityOwner_UE.DoCast` (`self.DoGet_AbilityEntity`))
    (:`Succeeded`
      (`|ExecutionSequence`
        (:`then_0`
          (bind _returnvalue_2 (`Ck_Utils_AbilityOwner_UE.Get_AbilityCount_Blocking` _returnvalue))
          (if (`/CkFoundation/CkCore/Math/Math_CkCore_ML.>0 (int)` _returnvalue_2)
            (`Ck_Utils_Ensure_UE.TriggerEnsure` (`|FormatText` "Ability kit [{ability}] has [{num}] blocking ability condition(s) which is NOT supported!" self _returnvalue_2))))
        (:`then_1`
          (bind _returnvalue_3 (`Ck_Utils_AbilityOwner_UE.Get_AbilityCount_Cost` _returnvalue))
          (if (`/CkFoundation/CkCore/Math/Math_CkCore_ML.>0 (int)` _returnvalue_3)
            (`Ck_Utils_Ensure_UE.TriggerEnsure` (`|FormatText` "Ability kit [{ability}] has [{num}] cost ability(s) which is NOT supported!" self _returnvalue_3))))
        (:`then_2`
          (bind _returnvalue_4 (`Ck_Utils_AbilityOwner_UE.Get_AbilityCount_Cooldown` _returnvalue))
          (if (`/CkFoundation/CkCore/Math/Math_CkCore_ML.>0 (int)` _returnvalue_4)
            (`Ck_Utils_Ensure_UE.TriggerEnsure` (`|FormatText` "Ability kit [{ability}] has [{num}] coldown ability(s) which is NOT supported!" self _returnvalue_4))))))))

(event `self.DoOnGiveAbility`
  (params (InOptionalPayload :type "Ck_Ability_Payload_OnGranted Structure (by ref)"))
  (`parent.DoOnGiveAbility` InOptionalPayload)
  (`self.Check Condition Subabilities`)
  ;[0 0 0] Add AbilityKit as EntityExtension
  (`Ck_Utils_EntityExtension_UE.DoCast` (`self.DoGet_AbilityEntity`)
    (:`Failed`
      (`Ck_Utils_EntityExtension_UE.Add` (`self.DoGet_AbilityOwnerEntity`) (`self.DoGet_AbilityEntity`)))))

(event `self.DoOnRevokeAbility`
  (`parent.DoOnRevokeAbility`)
  ;[0 0 0] Remove AbilityKit as EntityExtension
  (bind _returnvalue (`Ck_Utils_EntityExtension_UE.DoCast` (`self.DoGet_AbilityEntity`))
    (:`Succeeded`
      (`Ck_Utils_EntityExtension_UE.Remove` (`self.DoGet_AbilityOwnerEntity`) _returnvalue))))

(event `self.DoOnActivateAbility`
  (params (InActivationPayload :type "Ck_Ability_Payload_OnActivate Structure (by ref)"))
  (bind _eventstoexclude (`self.EventsToExclude`))
  (bind _specificeventstoforward (`self.SpecificEventsToForward`))
  (`parent.DoOnActivateAbility` InActivationPayload)
  (`|ExecutionSequence`
    (:`then_0`
      ;[0 0 0] Forward Events
      (bind _returnvalue (`Ck_Utils_AbilityOwner_UE.DoCast` (`self.DoGet_AbilityEntity`))
        (:`Succeeded`
          (switch `ECk_Ability_EventsForwarding_Policy` (`self.EventsForwardingPolicy`)
            (:`All`
              (bind (_taskobject _eventfired_outabilityownerhandle _eventfired_outevent) (`|Blueprint_Template` (`self.DoGet_AbilityOwnerEntity`))
                (:`EventFired`
                  (`Ck_Utils_AbilityOwner_UE.Request_SendAbilityEvent` _returnvalue (make `Ck_Request_AbilityOwner_SendEvent` _eventfired_outevent)))))
            (:`AllExcept`
              (bind (_taskobject_2 _eventfired_outabilityownerhandle_2 _eventfired_outevent_2) (`|Blueprint_Template` (`self.DoGet_AbilityOwnerEntity`) _eventstoexclude _eventstoexclude)
                (:`EventFired`
                  (`Ck_Utils_AbilityOwner_UE.Request_SendAbilityEvent` _returnvalue (make `Ck_Request_AbilityOwner_SendEvent` _eventfired_outevent_2)))))
            (:`Specific`
              (if (`KismetArrayLibrary.Array_IsNotEmpty` (`BlueprintGameplayTagLibrary.BreakGameplayTagContainer` _specificeventstoforward))
                (bind (_taskobject_3 _eventfired_outabilityownerhandle_3 _eventfired_outevent_3) (`|Blueprint_Template` (`self.DoGet_AbilityOwnerEntity`) _specificeventstoforward)
                  (:`EventFired`
                    (`Ck_Utils_AbilityOwner_UE.Request_SendAbilityEvent` _returnvalue (make `Ck_Request_AbilityOwner_SendEvent` _eventfired_outevent_3))))))))
        (:`Failed`
          (`Ck_Utils_Log_UE.Log` (`|FormatText` self "Ability Kit [{self}] has NO abilities. This may or may not be unexpected.") (struct :`_Name` "CkAbility")))))
    (:`then_1`
      ;[0 0 0] Propagate Ability Owner's Tags To Kit Tags
      (`|Blueprint_Template` (`self.DoGet_AbilityOwnerEntity`)
        (:`then`
          _)
        (:`TagsUpdated`
          _))
      (`self.SyncTagsWithAbilityOwner` (`self.RelevantTagsFromAbilityOwner`)))))

(fn `DoConstruct`
  (params (InHandle :type "Ck_Handle Structure (by ref)"))
  (`Ck_Utils_EntityExtension_UE.Add` (`Ck_Utils_EntityLifetime_UE.Get_LifetimeOwner` InHandle) InHandle)
  (return))

(fn `Get_ThumbnailIconAndColor`
  (returns (OutBackgroundColor :type "LinearColor Structure") (ReturnValue :type "Texture2D Object Reference"))
  (return (struct :`R` 0.01033 :`G` 0.01033 :`B` 0.01033 :`A` 1.0) "/CkFoundation/Textures/Icon_AbilityKit_64px.Icon_AbilityKit_64px"))