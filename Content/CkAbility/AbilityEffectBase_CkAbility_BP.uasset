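; Base CkAbility Blueprint for GAS-style gameplay effects that modify the owner's float attributes.
; When given, it waits a tick for SetByCaller values, then activates by duration policy, using entity timers for duration and period.
; Each activation applies non-revocable modifiers or overrides from discrete, attribute-based or SetByCaller magnitudes, then deactivates.
; Stacking policies govern limits, timer resets and expiry, but per-source stacking is unsupported and Source currently resolves like Target.
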(event `self.DoOnGiveAbility`
  (params (InOptionalPayload :type "Ck_Ability_Payload_OnGranted Structure (by ref)"))
  (bind (__contextentity __data) (break `Ck_Ability_Payload_OnGranted` InOptionalPayload))
  (bind (__contextentity_2 __data_2) (break `Ck_Ability_Payload_OnGranted` InOptionalPayload))
  (`parent.DoOnGiveAbility` InOptionalPayload)
  ;[0.07812 0 1] HACK: This is a workaround for "SetByCaller" values that will come 1 frame later
  (`KismetSystemLibrary.DelayUntilNextTick`)
  (`|ExecutionSequence`
    (:`then_0`
      (switch `ECk_Ability_Duration_Policy` (`self.DurationPolicy`)
        (:`Instant`
          (`self.DoRequest_ActivateAbility` (make `Ck_Ability_Payload_OnActivate` __contextentity_2 __data_2))
          (`/CkFoundation/CkAbility/Utils_CkAbility_FL.[Ck][AbilityOwner] Request Revoke Ability (By Entity)` (`self.DoGet_AbilityOwnerEntity`) (`self.DoGet_AbilityEntity`)))
        (:`Duration`
          (bind _outnewtimer (`self.AddNewTimerForMagnitude` (`self.DoGet_AbilityEntity`) (`self.DoGet_AbilityOwnerEntity`) (struct :`TagName` "Ck.Ability.Duration") (`self.DurationMagnitude`)))
          (`|Blueprint_Template` (struct) _outnewtimer
            (:`then`
              (if (`self.IsPeriodicEffect`) :!label _label
                (bind _outnewtimer_2 (`self.AddNewTimerForMagnitude` (`self.DoGet_AbilityEntity`) (`self.DoGet_AbilityOwnerEntity`) (struct :`TagName` "Ck.Ability.Period") (`self.PeriodMagnitude`)))
                (bind (_taskobject _timerdone_outtimerentity) (`|Blueprint_Template` (struct) _outnewtimer_2)
                  (:`then`
                    (if (`self.ExecutePeriodicEffectOnApplication`)
                      (`self.DoRequest_ActivateAbility` (struct))))
                  (:`TimerDone`
                    (bind _returnvalue (`Ck_Utils_Timer_UE.Request_Reset` _timerdone_outtimerentity))
                    (`Ck_Utils_Timer_UE.Request_Resume` _returnvalue)
                    (`self.DoRequest_ActivateAbility` (struct))))
                (else
                  (`self.DoRequest_ActivateAbility` (make `Ck_Ability_Payload_OnActivate` __contextentity __data)))))
            (:`TimerDone`
              (`self.OnDurationElapsed` (`self.DoGet_AbilityOwnerEntity`) (`self.DoGet_AbilityEntity`)))))
        (:`Infinite`
          (goto _label))))
    (:`then_1`
      (switch `ECk_Ability_Stacking_Policy` (`self.StackingPolicy`)
        (:`Stack_AggregateBySource`
          _)
        (:`Stack_AggregateByTarget`
          _))
      (`self.OnStackAdded` (`self.DoGet_AbilityOwnerEntity`) (`self.DoGet_AbilityEntity`)))))

(event `self.DoOnDeactivateAbility`
  (`parent.DoOnDeactivateAbility`))

(event `self.DoOnActivateAbility`
  (params (InActivationPayload :type "Ck_Ability_Payload_OnActivate Structure (by ref)"))
  ;[1 0.5625 0] Apply Effect
  (`parent.DoOnActivateAbility` InActivationPayload)
  (`self.ApplyEffect` (`self.DoGet_AbilityOwnerEntity`) (`self.DoGet_AbilityEntity`))
  (`self.DoRequest_DeactivateAbility`))

(event `self.DoOnRevokeAbility`
  (`parent.DoOnRevokeAbility`)
  (switch `ECk_Ability_Stacking_Policy` (`self.StackingPolicy`)
    (:`Stack_AggregateBySource`
      _)
    (:`Stack_AggregateByTarget`
      _))
  (`self.OnStackRemoved` (`self.DoGet_AbilityOwnerEntity`) (`self.DoGet_AbilityEntity`)))

(fn `AddNewTimerForMagnitude`
  (params (InAbility :type "Ck_Handle_Ability Structure") (InAbilityOwner :type "Ck_Handle_AbilityOwner Structure") (InTimerName :type "GameplayTag Structure") (InMagnitude :type "Ck_Ability_Magnitude Structure (by ref)"))
  (returns (OutNewTimer :type "Ck_Handle_Timer Structure"))
  (bind (__magnitudecalculation __attributesource __attributebasedmagnitude __snapshot __discretevaluemagnitude __setbycallermagnitude_datatag) (break `Ck_Ability_Magnitude` InMagnitude))
  (switch `ECk_Ability_Modifier_MagnitudeCalculation_Policy` __magnitudecalculation
    (:`DiscreteValue`
      (bind _outnewtimer (`/CkFoundation/CkTimer/Utils_CkTimer_FL.[Ck][Timer] Add New Timer` InTimerName (`local.InAbility`) __discretevaluemagnitude "PauseOnDone" "Running"))
      (return _outnewtimer))
    (:`AttributeBased`
      (bind _outcalculatedmagnitude (`/CkFoundation/CkAttribute/FloatAttribute/Utils_Float_CkAttribute_FL.[Ck][FloatAttribute] Calculate Attribute Magnitude` (`self.Get_SourceOrTarget_ForAbility` (`local.InAbility`) __attributesource) __attributebasedmagnitude))
      (bind _outnewtimer_2 (`/CkFoundation/CkTimer/Utils_CkTimer_FL.[Ck][Timer] Add New Timer` InTimerName (`local.InAbility`) _outcalculatedmagnitude "PauseOnDone" "Running"))
      (return _outnewtimer_2))
    (:`SetByCaller`
      (bind _value (`/CkFoundation/CkAttribute/FloatAttribute/Utils_Float_CkAttribute_FL.[Ck][FloatAttribute] Try Get Final Value_Or (Exec)` (`local.InAbility`) __setbycallermagnitude_datatag)
        (:`HasAttribute`
          (bind _outnewtimer_3 (`/CkFoundation/CkTimer/Utils_CkTimer_FL.[Ck][Timer] Add New Timer` InTimerName (`local.InAbility`) _value "PauseOnDone" "Running"))
          (return _outnewtimer_3))
        (:`MissingAttribute`
          (return))))))

(fn `ApplyEffect`
  (params (InAbilityOwner :type "Ck_Handle_AbilityOwner Structure") (InAbility :type "Ck_Handle_Ability Structure"))
  (locals (L_AttributeModifierValue :type "Float (single-precision)" :default 0.0) (L_Modifier :type "Ck_Ability_Modifier Structure") (L_ModifierMagnitude :type "Ck_Ability_Magnitude Structure") (L_AttributeToModify :type "GameplayTag Structure") (L_ModifierOperation :type "ECk_AttributeModifier_Operation Enum"))
  (bind _inability (`local.InAbility`))
  (bind (__attributetomodify __modifieroperation __modifiermagnitude) (break `Ck_Ability_Modifier` (`local.L_Modifier`)))
  (for _array_element (`self.Modifiers`)
    (set `local.L_Modifier` _array_element)
    (`|ExecutionSequence`
      (:`then_0`
        (set `local.L_AttributeToModify` __attributetomodify)
        (set `local.L_ModifierOperation` __modifieroperation)
        (bind _output_get (set `local.L_ModifierMagnitude` __modifiermagnitude))
        (bind (__magnitudecalculation __attributesource __attributebasedmagnitude __snapshot __discretevaluemagnitude __setbycallermagnitude_datatag) (break `Ck_Ability_Magnitude` _output_get))
        (switch `ECk_Ability_Modifier_MagnitudeCalculation_Policy` __magnitudecalculation
          (:`DiscreteValue`
            (set `local.L_AttributeModifierValue` __discretevaluemagnitude))
          (:`AttributeBased`
            (bind _outcalculatedmagnitude (`/CkFoundation/CkAttribute/FloatAttribute/Utils_Float_CkAttribute_FL.[Ck][FloatAttribute] Calculate Attribute Magnitude` (`self.Get_SourceOrTarget_ForAbility` _inability __attributesource) __attributebasedmagnitude))
            (set `local.L_AttributeModifierValue` _outcalculatedmagnitude))
          (:`SetByCaller`
            (set `local.L_AttributeModifierValue` (`.Value` (`/CkFoundation/CkAttribute/FloatAttribute/Utils_Float_CkAttribute_FL.[Ck][FloatAttribute] Try Get Final Value_Or` _inability __setbycallermagnitude_datatag))))))
      (:`then_1`
        (switch `ECk_AttributeModifier_Operation` (`local.L_ModifierOperation`)
          (:`Add`
            (`/CkFoundation/CkAttribute/FloatAttribute/Utils_Float_CkAttribute_FL.[Ck][FloatAttribute] Modify (NotRevocable)` (`local.InAbilityOwner`) (`local.L_AttributeToModify`) (`local.L_AttributeModifierValue`)))
          (:`Subtract`
            (`/CkFoundation/CkAttribute/FloatAttribute/Utils_Float_CkAttribute_FL.[Ck][FloatAttribute] Modify (NotRevocable)` (`local.InAbilityOwner`) (`local.L_AttributeToModify`) (`local.L_AttributeModifierValue`) "Current" "Subtract"))
          (:`Multiply`
            (`/CkFoundation/CkAttribute/FloatAttribute/Utils_Float_CkAttribute_FL.[Ck][FloatAttribute] Modify (NotRevocable)` (`local.InAbilityOwner`) (`local.L_AttributeToModify`) (`local.L_AttributeModifierValue`) "Current" "Multiply"))
          (:`Divide`
            (`/CkFoundation/CkAttribute/FloatAttribute/Utils_Float_CkAttribute_FL.[Ck][FloatAttribute] Modify (NotRevocable)` (`local.InAbilityOwner`) (`local.L_AttributeToModify`) (`local.L_AttributeModifierValue`) "Current" "Divide"))
          (:`Override`
            (`Ck_Utils_FloatAttribute_UE.Request_Override` (`Ck_Utils_FloatAttribute_UE.TryGet` (`local.InAbilityOwner`) (`local.L_AttributeToModify`)) (`local.L_AttributeModifierValue`))))))))

(fn `DoGet_CanBeGiven`
  (params (InAbilityOwner :type "Ck_Handle_AbilityOwner Structure (by ref)"))
  (returns (ReturnValue :type Boolean))
  (locals (L_ThisAbility_InstanceCount :type Integer :default 0))
  ;[1 0 0.3984] TODO: Pass in the Source
  (set `local.L_ThisAbility_InstanceCount` (`Ck_Utils_AbilityOwner_UE.Get_AbilityCount_OfClass` InAbilityOwner (`GameplayStatics.GetObjectClass` self)))
  (switch `ECk_Ability_Stacking_Policy` (`self.StackingPolicy`)
    (:`DoesNotStack`
      (return (`/CkFoundation/CkCore/Math/Math_CkCore_ML.<=0int` (`local.L_ThisAbility_InstanceCount`))))
    (:`Stack_AggregateBySource`
      (`Ck_Utils_Ensure_UE.TriggerEnsure` (`|FormatText` "Ability Stacking Policy [{policy}] is NOT supported yet!" (`|GetEnumeratorNameAsString` (`self.StackingPolicy`)))))
    (:`Stack_AggregateByTarget`
      (return (< (`local.L_ThisAbility_InstanceCount`) (`self.StackLimitCount`))))))

(fn `Get_SourceOrTarget_ForAbility`
  (params (InAbility :type "Ck_Handle_Ability Structure") (InSourceOrTarget :type "ECk_SourceOrTarget Enum" :default "Source"))
  (returns (OurEntity :type "Ck_Handle Structure"))
  (switch `ECk_SourceOrTarget` InSourceOrTarget
    (:`Source`
      ;[1 0 0.8203] TODO: Update this once we store the Source
      (return (`Ck_Utils_EntityLifetime_UE.Get_LifetimeOwner` InAbility)))
    (:`Target`
      (return (`Ck_Utils_EntityLifetime_UE.Get_LifetimeOwner` InAbility)))))

(fn `OnDurationElapsed`
  (params (InAbilityOwner :type "Ck_Handle_AbilityOwner Structure") (InAbility :type "Ck_Handle_Ability Structure"))
  (locals (L_FirstAbilityEntityOfClass_InTheStack :type "Ck_Handle_Ability Structure"))
  (switch `ECk_Ability_Stacking_Policy` (`self.StackingPolicy`)
    (:`DoesNotStack`
      (`/CkFoundation/CkAbility/Utils_CkAbility_FL.[Ck][AbilityOwner] Request Revoke Ability (By Entity)` (`local.InAbilityOwner`) (`local.InAbility`)))
    (:`Stack_AggregateBySource`
      (switch `ECk_Ability_StackExpiration_Policy` (`self.StackExpirationPolicy`) :!label _label
        (:`ClearEntireStack`
          (`/CkFoundation/CkAbility/Utils_CkAbility_FL.[Ck][AbilityOwner] Request Revoke Ability (By Entity)` (`local.InAbilityOwner`) (`local.InAbility`)))
        (:`RemoveSingleStackAndRefreshDuration`
          (set `local.L_FirstAbilityEntityOfClass_InTheStack` (`Ck_Utils_AbilityOwner_UE.TryGet_AbilityByClass` (`local.InAbilityOwner`) (`GameplayStatics.GetObjectClass` self)))
          (if (`Ck_Utils_Handle_UE.IsEqual` (`local.L_FirstAbilityEntityOfClass_InTheStack`) (`local.InAbility`))
            (`/CkFoundation/CkAbility/Utils_CkAbility_FL.[Ck][AbilityOwner] Request Revoke Ability (By Entity)` (`local.InAbilityOwner`) (`local.L_FirstAbilityEntityOfClass_InTheStack`))
            (else
              (`self.RefreshEffectDuration` (`local.InAbility`)))))))
    (:`Stack_AggregateByTarget`
      (goto _label))))

(fn `OnStackAdded`
  (params (InAbilityOwner :type "Ck_Handle_AbilityOwner Structure") (InAbilityAdded :type "Ck_Handle_Ability Structure"))
  (locals (L_DurationTimer :type "Ck_Handle_Timer Structure") (L_Ability :type "Ck_Handle_Ability Structure") (L_PeriodTimer :type "Ck_Handle_Timer Structure"))
  (bind _returnvalue (`Ck_Utils_AbilityOwner_UE.ForEach_Ability_OfClass` InAbilityOwner (`GameplayStatics.GetObjectClass` self)))
  (for _array_element _returnvalue
    (set `local.L_Ability` _array_element)
    (`|ExecutionSequence`
      (:`then_0`
        ;[0 1 0.6484] Try Refresh Duration
        (switch `ECk_Ability_StackDurationRefresh_Policy` (`self.StackDurationRefreshPolicy`)
          (:`RefreshOnSuccessfulApplication`
            (bind _output_get (set `local.L_DurationTimer` (`Ck_Utils_Timer_UE.TryGet_Timer` (`local.L_Ability`) (struct :`TagName` "Ck.Ability.Duration"))))
            (bind _outhandle (`/CkFoundation/CkEcs/EntityHandle_CkEcs_ML.ValidateEntityHandle` _output_get)
              (:`IsValid`
                (bind _returnvalue_2 (`Ck_Utils_Timer_UE.Request_Reset` _outhandle))
                (`Ck_Utils_Timer_UE.Request_Resume` _returnvalue_2))))))
      (:`then_1`
        ;[0.8984 0 1] Try Refresh Period
        (switch `ECk_Ability_StackPeriodReset_Policy` (`self.StackPeriodResetPolicy`)
          (:`ResetOnSuccessfulApplication`
            (bind _output_get_2 (set `local.L_PeriodTimer` (`Ck_Utils_Timer_UE.TryGet_Timer` (`local.L_Ability`) (struct :`TagName` "Ck.Ability.Period"))))
            (bind _outhandle_2 (`/CkFoundation/CkEcs/EntityHandle_CkEcs_ML.ValidateEntityHandle` _output_get_2)
              (:`IsValid`
                (bind _returnvalue_3 (`Ck_Utils_Timer_UE.Request_Reset` _outhandle_2))
                (`Ck_Utils_Timer_UE.Request_Resume` _returnvalue_3)))))))))

(fn `OnStackRemoved`
  (params (InAbilityOwner :type "Ck_Handle_AbilityOwner Structure") (InAbilityRemoved :type "Ck_Handle_Ability Structure")))

(fn `RefreshEffectDuration`
  (params (InHandle :type "Ck_Handle Structure"))
  (bind _outhandle (`/CkFoundation/CkEcs/EntityHandle_CkEcs_ML.ValidateEntityHandle` (`Ck_Utils_Timer_UE.TryGet_Timer` InHandle (struct :`TagName` "Ck.Ability.Duration")))
    (:`IsValid`
      (bind _returnvalue (`Ck_Utils_Timer_UE.Request_Reset` _outhandle))
      (`Ck_Utils_Timer_UE.Request_Resume` _returnvalue))))

(fn `ResetEffectPeriod`
  (params (InHandle :type "Ck_Handle Structure"))
  (bind _outhandle (`/CkFoundation/CkEcs/EntityHandle_CkEcs_ML.ValidateEntityHandle` (`Ck_Utils_Timer_UE.TryGet_Timer` InHandle (struct :`TagName` "Ck.Ability.Period")))
    (:`IsValid`
      (bind _returnvalue (`Ck_Utils_Timer_UE.Request_Reset` _outhandle))
      (`Ck_Utils_Timer_UE.Request_Resume` _returnvalue))))