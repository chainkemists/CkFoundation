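; Base Blueprint for CkAbility costs paid from a float attribute on the ability owner.
; The cost is met when the named attribute's current value passes a configurable comparison.
; Applying it adds a non-revocable modifier to that attribute, using a configured delta and operation.
; While granted, it listens for attribute value changes to call TryAddCostNotMet, and unbinds on revoke.
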(event `self.DoOnGiveAbility`
  (params (InOptionalPayload :type "Ck_Ability_Payload_OnGranted Structure (by ref)"))
  (`parent.DoOnGiveAbility` InOptionalPayload)
  (`Ck_Utils_FloatAttribute_UE.BindTo_OnValueChanged` (`self.DoGet_AbilityOwnerEntity`) (`self.AttributeName`) "FireIfPayloadInFlightThisFrame" "DoNothing" (delegate `OnAttributeChanged`)))

(event `OnAttributeChanged`
  (params (InHandle :type "Ck_Handle Structure") (InPayload :type "Ck_Payload_FloatAttribute_OnValueChanged Structure"))
  (`self.TryAddCostNotMet`))

(event `self.DoOnRevokeAbility`
  (`parent.DoOnRevokeAbility`)
  (`Ck_Utils_FloatAttribute_UE.UnbindFrom_OnValueChanged` (`self.DoGet_AbilityOwnerEntity`) (`self.AttributeName`) (`|CreateDelegate` :!event `OnAttributeChanged`)))

(fn `ApplyCost`
  (params (InContextEntity :type "Ck_Handle Structure") (InData :type "InstancedStruct Structure"))
  (`parent.ApplyCost` InContextEntity InData)
  (`Ck_Utils_FloatAttributeModifier_UE.Add` (`self.DoGet_AbilityOwnerEntity`) (struct) (make `Ck_Fragment_FloatAttributeModifier_ParamsData` (`self.CostDelta`) (`self.AttributeName`) (`self.CostModifierOperation`) "NotRevocable")))

(fn `Get_IsCostMet`
  (returns (OutResult :type Boolean))
  (return (`Ck_Utils_FloatComparison_UE.Get_IsComparisonTrue` (`Ck_Utils_NumericAttribute_UE.Get_CurrentValue` (`self.DoGet_AbilityOwnerEntity`) (`self.AttributeName`)) (`self.AttributeComparison`))))