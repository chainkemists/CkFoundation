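; Base Blueprint for ability costs in the Ck ability system, itself built as an ability whose active state signals that the cost is not met.
; When given, it activates if GetIsCostMet fails and deactivates otherwise, then listens on the owner for the ApplyCost trigger event.
; That event calls ApplyCost with its context and data.
; Subclasses override GetIsCostMet, which defaults to true, and the empty ApplyCost.
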(event `self.DoOnGiveAbility`
  (params (InOptionalPayload :type "Ck_Ability_Payload_OnGranted Structure (by ref)"))
  (`self.TryAddCostNotMet`)
  (`parent.DoOnGiveAbility` InOptionalPayload)
  (bind (_taskobject _eventfired_outabilityownerhandle _eventfired_outevent) (`|Blueprint_Template` (`self.DoGet_AbilityOwnerEntity`) (struct :`GameplayTags` (struct :`(TagName` "Ck.AbilityTrigger.ApplyCost"))))
    (:`EventFired`
      (bind (__eventname __contextentity __eventdata) (break `Ck_AbilityOwner_Event` _eventfired_outevent))
      (`self.ApplyCost` (`self.DoGet_AbilityOwnerEntity`) (`self.DoGet_AbilityEntity`) __contextentity __eventdata))))

(fn `ApplyCost`
  (params (InAbilityOwner :type "Ck_Handle_AbilityOwner Structure") (InAbility :type "Ck_Handle_Ability Structure") (InContextEntity :type "Ck_Handle Structure") (InData :type "InstancedStruct Structure")))

(fn `Get_IsCostMet`
  (params (InAbilityOwner :type "Ck_Handle_AbilityOwner Structure") (InAbility :type "Ck_Handle_Ability Structure"))
  (returns (OutResult :type Boolean))
  ;[1 0.6797 0] To Override
  (return true))

(fn `Get_ThumbnailIconAndColor`
  (returns (OutBackgroundColor :type "LinearColor Structure") (ReturnValue :type "Texture2D Object Reference"))
  (return (struct :`R` 0.01033 :`G` 0.01033 :`B` 0.01033 :`A` 1.0) "/CkFoundation/Textures/Icon_AbilityCost_64px.Icon_AbilityCost_64px"))

(fn `TryAddCostNotMet`
  (if (`self.Get_IsCostMet` (`self.DoGet_AbilityOwnerEntity`) (`self.DoGet_AbilityEntity`))
    (`self.DoRequest_DeactivateAbility`)
    (else
      (`self.DoRequest_ActivateAbility` (struct)))))