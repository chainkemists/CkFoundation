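; Base ability Blueprint for applying a cost to an ability owner in the CkAbility framework.
; Subclasses supply the cost logic through ApplyCost and GetIsCostMet, which default to doing nothing and returning true.
; Activation applies the cost using the payload's context entity and data, then requests immediate deactivation.
; Both give and activation check the cost, sending an ApplyCostsNotMet event to the owner when it is not met.
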(event `self.DoOnGiveAbility`
  (`self.DoTryAddCostNotMet`)
  (`parent.DoOnGiveAbility`))

(event `self.DoOnActivateAbility`
  (params (InActivationPayload :type "Ck_Ability_ActivationPayload Structure (by ref)"))
  (bind (__contextentity __data) (break `Ck_Ability_ActivationPayload` InActivationPayload))
  (`parent.DoOnActivateAbility` InActivationPayload)
  (`self.ApplyCost` __contextentity __data)
  (`self.DoTryAddCostNotMet`)
  (`self.DoRequest_DeactivateAbility`))

(fn `ApplyCost`
  (params (InContextEntity :type "Ck_Handle Structure") (InData :type "InstancedStruct Structure")))

(fn `DoTryAddCostNotMet`
  (if (not (`self.Get_IsCostMet`))
    (`Ck_Utils_AbilityOwner_UE.Request_SendAbilityEvent` (`self.DoGet_AbilityOwnerEntity`) (make `Ck_Request_AbilityOwner_SendEvent` (make `Ck_AbilityOwner_Event` (struct :`TagName` "Ck.AbilityTrigger.ApplyCostsNotMet"))))))

(fn `Get_IsCostMet`
  (returns (OutResult :type Boolean))
  ;[1 0.6797 0] To Override
  (return true))