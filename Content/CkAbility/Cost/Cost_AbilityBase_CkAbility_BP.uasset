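; Base Blueprint for ability costs in the CkAbility system, with IsCostMet and ApplyCost as stubs for subclasses.
; When given, it activates itself if the cost is unmet and deactivates if met, so its active state represents "cost not met".
; It also starts a tracked event-listening task on the owner, calling ApplyCost with the first ApplyCostTag event's context and data.
; Revoking deactivates that task.
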(event `self.DoOnGiveAbility`
  (params (InOptionalPayload :type "Ck_Ability_Payload_OnGranted Structure (by ref)"))
  (`self.TryAddCostNotMet`)
  (`parent.DoOnGiveAbility` InOptionalPayload)
  (bind (_taskobject _eventsfired_outabilityownerentity _eventsfired_outevents) (`|Blueprint_Template` (struct) (`self.DoGet_AbilityOwnerEntity`) :!label _label)
    (:`then`
      (`self.DoRequest_TrackTask` _taskobject))
    (:`EventsFired`
      (bind (_outresult _outcontextentity _outeventdata) (`self.DoGet_NeedToApplyCost` _eventsfired_outevents))
      (if _outresult
        (`self.ApplyCost` (`self.DoGet_AbilityOwnerEntity`) (`self.DoGet_AbilityEntity`) _outcontextentity _outeventdata)))))

(event `self.DoOnRevokeAbility`
  (`parent.DoOnRevokeAbility`)
  (goto _label :!via `Deactivate`))

(fn `ApplyCost`
  (params (InAbilityOwner :type "Ck_Handle_AbilityOwner Structure") (InAbility :type "Ck_Handle_Ability Structure") (InContextEntity :type "Ck_Handle Structure") (InData :type "InstancedStruct Structure")))

(fn `DoGet_NeedToApplyCost`
  (params (InEvents :type "Array of Ck_AbilityOwner_Event Structure"))
  (returns (OutResult :type Boolean) (OutContextEntity :type "Ck_Handle Structure") (OutEventData :type "InstancedStruct Structure"))
  (for _array_element InEvents
    (bind (__eventname __contextentity __eventdata) (break `Ck_AbilityOwner_Event` _array_element))
    (if (== __eventname (`self.ApplyCostTag`))
      (return true __contextentity __eventdata)))
  (return false))

(fn `Get_IsCostMet`
  (params (InAbilityOwner :type "Ck_Handle_AbilityOwner Structure") (InAbility :type "Ck_Handle_Ability Structure"))
  (returns (OutResult :type Boolean))
  ;[1 0.6797 0] To Override
  (return true))

(fn `TryAddCostNotMet`
  (if (`self.Get_IsCostMet` (`self.DoGet_AbilityOwnerEntity`) (`self.DoGet_AbilityEntity`))
    (`self.DoRequest_DeactivateAbility`)
    (else
      (`self.DoRequest_ActivateAbility` (struct)))))