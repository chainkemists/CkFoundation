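; Base Blueprint for an ability cost paid from a float attribute, found by name in the ability entity's ownership chain.
; The cost is met when the attribute's current final value passes a configurable comparison.
; Applying it makes a non-revocable modification using a configured delta and operation.
; On give, it validates that the attribute exists and listens for changes to re-evaluate the cost-not-met state.
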(event `self.DoOnGiveAbility`
  (params (InOptionalPayload :type "Ck_Ability_Payload_OnGranted Structure (by ref)"))
  (bind _outattribute (`/CkFoundation/CkAttribute/FloatAttribute/Utils_Float_CkAttribute_FL.[Ck][FloatAttribute] Try Get Attribute In Ownership Chain` (`self.DoGet_AbilityEntity`) (`self.AttributeName`)))
  (`parent.DoOnGiveAbility` InOptionalPayload)
  (`Ck_Utils_EcsEnsure_UE.EnsureMsgf_IsValid` _outattribute (`|FormatText` "Could not find Attribute [{Attribute}] in the Ownership chain starting with Entity [{ability}]" (`BlueprintGameplayTagLibrary.GetTagName` (`self.AttributeName`)) (`Ck_Utils_Handle_UE.Conv_HandleToText` (`self.DoGet_AbilityEntity`)))
    (:`Valid`
      (`|Blueprint_Template` _outattribute
        (:`AttributeChanged`
          (`self.TryAddCostNotMet`))))))

(fn `ApplyCost`
  (params (InAbilityOwner :type "Ck_Handle_AbilityOwner Structure") (InAbility :type "Ck_Handle_Ability Structure") (InContextEntity :type "Ck_Handle Structure") (InData :type "InstancedStruct Structure"))
  (`parent.ApplyCost` InAbilityOwner InAbility InContextEntity InData)
  (`/CkFoundation/CkAttribute/FloatAttribute/Utils_Float_CkAttribute_FL.[Ck][FloatAttribute] Modify (NotRevocable)` (`Ck_Utils_FloatAttribute_UE.TryGet_Entity_WithAttribute_InOwnershipChain` InAbility (`self.AttributeName`)) (`self.AttributeName`) (`self.CostDelta`) "Current" (`self.CostModifierOperation`)))

(fn `Get_IsCostMet`
  (params (InAbilityOwner :type "Ck_Handle_AbilityOwner Structure") (InAbility :type "Ck_Handle_Ability Structure"))
  (returns (OutResult :type Boolean))
  (return (`Ck_Utils_FloatComparison_UE.Get_IsComparisonTrue` (`Ck_Utils_FloatAttribute_UE.Get_FinalValue` (`/CkFoundation/CkAttribute/FloatAttribute/Utils_Float_CkAttribute_FL.[Ck][FloatAttribute] Try Get Attribute In Ownership Chain` InAbility (`self.AttributeName`))) (`self.AttributeComparison`))))