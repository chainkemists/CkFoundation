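; Base Blueprint for a duration-based ability cooldown that keeps the ability active until the cooldown time elapses.
; On activation, it creates a transient entity with a timer set to the cooldown duration and adds it as an extension of the ability entity.
; When the timer finishes, it destroys that entity and requests deactivation.
; Deactivation also force-destroys the timer entity.
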(event `self.DoOnActivateAbility`
  (params (InActivationPayload :type "Ck_Ability_Payload_OnActivate Structure (by ref)"))
  (`parent.DoOnActivateAbility` InActivationPayload)
  (bind _returnvalue (`Ck_Utils_EntityLifetime_UE.Request_CreateEntity_TransientOwner`))
  (bind _output_get (set `self._EntityWithTimer` _returnvalue))
  (bind _outnewtimer (`/CkFoundation/CkTimer/Utils_CkTimer_FL.[Ck][Timer] Add Or Replace Timer` _output_get (struct) (`._Seconds` (break `Ck_Time` (`self.CooldownDuration`))) "PauseOnDone" "Running"))
  (bind _returnvalue_2 (`Ck_Utils_Timer_UE.Request_Reset` _outnewtimer))
  (bind _returnvalue_3 (`Ck_Utils_Timer_UE.Request_Resume` _returnvalue_2))
  (`|Blueprint_Template` _returnvalue_3
    (:`then`
      (`Ck_Utils_EntityExtension_UE.Add` (`self.DoGet_AbilityEntity`) (`self._EntityWithTimer`)))
    (:`TimerDone`
      (`Ck_Utils_EntityLifetime_UE.Request_DestroyEntity` (`self._EntityWithTimer`))
      (`self.DoRequest_DeactivateAbility`))))

(event `self.DoOnDeactivateAbility`
  (`parent.DoOnDeactivateAbility`)
  (`Ck_Utils_EntityLifetime_UE.Request_DestroyEntity` (`self._EntityWithTimer`)))