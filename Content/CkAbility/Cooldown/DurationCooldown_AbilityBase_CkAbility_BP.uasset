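; Base ability Blueprint for a duration-based cooldown in the Ck ability framework, which stays active for a set cooldown time and then ends itself.
; On activation it adds or replaces an optionally named timer on the ability entity, using the cooldown duration, and binds to its completion.
; When the timer finishes, the ability requests its own deactivation, and deactivation force-destroys the timer entity.
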(event `self.DoOnActivateAbility`
  (params (InActivationPayload :type "Ck_Ability_ActivationPayload Structure (by ref)"))
  (`parent.DoOnActivateAbility` InActivationPayload)
  (bind _returnvalue (`Ck_Utils_Timer_UE.AddOrReplace` (`self.DoGet_AbilityEntity`) (make `Ck_Fragment_Timer_ParamsData` (`self.OptionalTimerName`) (`self.CooldownDuration`) "CountUp" "PauseOnDone" "Running")))
  (set `self._TimerHandle` _returnvalue)
  (`Ck_Utils_Timer_UE.BindTo_OnDone` (`self._TimerHandle`) "FireIfPayloadInFlightThisFrame" (delegate `OnDone`)))

(event `OnDone`
  (params (InHandle :type "Ck_Handle Structure") (InChrono :type "Ck_Chrono Structure"))
  (`self.DoRequest_DeactivateAbility`))

(event `self.DoOnDeactivateAbility`
  (`parent.DoOnDeactivateAbility`)
  (`Ck_Utils_EntityLifetime_UE.Request_DestroyEntity` (`self._TimerHandle`)))