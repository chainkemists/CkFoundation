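; An animation notify that sends a gameplay-tagged ability event to the owning entity when an animation reaches it.
; On notify, it casts the owner entity to an AbilityOwner and requests the event with the owner as context, triggering an ensure if the cast fails.
; Event data comes from an overridable getter that returns the EventData property by default.
; The notify name shows the configured tag, flagging invalid ones.
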(fn `[Ck] Received_Notify (Override)`
  (params (InOwnerActor :type "Actor Object Reference") (InOwnerEntity :type "Ck_Handle Structure") (InMeshComp :type "SkeletalMeshComponent Object Reference") (InAnimation :type "AnimSequenceBase Object Reference") (InEventReference :type "AnimNotifyEventReference Structure"))
  (returns (OutResult :type Boolean))
  (bind _returnvalue (`Ck_Utils_AbilityOwner_UE.DoCast` InOwnerEntity)
    (:`Succeeded`
      (`/CkFoundation/CkAbility/Utils_CkAbility_FL.[Ck][AbilityOwner] Request Send Ability Event` _returnvalue (`self.AbilityEventName`) (`local.InOwnerEntity`) (`self.Get_EventData (Override Optional)`))
      (return false))
    (:`Failed`
      (`Ck_Utils_Ensure_UE.TriggerEnsure` (`|FormatText` self "Anim Notify [{self}] used in Animation [{anim}] requires the Owner [{owner}] to be an AbilityOwner!" (`local.InAnimation`) (`Ck_Utils_Handle_UE.Conv_HandleToText` (`local.InOwnerEntity`)))))))

(fn `Get_EventData (Override Optional)`
  (returns (EventData :type "InstancedStruct Structure"))
  (return (`self.EventData`)))

(fn `GetNotifyName`
  (returns (ReturnValue :type String))
  (if (`BlueprintGameplayTagLibrary.IsGameplayTagValid` (`self.AbilityEventName`))
    (return (`KismetTextLibrary.Conv_TextToString` (`|FormatText` "[Ck] SendAbilityEvent [{tag}]" (`BlueprintGameplayTagLibrary.GetTagName` (`self.AbilityEventName`)))))
    (else
      (return "[Ck] SendAbilityEvent [INVALID_TAG]"))))