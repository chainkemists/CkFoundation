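; Ability condition base that passes or fails based on comparing a byte attribute's value.
; When given, it finds the named attribute in the ability's ownership chain; a missing one succeeds if optional, otherwise triggers an ensure and fails.
; A found attribute's base, bonus or final value is compared against the configured comparison.
; The optional path also binds to attribute changes and re-evaluates the condition on each change.
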(event `self.DoOnGiveAbility`
  (params (InOptionalPayload :type "Ck_Ability_Payload_OnGranted Structure (by ref)"))
  (`parent.DoOnGiveAbility` InOptionalPayload)
  (bind _output_get (set `self._Attribute` (`/CkFoundation/CkAttribute/ByteAttribute/Utils_Byte_CkAttribute_FL.[Ck][ByteAttribute] Try Get Attribute In Ownership Chain` (`self.DoGet_AbilityEntity`) (`self.AttributeName`))))
  (if (`self.Optional`)
    (bind _outhandle (`/CkFoundation/CkEcs/EntityHandle_CkEcs_ML.ValidateEntityHandle` _output_get)
      (:`IsValid`
        (`self.DoEvaluateAttributeValueComparison` _outhandle :!label _label)
        (bind (_taskobject _attributechanged_outattributeownerhandle _attributechanged_outatributehandle) (`|Blueprint_Template` _outhandle (`self.AttributeComponent`))
          (:`AttributeChanged`
            (`self.DoEvaluateAttributeValueComparison` _attributechanged_outatributehandle))))
      (:`NotValid`
        (`self.OnCondition_Success`)))
    (else
      (`Ck_Utils_EcsEnsure_UE.EnsureMsgf_IsValid` _outhandle (`|FormatText` "Could not find Attribute [{Attribute}] in the Ownership chain starting with Entity [{ability}]" (`BlueprintGameplayTagLibrary.GetTagName` (`self.AttributeName`)) (`Ck_Utils_Handle_UE.Conv_HandleToText` (`self.DoGet_AbilityEntity`)))
        (:`Valid`
          (goto _label))
        (:`Invalid`
          (`self.OnCondition_Fail`))))))

(fn `DoEvaluateAttributeValueComparison`
  (params (InAttributeEntity :type "Ck_Handle_ByteAttribute Structure"))
  (locals (L_AttributeValue :type Byte :default 0))
  (`/CkFoundation/CkEcs/EntityHandle_CkEcs_ML.ValidateEntityHandle` InAttributeEntity
    (:`IsValid`
      (`|ExecutionSequence`
        (:`then_0`
          (switch `ECk_Attribute_BaseBonusFinal` (`self.AttributeBaseBonusFinal`)
            (:`Base`
              (set `local.L_AttributeValue` (`Ck_Utils_ByteAttribute_UE.Get_BaseValue` (`local.InAttributeEntity`) (`self.AttributeComponent`))))
            (:`Bonus`
              (set `local.L_AttributeValue` (`Ck_Utils_ByteAttribute_UE.Get_BonusValue` (`local.InAttributeEntity`) (`self.AttributeComponent`))))
            (:`Final`
              (set `local.L_AttributeValue` (`Ck_Utils_ByteAttribute_UE.Get_FinalValue` (`local.InAttributeEntity`) (`self.AttributeComponent`))))))
        (:`then_1`
          (if (`Ck_Utils_IntComparison_UE.Get_IsComparisonTrue` (`KismetMathLibrary.Conv_ByteToInt` (`local.L_AttributeValue`)) (`self.AttributeComparison`))
            (`self.OnCondition_Success`)
            (else
              (`self.OnCondition_Fail`))))))
    (:`NotValid`
      (`self.OnCondition_Fail`))))