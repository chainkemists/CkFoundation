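; Base ability for trait conditions, which gate when the owning trait activates its payoffs.
; On give, it listens for events on the trait, tests each with overridable EvaluateTraitTriggerCondition (passes by default), then queues passing payloads and signals condition success or failure.
; On deactivate, it requests trait activation with the first queued payload if requirements are met, then resets to failed and dequeues it.
; Trait activation fires the overridable OnSuccessfulTraitTrigger hook.
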(event `self.DoOnGiveAbility`
  (params (InOptionalPayload :type "Ck_Ability_Payload_OnGranted Structure (by ref)"))
  (`parent.DoOnGiveAbility` InOptionalPayload)
  (`self.OnCondition_Fail`)
  (bind (_taskobject _eventsfired_outabilityownerentity _eventsfired_outevents) (`|Blueprint_Template` (`self.DoGet_AbilityOwnerEntity`))
    (:`then`
      (`self.DoRequest_AddTaskToDeactivateOnRevoke` _taskobject)
      (bind _taskobject_2 (`|Blueprint_Template` (`Ck_Utils_Ability_UE.DoCastChecked` (`self.DoGet_AbilityOwnerEntity`)))
        (:`then`
          (`self.DoRequest_AddTaskToDeactivateOnRevoke` _taskobject_2))
        (:`AbilityActivated`
          (`self.OnSuccessfulTraitTrigger`))))
    (:`EventsFired`
      (for _array_element _eventsfired_outevents
        (bind (__eventname __contextentity __eventdata) (break `Ck_AbilityOwner_Event` _array_element))
        (bind _outconditionresult (`self.EvaluateTraitTriggerCondition` __contextentity __eventdata))
        (switch `ECk_SucceededFailed` _outconditionresult
          (:`Succeeded`
            (`KismetArrayLibrary.Array_Add` (`self._TraitPayloadsToProcess`) _array_element)
            (`self.OnCondition_Success`))
          (:`Failed`
            (`self.OnCondition_Fail`)))))))

(event `self.DoOnDeactivateAbility`
  (bind _returnvalue (`self.DoGet_AbilityOwnerEntity`))
  (`parent.DoOnDeactivateAbility`)
  (bind _output (`/CkFoundation/CkCore/Container/Container_CkCore_ML.Array_GetFirstElementValidated` (`self._TraitPayloadsToProcess`))
    (:`IsValid`
      (switch `ECk_Ability_ActivationRequirementsResult` (`Ck_Utils_Ability_UE.Get_CanActivate` (`Ck_Utils_Ability_UE.DoCastChecked` (`self.DoGet_AbilityOwnerEntity`)))
        (:`RequirementsMet`
          (bind (__eventname __contextentity __eventdata) (break `Ck_AbilityOwner_Event` _output))
          ;[0.8516 0 1] Notify parent Trait to try to Activate (Payoffs)
          (`/CkFoundation/CkAbility/Utils_CkAbility_FL.[Ck][AbilityOwner] Request Try Activate Ability (By Entity)` (`Ck_Utils_AbilityOwner_UE.DoCastChecked` (`Ck_Utils_EntityLifetime_UE.Get_LifetimeOwner` _returnvalue)) (`Ck_Utils_Ability_UE.DoCastChecked` _returnvalue) (make `Ck_Ability_Payload_OnActivate` __contextentity __eventdata)))
        (:`RequirementsMet_ButAlreadyActive`
          _)
        (:`RequirementsNotMet_OnSelf`
          _)
        (:`RequirementsNotMet_OnOwner`
          _)
        (:`RequirementsNotMet_OnOwnerAndSelf`
          _))
      (`self.OnCondition_Fail`)
      (`KismetArrayLibrary.Array_Remove` (`self._TraitPayloadsToProcess`)))
    (:`NotValid`
      (`Ck_Utils_Log_UE.Log_Verbose` (`|FormatText` self "Ability trait condition [{self}] deactivated with no payoffs to process, this usually happens if the condition succeeds but was not evaluated as part of a trait message") (struct :`_Name` "CkAbilityExt")))))

(event `OnSuccessfulTraitTrigger`
  ;[1 0.2344 0] Override this
)

(fn `EvaluateTraitTriggerCondition`
  (params (InContextEntity :type "Ck_Handle Structure") (InTraitTriggerPayload :type "InstancedStruct Structure"))
  (returns (OutConditionResult :type "ECk_SucceededFailed Enum"))
  (return "Succeeded"))