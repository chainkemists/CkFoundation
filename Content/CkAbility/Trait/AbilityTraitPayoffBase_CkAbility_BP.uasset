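; Base Blueprint for trait payoff abilities in CkAbility, which can always be given by default.
; When given, it starts a task on the ability owner that requests this ability's activation whenever the task fires Ability Activated, registered to deactivate on revoke.
; On activation it passes the context entity and payload data to PayoffToTargets, an empty hook, then immediately requests its own deactivation.
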(event `self.DoOnGiveAbility`
  (params (InOptionalPayload :type "Ck_Ability_Payload_OnGranted Structure (by ref)"))
  (`parent.DoOnGiveAbility` InOptionalPayload)
  (bind (_taskobject _abilityalreadyactive_outabilityhandle _abilityactivated_outabilityhandle _abilityactivated_outactivationpayload) (`|Blueprint_Template` (`Ck_Utils_Ability_UE.DoCastChecked` (`self.DoGet_AbilityOwnerEntity`)))
    (:`then`
      (`self.DoRequest_AddTaskToDeactivateOnRevoke` _taskobject))
    (:`AbilityActivated`
      (`self.DoRequest_ActivateAbility` _abilityactivated_outactivationpayload))))

(event `self.DoOnActivateAbility`
  (params (InActivationPayload :type "Ck_Ability_Payload_OnActivate Structure (by ref)"))
  (bind (__contextentity __data) (break `Ck_Ability_Payload_OnActivate` InActivationPayload))
  (`parent.DoOnActivateAbility` InActivationPayload)
  (`self.PayoffToTargets` __contextentity __data)
  (`self.DoRequest_DeactivateAbility`))

(fn `DoGet_CanBeGiven`
  (params (InAbilityOwner :type "Ck_Handle_AbilityOwner Structure (by ref)") (InAbilitySource :type "Ck_Handle Structure (by ref)"))
  (returns (ReturnValue :type Boolean))
  ;[0 1 0.5313] Payoffs are always given by default
  (return true))

(fn `PayoffToTargets`
  (params (InContextEntity :type "Ck_Handle Structure") (InPayoffPayload :type "InstancedStruct Structure (by ref)")))