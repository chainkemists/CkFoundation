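; Base ability Blueprint for trait conditions, with empty evaluation and success hooks for children to fill in.
; On give, it starts an event-listening task on the ability owner, registers it to deactivate on revoke, then calls OnConditionFail.
; Each fired event matching the trait-triggered name calls OnSuccessfulTraitTrigger.
; All other events pass their context entity and data to EvaluateTraitTriggerCondition.
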(event `self.DoOnGiveAbility`
  (params (InOptionalPayload :type "Ck_Ability_Payload_OnGranted Structure (by ref)"))
  (`parent.DoOnGiveAbility` InOptionalPayload)
  (bind (_taskobject _eventsfired_outabilityownerentity _eventsfired_outevents) (`|Blueprint_Template` (`self.DoGet_AbilityOwnerEntity`))
    (:`then`
      (`self.DoRequest_AddTaskToDeactivateOnRevoke` _taskobject)
      (`self.OnCondition_Fail`))
    (:`EventsFired`
      (for _array_element _eventsfired_outevents
        (bind (__eventname __contextentity __eventdata) (break `Ck_AbilityOwner_Event` _array_element))
        (if (== __eventname (`self._TraitTriggeredEventName`))
          (`self.OnSuccessfulTraitTrigger`)
          (else
            (`self.EvaluateTraitTriggerCondition` __contextentity __eventdata)))))))

(event `self.DoOnRevokeAbility`
  (`parent.DoOnRevokeAbility`))

(event `OnSuccessfulTraitTrigger`)

(fn `EvaluateTraitTriggerCondition`
  (params (InContextEntity :type "Ck_Handle Structure") (InTraitTriggerPayload :type "InstancedStruct Structure")))