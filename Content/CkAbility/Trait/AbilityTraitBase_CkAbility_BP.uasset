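; Base Blueprint for CkAbility traits: always-givable abilities that bundle Condition and Payoff sub-abilities and respond to triggering events.
; When given, it ensures triggering events exist, then starts a message listener on the owner entity, torn down on revoke.
; Each message is forwarded to its sub-abilities as an ability event, then requests trait activation with that payload.
; Activation immediately requests deactivation, making each trigger a momentary pulse.
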(event `self.DoOnGiveAbility`
  (params (InOptionalPayload :type "Ck_Ability_Payload_OnGranted Structure (by ref)"))
  ;[0 1 0.6719] Forward Trigger Events to Sub-Abilities
  (`parent.DoOnGiveAbility` InOptionalPayload)
  (`Ck_Utils_Ensure_UE.EnsureMsgf` (`/CkFoundation/CkCore/Math/Math_CkCore_ML.>0int` (`BlueprintGameplayTagLibrary.GetNumGameplayTagsInContainer` (`self.TriggeringEvents (Messages)`))) (`|FormatText` self "Ability Trait [{self}] has NO TriggeringEvents set! Ability Trait will NOT work properly")
    (:`Valid`
      (bind (_taskobject _onnewmessage_outhandle _onnewmessage_outmessagename _onnewmessage_outpayload) (`|Blueprint_Template` (`Ck_Utils_Handle_UE.Get_RawHandle` (`self.DoGet_AbilityOwnerEntity`)) (`self.TriggeringEvents (Messages)`))
        (:`then`
          (`self.DoRequest_AddTaskToDeactivateOnRevoke` _taskobject))
        (:`OnNewMessage`
          (`/CkFoundation/CkAbility/Utils_CkAbility_FL.[Ck][AbilityOwner] Request Send Ability Event` (`Ck_Utils_AbilityOwner_UE.DoCastChecked` (`self.DoGet_AbilityEntity`)) _onnewmessage_outmessagename (`self.DoGet_AbilityOwnerEntity`) _onnewmessage_outpayload)
          (`self.DoRequest_ActivateAbility` (make `Ck_Ability_Payload_OnActivate` (`self.DoGet_AbilityOwnerEntity`) _onnewmessage_outpayload)))))))

(event `self.DoOnActivateAbility`
  (params (InActivationPayload :type "Ck_Ability_Payload_OnActivate Structure (by ref)"))
  ;[0 1 0.3438] Notify Payoff SubAbilities
  (`parent.DoOnActivateAbility` InActivationPayload)
  (`self.DoRequest_DeactivateAbility`))

(event `self.DoOnDeactivateAbility`
  (`parent.DoOnDeactivateAbility`))

(event `self.DoOnRevokeAbility`
  (`parent.DoOnRevokeAbility`))

(fn `DoGet_AdditionalSubAbilities`
  (returns (ReturnValue :type "Array of Ck_Ability_Script_PDA Object Reference"))
  (locals (L_AdditionalSubAbilities :type "Array of Ck_Ability_Script_PDA Object Reference"))
  (`KismetArrayLibrary.Array_Append` (`local.L_AdditionalSubAbilities`) (`._Conditions` (break `Ck_Ability_TraitCondition_Instances` (`self._TraitConditions`))))
  (`KismetArrayLibrary.Array_Append` (`local.L_AdditionalSubAbilities`) (`._Payoffs` (break `Ck_Ability_TraitPayoff_Instances` (`self._TraitPayoffs`))))
  (return (`local.L_AdditionalSubAbilities`)))

(fn `DoGet_CanBeGiven`
  (params (InAbilityOwner :type "Ck_Handle_AbilityOwner Structure (by ref)") (InAbilitySource :type "Ck_Handle Structure (by ref)"))
  (returns (ReturnValue :type Boolean))
  ;[1 0.1406 0] Traits are always given by default
  (return true))