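; Base CkAbility effect, similar to a GAS GameplayEffect, that modifies float attributes on its ability owner.
; When given, it waits a tick for SetByCaller values, then activates as instant, duration or infinite, optionally periodic via timers.
; Each activation applies non-revocable modifiers or overrides, using discrete, attribute-based or set-by-caller magnitudes.
; Each stack is its own ability instance; policies limit stacks by source or target and govern timer refresh and expiration.
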(event `self.DoOnGiveAbility`
  (params (InOptionalPayload :type "Ck_Ability_Payload_OnGranted Structure (by ref)"))
  (bind (__contextentity __data) (break `Ck_Ability_Payload_OnGranted` InOptionalPayload))
  (bind (__contextentity_2 __data_2) (break `Ck_Ability_Payload_OnGranted` InOptionalPayload))
  (`parent.DoOnGiveAbility` InOptionalPayload)
  ;[0.07812 0 1] HACK: This is a workaround for "SetByCaller" values that will come 1 frame later
  (`KismetSystemLibrary.DelayUntilNextTick`)
  (`|ExecutionSequence`
    (:`then_0`
      (`self.DoValidate_Modifiers`))
    (:`then_1`
      (switch `ECk_Ability_Duration_Policy` (`self.DurationPolicy`)
        (:`Instant`
          (`self.DoRequest_ActivateAbility` (make `Ck_Ability_Payload_OnActivate` __contextentity_2 __data_2))
          (`/CkFoundation/CkAbility/Utils_CkAbility_FL.[Ck][AbilityOwner] Request Revoke Ability (By Entity)` (`self.DoGet_AbilityOwnerEntity`) (`self.DoGet_AbilityEntity`)))
        (:`Duration`
          (bind _outnewtimer (`self.AddNewTimerForMagnitude` (`self.DoGet_AbilityEntity`) (`self.DoGet_AbilityOwnerEntity`) (struct :`TagName` "Ck.Ability.Duration") (`self.DurationMagnitude`)))
          (`|Blueprint_Template` (struct) _outnewtimer
            (:`then`
              (if (`self.IsPeriodicEffect`) :!label _label
                (bind _outnewtimer_2 (`self.AddNewTimerForMagnitude` (`self.DoGet_AbilityEntity`) (`self.DoGet_AbilityOwnerEntity`) (struct :`TagName` "Ck.Ability.Period") (`self.PeriodMagnitude`)))
                (bind (_taskobject _timerdone_outtimerentity) (`|Blueprint_Template` (struct) _outnewtimer_2)
                  (:`then`
                    ;[0.3828 0 1] Immediately Activate the Effect AND when the period is done OR wait until the period is done (i.e. only Activate once per period)
                    (if (`self.ExecutePeriodicEffectOnApplication`)
                      (`self.DoRequest_ActivateAbility` (struct))))
                  (:`TimerDone`
                    (bind _returnvalue (`Ck_Utils_Timer_UE.Request_Reset` _timerdone_outtimerentity))
                    (`Ck_Utils_Timer_UE.Request_Resume` _returnvalue)
                    (`self.DoRequest_ActivateAbility` (struct))))
                (else
                  (`self.DoRequest_ActivateAbility` (make `Ck_Ability_Payload_OnActivate` __contextentity __data)))))
            (:`TimerDone`
              (`self.OnDurationElapsed` (`self.DoGet_AbilityOwnerEntity`) (`self.DoGet_AbilityEntity`)))))
        (:`Infinite`
          (goto _label))))
    (:`then_2`
      (switch `ECk_Ability_Stacking_Policy` (`self.StackingPolicy`)
        (:`Stack_AggregateBySource`
          _)
        (:`Stack_AggregateByTarget`
          _))
      (`self.OnStackAdded` (`self.DoGet_AbilityOwnerEntity`) (`self.DoGet_AbilityEntity`)))))

(event `self.DoOnDeactivateAbility`
  (`parent.DoOnDeactivateAbility`))

(event `self.DoOnActivateAbility`
  (params (InActivationPayload :type "Ck_Ability_Payload_OnActivate Structure (by ref)"))
  ;[1 0.5625 0] Apply Effect
  (`parent.DoOnActivateAbility` InActivationPayload)
  (`self.ApplyEffect` (`self.DoGet_AbilityOwnerEntity`) (`self.DoGet_AbilityEntity`))
  (`self.DoRequest_DeactivateAbility`))

(event `self.DoOnRevokeAbility`
  (`parent.DoOnRevokeAbility`)
  (switch `ECk_Ability_Stacking_Policy` (`self.StackingPolicy`)
    (:`Stack_AggregateBySource`
      _)
    (:`Stack_AggregateByTarget`
      _))
  (`self.OnStackRemoved` (`self.DoGet_AbilityOwnerEntity`) (`self.DoGet_AbilityEntity`)))

(fn `AddNewTimerForMagnitude`
  (params (InAbility :type "Ck_Handle_Ability Structure") (InAbilityOwner :type "Ck_Handle_AbilityOwner Structure") (InTimerName :type "GameplayTag Structure") (InMagnitude :type "Ck_Ability_Magnitude Structure (by ref)"))
  (returns (OutNewTimer :type "Ck_Handle_Timer Structure"))
  (bind (__magnitudecalculation __attributesource __attributebasedmagnitude __snapshot __discretevaluemagnitude __setbycallermagnitude_datatag) (break `Ck_Ability_Magnitude` InMagnitude))
  (switch `ECk_Ability_Modifier_MagnitudeCalculation_Policy` __magnitudecalculation
    (:`DiscreteValue`
      (bind _outnewtimer (`/CkFoundation/CkTimer/Utils_CkTimer_FL.[Ck][Timer] Add New Timer` InTimerName (`local.InAbility`) __discretevaluemagnitude "PauseOnDone" "Running"))
      (return _outnewtimer))
    (:`AttributeBased`
      (bind _outcalculatedmagnitude (`/CkFoundation/CkAttribute/FloatAttribute/Utils_Float_CkAttribute_FL.[Ck][FloatAttribute] Calculate Attribute Magnitude` (`self.Get_SourceOrTarget_ForAbility` (`local.InAbility`) __attributesource) __attributebasedmagnitude))
      (bind _outnewtimer_2 (`/CkFoundation/CkTimer/Utils_CkTimer_FL.[Ck][Timer] Add New Timer` InTimerName (`local.InAbility`) _outcalculatedmagnitude "PauseOnDone" "Running"))
      (return _outnewtimer_2))
    (:`SetByCaller`
      (bind _value (`/CkFoundation/CkAttribute/FloatAttribute/Utils_Float_CkAttribute_FL.[Ck][FloatAttribute] Try Get Final Value_Or (Exec)` (`local.InAbility`) __setbycallermagnitude_datatag)
        (:`HasAttribute`
          (bind _outnewtimer_3 (`/CkFoundation/CkTimer/Utils_CkTimer_FL.[Ck][Timer] Add New Timer` InTimerName (`local.InAbility`) _value "PauseOnDone" "Running"))
          (return _outnewtimer_3))
        (:`MissingAttribute`
          (return))))))

(fn `ApplyEffect`
  (params (InAbilityOwner :type "Ck_Handle_AbilityOwner Structure") (InAbility :type "Ck_Handle_Ability Structure"))
  (locals (L_AttributeModifierValue :type "Float (single-precision)" :default 0.0) (L_Modifier :type "Ck_Ability_Modifier Structure") (L_ModifierMagnitude :type "Ck_Ability_Magnitude Structure") (L_AttributeToModify :type "GameplayTag Structure") (L_ModifierOperation :type "ECk_AttributeModifier_Operation Enum"))
  (bind (__attributetomodify __modifieroperation __modifiermagnitude) (break `Ck_Ability_Modifier` (`local.L_Modifier`)))
  (for _array_element (`self.Modifiers`)
    (set `local.L_Modifier` _array_element)
    (`|ExecutionSequence`
      (:`then_0`
        (set `local.L_AttributeToModify` __attributetomodify)
        (set `local.L_ModifierOperation` __modifieroperation)
        (bind _output_get (set `local.L_ModifierMagnitude` __modifiermagnitude))
        (bind (__magnitudecalculation __attributesource __attributebasedmagnitude __snapshot __discretevaluemagnitude __setbycallermagnitude_datatag) (break `Ck_Ability_Magnitude` _output_get))
        (switch `ECk_Ability_Modifier_MagnitudeCalculation_Policy` __magnitudecalculation
          (:`DiscreteValue`
            (set `local.L_AttributeModifierValue` __discretevaluemagnitude))
          (:`AttributeBased`
            (bind _outcalculatedmagnitude (`/CkFoundation/CkAttribute/FloatAttribute/Utils_Float_CkAttribute_FL.[Ck][FloatAttribute] Calculate Attribute Magnitude` (`self.Get_SourceOrTarget_ForAbility` (`local.InAbility`) __attributesource) __attributebasedmagnitude))
            (set `local.L_AttributeModifierValue` _outcalculatedmagnitude))
          (:`SetByCaller`
            (bind (_hasattribute _value) (`/CkFoundation/CkAttribute/FloatAttribute/Utils_Float_CkAttribute_FL.[Ck][FloatAttribute] Try Get Final Value_Or` (`local.InAbility`) __setbycallermagnitude_datatag))
            (set `local.L_AttributeModifierValue` _value)
            (`Ck_Utils_Ensure_UE.EnsureMsgf` _hasattribute (`|FormatText` "Expected SetByCallerAttribute [{Name}] to be Found on AbilityEffect [{this}]. Was this not correctly added as part of the Ability Effect Construction Script?" (`BlueprintGameplayTagLibrary.GetTagName` __setbycallermagnitude_datatag) self)))))
      (:`then_1`
        (switch `ECk_AttributeModifier_Operation` (`local.L_ModifierOperation`)
          (:`Add`
            (`/CkFoundation/CkAttribute/FloatAttribute/Utils_Float_CkAttribute_FL.[Ck][FloatAttribute] Modify (NotRevocable)` (`local.InAbilityOwner`) (`local.L_AttributeToModify`) (`local.L_AttributeModifierValue`)))
          (:`Subtract`
            (`/CkFoundation/CkAttribute/FloatAttribute/Utils_Float_CkAttribute_FL.[Ck][FloatAttribute] Modify (NotRevocable)` (`local.InAbilityOwner`) (`local.L_AttributeToModify`) (`local.L_AttributeModifierValue`) "Current" "Subtract"))
          (:`Multiply`
            (`/CkFoundation/CkAttribute/FloatAttribute/Utils_Float_CkAttribute_FL.[Ck][FloatAttribute] Modify (NotRevocable)` (`local.InAbilityOwner`) (`local.L_AttributeToModify`) (`local.L_AttributeModifierValue`) "Current" "Multiply"))
          (:`Divide`
            (`/CkFoundation/CkAttribute/FloatAttribute/Utils_Float_CkAttribute_FL.[Ck][FloatAttribute] Modify (NotRevocable)` (`local.InAbilityOwner`) (`local.L_AttributeToModify`) (`local.L_AttributeModifierValue`) "Current" "Divide"))
          (:`Override`
            (`Ck_Utils_FloatAttribute_UE.Request_Override` (`Ck_Utils_FloatAttribute_UE.TryGet` (`local.InAbilityOwner`) (`local.L_AttributeToModify`)) (`local.L_AttributeModifierValue`))))))))

(fn `DoGet_CanBeGiven`
  (params (InAbilityOwner :type "Ck_Handle_AbilityOwner Structure (by ref)") (InAbilitySource :type "Ck_Handle Structure (by ref)"))
  (returns (ReturnValue :type Boolean))
  (locals (L_ThisAbility_InstanceCount :type Integer :default 0) (L_ThisAbilityEffectClass :type "/Game/CkAbility/Effect/AbilityEffectBase_CkAbility_BP Class Reference") (L_ThisAbility_InstanceCount_WithSource :type Integer))
  (`self.DoGet_FulfillsModifiersRequirement` InAbilityOwner
    (:`Yes`
      (set `local.L_ThisAbilityEffectClass` (`GameplayStatics.GetObjectClass` self))
      (set `local.L_ThisAbility_InstanceCount` (`Ck_Utils_AbilityOwner_UE.Get_AbilityCount_OfClass` InAbilityOwner (`local.L_ThisAbilityEffectClass`)))
      (switch `ECk_Ability_Stacking_Policy` (`self.StackingPolicy`)
        (:`DoesNotStack`
          (return (`/CkFoundation/CkCore/Math/Math_CkCore_ML.<=0int` (`local.L_ThisAbility_InstanceCount`))))
        (:`Stack_AggregateBySource`
          (bind _returnvalue (`Ck_Utils_AbilityOwner_UE.ForEach_Ability_OfClass` (`local.InAbilityOwner`) (`local.L_ThisAbilityEffectClass`)))
          (for _array_element _returnvalue
            (if (`Ck_Utils_Handle_UE.IsEqual` (`Ck_Utils_Ability_UE.Get_Source` _array_element) (`local.InAbilitySource`))
              (`/Engine/EditorBlueprintResources/StandardMacros.IncrementInt` (`local.L_ThisAbility_InstanceCount_WithSource`))))
          (return (< (`local.L_ThisAbility_InstanceCount_WithSource`) (`self.StackLimitCount`))))
        (:`Stack_AggregateByTarget`
          (return (< (`local.L_ThisAbility_InstanceCount`) (`self.StackLimitCount`))))))))

(fn `DoGet_FulfillsModifiersRequirement`
  (params (InAbilityOwner :type "Ck_Handle_AbilityOwner Structure"))
  (returns (OutResult :type "ECk_MessageDialog_YesNo Enum"))
  (bind _modifiers (`self.Modifiers`))
  (`/CkFoundation/CkCore/Container/Container_CkCore_ML.Array_IsEmpty_Exec` _modifiers
    (:`Empty`
      (return "Yes"))
    (:`NotEmpty`
      (for _array_element _modifiers
        (`/CkFoundation/CkAttribute/FloatAttribute/Utils_Float_CkAttribute_FL.[Ck][FloatAttribute] Has Attribute (Exec)` (`local.InAbilityOwner`) (`._AttributeToModify` (break `Ck_Ability_Modifier` _array_element))
          (:`HasAttribute`
            (return "Yes"))))
      (return "No"))))

(fn `DoValidate_Modifiers`
  (for _array_element (`self.Modifiers`)
    (bind __attributetomodify (break `Ck_Ability_Modifier` _array_element))
    (`Ck_Utils_Ensure_UE.EnsureMsgf` (`/CkFoundation/CkAttribute/FloatAttribute/Utils_Float_CkAttribute_FL.[Ck][FloatAttribute] Has Attribute` (`self.DoGet_AbilityOwnerEntity`) __attributetomodify) (`|FormatText` "AbilityOwner [{Owner}] does NOT have Attribute [{Attribute}]. The Effect [{Effect}] will not work properly." (`Ck_Utils_Handle_UE.Conv_HandleToText` (`self.DoGet_AbilityOwnerEntity`)) (`BlueprintGameplayTagLibrary.GetDebugStringFromGameplayTag` __attributetomodify) self))))

(fn `Get_SourceOrTarget_ForAbility`
  (params (InAbility :type "Ck_Handle_Ability Structure") (InSourceOrTarget :type "ECk_SourceOrTarget Enum" :default "Source"))
  (returns (OurEntity :type "Ck_Handle Structure"))
  (switch `ECk_SourceOrTarget` InSourceOrTarget
    (:`Source`
      (return (`Ck_Utils_Ability_UE.Get_Source` InAbility)))
    (:`Target`
      (return (`Ck_Utils_EntityLifetime_UE.Get_LifetimeOwner` InAbility)))))

(fn `OnDurationElapsed`
  (params (InAbilityOwner :type "Ck_Handle_AbilityOwner Structure") (InAbility :type "Ck_Handle_Ability Structure"))
  (locals (L_FirstAbilityEntityOfClass_InTheStack :type "Ck_Handle_Ability Structure") (L_FirstAbilityEntityOfClassWithSource_InTheStack :type "Ck_Handle_Ability Structure"))
  (switch `ECk_Ability_Stacking_Policy` (`self.StackingPolicy`)
    (:`DoesNotStack`
      (`/CkFoundation/CkAbility/Utils_CkAbility_FL.[Ck][AbilityOwner] Request Revoke Ability (By Entity)` (`local.InAbilityOwner`) (`local.InAbility`)))
    (:`Stack_AggregateBySource`
      (switch `ECk_Ability_StackExpiration_Policy` (`self.StackExpirationPolicy`)
        (:`ClearEntireStack`
          (bind _returnvalue (`StructUtilsFunctionLibrary.MakeInstancedStruct` (make `/CkFoundation/CkAbility/Effect/AbilityEffectContext_CkAbility_ST` (`local.InAbilityOwner`) (`Ck_Utils_Ability_UE.Get_Source` (`local.InAbility`)) (`GameplayStatics.GetObjectClass` self))))
          (bind _returnvalue_2 (`Ck_Utils_AbilityOwner_UE.ForEach_Ability_If` :`InAbilityOwnerEntity` (`local.InAbilityOwner`) :`InOptionalPayload` _returnvalue :`InPredicate` (`|CreateDelegate` :!event `Predicate_IsAbilityOfClassWithSource`)))
          (for _array_element _returnvalue_2
            (`/CkFoundation/CkAbility/Utils_CkAbility_FL.[Ck][AbilityOwner] Request Revoke Ability (By Entity)` (`local.InAbilityOwner`) _array_element)))
        (:`RemoveSingleStackAndRefreshDuration`
          (bind _returnvalue_3 (`StructUtilsFunctionLibrary.MakeInstancedStruct` (make `/CkFoundation/CkAbility/Effect/AbilityEffectContext_CkAbility_ST` (`local.InAbilityOwner`) (`Ck_Utils_Ability_UE.Get_Source` (`local.InAbility`)) (`GameplayStatics.GetObjectClass` self))))
          (set `local.L_FirstAbilityEntityOfClassWithSource_InTheStack` (`Ck_Utils_AbilityOwner_UE.TryGet_Ability_If` (`local.InAbilityOwner`) _returnvalue_3 (`|CreateDelegate` :!event `Predicate_IsAbilityOfClassWithSource`)))
          (if (`Ck_Utils_Handle_UE.IsEqual` (`local.L_FirstAbilityEntityOfClassWithSource_InTheStack`) (`local.InAbility`))
            (`/CkFoundation/CkAbility/Utils_CkAbility_FL.[Ck][AbilityOwner] Request Revoke Ability (By Entity)` (`local.InAbilityOwner`) (`local.L_FirstAbilityEntityOfClassWithSource_InTheStack`))
            (else
              (`self.RefreshEffectDuration` (`local.InAbility`)))))))
    (:`Stack_AggregateByTarget`
      (switch `ECk_Ability_StackExpiration_Policy` (`self.StackExpirationPolicy`)
        (:`ClearEntireStack`
          (bind _returnvalue_4 (`Ck_Utils_AbilityOwner_UE.ForEach_Ability_OfClass` (`local.InAbilityOwner`) (`GameplayStatics.GetObjectClass` self)))
          (for _array_element_2 _returnvalue_4
            (`/CkFoundation/CkAbility/Utils_CkAbility_FL.[Ck][AbilityOwner] Request Revoke Ability (By Entity)` (`local.InAbilityOwner`) _array_element_2)))
        (:`RemoveSingleStackAndRefreshDuration`
          (set `local.L_FirstAbilityEntityOfClass_InTheStack` (`Ck_Utils_AbilityOwner_UE.TryGet_AbilityByClass` (`local.InAbilityOwner`) (`GameplayStatics.GetObjectClass` self)))
          (if (`Ck_Utils_Handle_UE.IsEqual` (`local.L_FirstAbilityEntityOfClass_InTheStack`) (`local.InAbility`))
            (`/CkFoundation/CkAbility/Utils_CkAbility_FL.[Ck][AbilityOwner] Request Revoke Ability (By Entity)` (`local.InAbilityOwner`) (`local.L_FirstAbilityEntityOfClass_InTheStack`))
            (else
              (`self.RefreshEffectDuration` (`local.InAbility`)))))))))

(fn `OnStackAdded`
  (params (InAbilityOwner :type "Ck_Handle_AbilityOwner Structure") (InAbilityAdded :type "Ck_Handle_Ability Structure"))
  (locals (L_DurationTimer :type "Ck_Handle_Timer Structure") (L_Ability :type "Ck_Handle_Ability Structure") (L_PeriodTimer :type "Ck_Handle_Timer Structure"))
  (bind _durationpolicy (`self.DurationPolicy`))
  (bind _returnvalue (`Ck_Utils_AbilityOwner_UE.ForEach_Ability_OfClass` InAbilityOwner (`GameplayStatics.GetObjectClass` self)))
  (for _array_element _returnvalue
    (set `local.L_Ability` _array_element)
    (switch `ECk_Ability_Stacking_Policy` (`self.StackingPolicy`)
      (:`Stack_AggregateBySource`
        (if (`Ck_Utils_Handle_UE.IsEqual` (`Ck_Utils_Ability_UE.Get_Source` (`local.L_Ability`)) (`Ck_Utils_Ability_UE.Get_Source` (`local.InAbilityAdded`)))
          (`|ExecutionSequence` :!label _label
            (:`then_0`
              ;[0.3125 0 1] Try Refresh Duration
              (switch `ECk_Ability_StackDurationRefresh_Policy` (`self.StackDurationRefreshPolicy`)
                (:`RefreshOnSuccessfulApplication`
                  (bind _output_get (set `local.L_DurationTimer` (`Ck_Utils_Timer_UE.TryGet_Timer` (`local.L_Ability`) (struct :`TagName` "Ck.Ability.Duration"))))
                  (bind _outhandle (`/CkFoundation/CkEcs/EntityHandle_CkEcs_ML.ValidateEntityHandle` _output_get)
                    (:`IsValid`
                      (bind _returnvalue_2 (`Ck_Utils_Timer_UE.Request_Reset` _outhandle))
                      (`Ck_Utils_Timer_UE.Request_Resume` _returnvalue_2))
                    (:`NotValid`
                      (`Ck_Utils_Ensure_UE.EnsureMsgf` (or (`|EnumEquality` _durationpolicy "Instant") (`|EnumEquality` _durationpolicy "Infinite")) (`|FormatText` "Could not find the [{TimerName}] for AbilityEffect [{this}] that is NOT " (`BlueprintGameplayTagLibrary.GetTagName` (`BlueprintGameplayTagLibrary.MakeLiteralGameplayTag` (struct :`TagName` "Ck.Ability.Duration"))) self)))))))
            (:`then_1`
              ;[0.8984 0 1] Try Refresh Period
              (switch `ECk_Ability_StackPeriodReset_Policy` (`self.StackPeriodResetPolicy`)
                (:`ResetOnSuccessfulApplication`
                  (bind _output_get_2 (set `local.L_PeriodTimer` (`Ck_Utils_Timer_UE.TryGet_Timer` (`local.L_Ability`) (struct :`TagName` "Ck.Ability.Period"))))
                  (bind _outhandle_2 (`/CkFoundation/CkEcs/EntityHandle_CkEcs_ML.ValidateEntityHandle` _output_get_2)
                    (:`IsValid`
                      (bind _returnvalue_3 (`Ck_Utils_Timer_UE.Request_Reset` _outhandle_2))
                      (`Ck_Utils_Timer_UE.Request_Resume` _returnvalue_3))
                    (:`NotValid`
                      (`Ck_Utils_Ensure_UE.EnsureMsgf` (not (`self.IsPeriodicEffect`)) (`|FormatText` "Could not find the [{TimerName}] for AbilityEffect [{this}] that IS a Periodic Effect" (`BlueprintGameplayTagLibrary.GetTagName` (`BlueprintGameplayTagLibrary.MakeLiteralGameplayTag` (struct :`TagName` "Ck.Ability.Period"))) self))))))))))
      (:`Stack_AggregateByTarget`
        (goto _label)))))

(fn `OnStackRemoved`
  (params (InAbilityOwner :type "Ck_Handle_AbilityOwner Structure") (InAbilityRemoved :type "Ck_Handle_Ability Structure")))

(fn `Predicate_IsAbilityOfClassWithSource`
  (params (InHandle :type "Ck_Handle Structure") (OutResult :type "Ck_SharedBool Structure") (InOptionalPayload :type "InstancedStruct Structure"))
  (locals (L_AbilityOwner :type "Ck_Handle_AbilityOwner Structure") (L_AbilitySource :type "Ck_Handle Structure") (L_AbilityScript :type "Ck_Ability_Script_PDA Class Reference") (L_Ability :type "Ck_Handle_Ability Structure"))
  (set `local.L_Ability` (`Ck_Utils_Ability_UE.DoCastChecked` InHandle))
  (bind _value (`StructUtilsFunctionLibrary.GetInstancedStructValue` InOptionalPayload)
    (:`Valid`
      (bind (_inabilityowner _inabilitysource _inabilityscript) (break `/CkFoundation/CkAbility/Effect/AbilityEffectContext_CkAbility_ST` _value))
      (set `local.L_AbilityOwner` _inabilityowner)
      (set `local.L_AbilitySource` _inabilitysource)
      (set `local.L_AbilityScript` _inabilityscript)
      (if (== (`Ck_Utils_Ability_UE.Get_ScriptClass` (`local.L_Ability`)) (`local.L_AbilityScript`))
        (if (`Ck_Utils_Handle_UE.IsEqual` (`Ck_Utils_Ability_UE.Get_Source` (`local.L_Ability`)) (`local.L_AbilitySource`))
          (`Ck_Utils_SharedBool_UE.Set` (`local.OutResult`) true))))))

(fn `RefreshEffectDuration`
  (params (InHandle :type "Ck_Handle Structure"))
  (bind _outhandle (`/CkFoundation/CkEcs/EntityHandle_CkEcs_ML.ValidateEntityHandle` (`Ck_Utils_Timer_UE.TryGet_Timer` InHandle (struct :`TagName` "Ck.Ability.Duration")))
    (:`IsValid`
      (bind _returnvalue (`Ck_Utils_Timer_UE.Request_Reset` _outhandle))
      (`Ck_Utils_Timer_UE.Request_Resume` _returnvalue))))

(fn `ResetEffectPeriod`
  (params (InHandle :type "Ck_Handle Structure"))
  (bind _outhandle (`/CkFoundation/CkEcs/EntityHandle_CkEcs_ML.ValidateEntityHandle` (`Ck_Utils_Timer_UE.TryGet_Timer` InHandle (struct :`TagName` "Ck.Ability.Period")))
    (:`IsValid`
      (bind _returnvalue (`Ck_Utils_Timer_UE.Request_Reset` _outhandle))
      (`Ck_Utils_Timer_UE.Request_Resume` _returnvalue))))