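; Base construction script for ability effect entities that creates the attributes backing their Set by Caller magnitudes.
; After parent construction, it reads the effect's class defaults from the entity's script class, raising an ensure if the class is not a base ability effect.
; It adds a non-replicated float attribute, named by data tag, for a Set by Caller duration on timed effects and for each Set by Caller modifier.
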(fn `DoAdd_SetByCaller_Attributes`
  (params (InHandle :type "Ck_Handle Structure") (InAbilityEffectCDO :type "/CkFoundation/CkAbility/AbilityEffectBase_CkAbility_BP Object Reference"))
  (locals (L_DurationPolicy :type "ECk_Ability_Duration_Policy Enum" :default "Instant") (L_DurationMagnitude :type "Ck_Ability_Magnitude Structure"))
  (bind (__magnitudecalculation __attributebasedmagnitude __discretevaluemagnitude __setbycallermagnitude_datatag) (break `Ck_Ability_Magnitude` (`/CkFoundation/CkAbility/AbilityEffectBase_CkAbility_BP.DurationMagnitude` (`local.InAbilityEffectCDO`))))
  (`|ExecutionSequence`
    (:`then_0`
      ;[0 1 0.25] Duration Magnitude
      (switch `ECk_Ability_Duration_Policy` (`/CkFoundation/CkAbility/AbilityEffectBase_CkAbility_BP.DurationPolicy` (`local.InAbilityEffectCDO`))
        (:`Duration`
          (switch `ECk_Ability_Modifier_MagnitudeCalculation_Policy` __magnitudecalculation
            (:`SetByCaller`
              (`/CkFoundation/CkAttribute/FloatAttribute/Utils_Float_CkAttribute_FL.[Ck][FloatAttribute] Add New Attribute` (`local.InHandle`) __setbycallermagnitude_datatag 0.0 "DoesNotReplicate"))))))
    (:`then_1`
      ;[0.6172 0 1] Modifier Magnitudes
      (for _array_element (`/CkFoundation/CkAbility/AbilityEffectBase_CkAbility_BP.Modifiers` (`local.InAbilityEffectCDO`))
        (bind (__magnitudecalculation_2 __attributebasedmagnitude_2 __discretevaluemagnitude_2 __setbycallermagnitude_datatag_2) (break `Ck_Ability_Magnitude` (`._ModifierMagnitude` (break `Ck_Ability_Modifier` _array_element))))
        (switch `ECk_Ability_Modifier_MagnitudeCalculation_Policy` __magnitudecalculation_2
          (:`SetByCaller`
            (`/CkFoundation/CkAttribute/FloatAttribute/Utils_Float_CkAttribute_FL.[Ck][FloatAttribute] Add New Attribute` (`local.InHandle`) __setbycallermagnitude_datatag_2 0.0 "DoesNotReplicate")))))))

(fn `DoConstruct`
  (params (InHandle :type "Ck_Handle Structure (by ref)") (InOptionalParams :type "InstancedStruct Structure (by ref)"))
  (locals (L_AbilityEffectScriptClass :type "/CkFoundation/CkAbility/AbilityEffectBase_CkAbility_BP Class Reference") (L_AbilityEffectScriptCDO :type "/CkFoundation/CkAbility/AbilityEffectBase_CkAbility_BP Object Reference"))
  (`parent.DoConstruct` InHandle InOptionalParams)
  (bind _asability_effect_base_ck_ability_bp (castclass `/CkFoundation/CkAbility/AbilityEffectBase_CkAbility_BP` (`Ck_Utils_Ability_UE.Get_ScriptClass` (`Ck_Utils_Ability_UE.DoCastChecked` InHandle)))
    (:`then`
      (bind _output_get (set `local.L_AbilityEffectScriptClass` _asability_effect_base_ck_ability_bp))
      (set `local.L_AbilityEffectScriptCDO` (`Ck_Utils_Object_UE.DoGet_ClassDefaultObject` _output_get))
      (`self.DoAdd_SetByCaller_Attributes` InHandle (`local.L_AbilityEffectScriptCDO`))
      (return))
    (:`CastFailed`
      (`Ck_Utils_Ensure_UE.TriggerEnsure` (`|FormatText` "Base Ability Effect ConstructionScript [{cs}] is being used to construct Entity [{entity}] that is NOT an Ability" self (`Ck_Utils_Handle_UE.Conv_HandleToText` InHandle))))))