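; Test target dummy that reacts to damage with a physics jolt and a hit flash.
; On BeginPlay it simulates physics on the skeletal mesh bodies below the hip bone, leaving the hip itself out.
; Any damage calls an MC event that applies a fixed impulse to the chest bone and stamps game time into the ActivationTime parameter on the mesh materials and a dynamic overlay material created in the construction script.
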(event `self.ReceiveBeginPlay`
  (`SkeletalMeshComponent.SetAllBodiesBelowSimulatePhysics` (`self.SkeletalMesh`) "HipBone" true false))

(event `self.ReceiveAnyDamage`
  (params (Damage :type "Float (single-precision)") (DamageType :type "DamageType Object Reference") (InstigatedBy :type "Controller Object Reference") (DamageCauser :type "Actor Object Reference"))
  (`self.MC_OnDamageTaken`))

(event `MC_OnDamageTaken`
  (`PrimitiveComponent.AddImpulseAtLocation` (`self.SkeletalMesh`) (10000.0 10000.0 100000.0) (0.0 0.0 0.0) "ChestBoneA")
  (`MeshComponent.SetScalarParameterValueOnMaterials` (`self.SkeletalMesh`) "ActivationTime" (`KismetSystemLibrary.GetGameTimeInSeconds`))
  (`MaterialInstanceDynamic.SetScalarParameterValue` (`self._HitReactFlash_DynamicMaterial`) "ActivationTime" (`KismetSystemLibrary.GetGameTimeInSeconds`)))

(event `self.ReceiveTick`
  (params (DeltaSeconds :type "Float (single-precision)")))

(fn `UserConstructionScript`
  (bind _returnvalue (`KismetMaterialLibrary.CreateDynamicMaterialInstance` "/CkFoundation/Materials/HitReactFlash/MI_HitReactFlash.MI_HitReactFlash"))
  (bind _output_get (set `self._HitReactFlash_DynamicMaterial` _returnvalue))
  (`MeshComponent.SetOverlayMaterial` (`self.SkeletalMesh`) _output_get))