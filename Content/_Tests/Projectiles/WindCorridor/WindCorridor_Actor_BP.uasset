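; Test actor for a wind corridor that alters the velocity of projectiles or other entities passing through it, built on the Ck ECS framework.
; On BeginPlay it binds to the begin and end overlap of its WindCorridor gym sensor.
; Overlap begin adds the detected marker's attached entity as a target of a bulk velocity modifier, and overlap end removes it.
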(event `self.ReceiveBeginPlay`
  (`Ck_Utils_Sensor_UE.BindTo_OnBeginOverlap` (`Ck_EcsConstructionScript_ActorComponent_UE._Entity` (`self.Ecs_ConstructionScript_AC`)) (struct :`TagName` "Ck.Gyms.Sensor.WindCorridor") "FireIfPayloadInFlight" (delegate `OnBeginOverlap`))
  (`Ck_Utils_Sensor_UE.BindTo_OnEndOverlap` (`Ck_EcsConstructionScript_ActorComponent_UE._Entity` (`self.Ecs_ConstructionScript_AC`)) (struct :`TagName` "Ck.Gyms.Sensor.WindCorridor") "FireIfPayloadInFlight" (delegate `OnEndOverlap`)))

(event `OnBeginOverlap`
  (params (InHandle :type "Ck_Handle Structure") (InPayload :type "Ck_Sensor_Payload_OnBeginOverlap Structure"))
  (`Ck_Utils_BulkVelocityModifier_UE.Request_AddTarget` InHandle (struct) (make `Ck_Request_BulkVelocityModifier_AddTarget` (`._Handle` (break `Ck_EntityOwningActor_BasicDetails` (`._MarkerAttachedEntityAndActor` (break `Ck_Marker_BasicDetails` (`._MarkerDetails` (break `Ck_Sensor_Payload_OnBeginOverlap` InPayload)))))))))

(event `OnEndOverlap`
  (params (InHandle :type "Ck_Handle Structure") (InPayload :type "Ck_Sensor_Payload_OnEndOverlap Structure"))
  (`Ck_Utils_BulkVelocityModifier_UE.Request_RemoveTarget` InHandle (struct) (make `Ck_Request_BulkVelocityModifier_RemoveTarget` (`._Handle` (break `Ck_EntityOwningActor_BasicDetails` (`._MarkerAttachedEntityAndActor` (break `Ck_Marker_BasicDetails` (`._MarkerDetails` (break `Ck_Sensor_Payload_OnEndOverlap` InPayload)))))))))

(fn `UserConstructionScript`)