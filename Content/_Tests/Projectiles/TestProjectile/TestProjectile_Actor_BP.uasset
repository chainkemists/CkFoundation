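; Test projectile actor that damages what it hits through an ECS Sensor and spawns an explosion effect on EndPlay.
; BeginPlay binds two overlap delegates to the test sensor: regular overlaps destroy the entity and damage the other actor, while non-marker overlaps only destroy it.
; Unconnected nodes keep a plain capsule-overlap version for comparison with the Sensor/Marker approach, plus a client-versus-server position debug draw.
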(event `self.ReceiveBeginPlay`
  ;[1 0 0.6562] Sensor Overlaps
  (`Ck_Utils_Sensor_UE.BindTo_OnBeginOverlap_NonMarker` (`Ck_EcsConstructionScript_ActorComponent_UE._Entity` (`self.Ecs_ConstructionScript_AC`)) (struct :`TagName` "Ck.Gyms.Sensor.TestProjectile") "FireIfPayloadInFlight" (delegate `OnNonMarkerOverlap`))
  (`Ck_Utils_Sensor_UE.BindTo_OnBeginOverlap` (`Ck_EcsConstructionScript_ActorComponent_UE._Entity` (`self.Ecs_ConstructionScript_AC`)) (struct :`TagName` "Ck.Gyms.Sensor.TestProjectile") "FireIfPayloadInFlight" (delegate `OnRegularOverlap`)))

(event `self.ReceiveEndPlay`
  (params (EndPlayReason :type "EEndPlayReason Enum" :default "Destroyed"))
  (`NiagaraFunctionLibrary.SpawnSystemAtLocation` "/CkFoundation/_Tests/Projectiles/TestProjectile/Effects/NS_Boom.NS_Boom" (`self.K2_GetActorLocation`) (`self.K2_GetActorRotation`)))

(event `OnNonMarkerOverlap`
  (params (InHandle :type "Ck_Handle Structure") (InPayload :type "Ck_Sensor_Payload_OnBeginOverlap_NonMarker Structure"))
  ;[1 0 0.6562] Sensor Overlaps
  (`Ck_Utils_EntityLifetime_UE.Request_DestroyEntity` InHandle))

(event `OnRegularOverlap`
  (params (InHandle :type "Ck_Handle Structure") (InPayload :type "Ck_Sensor_Payload_OnBeginOverlap Structure"))
  ;[1 0 0.6562] Sensor Overlaps
  (`Ck_Utils_EntityLifetime_UE.Request_DestroyEntity` InHandle)
  (`GameplayStatics.ApplyDamage` (`._OtherActor` (break `Ck_Sensor_BeginOverlap_UnrealDetails` (`._OverlapDetails` (break `Ck_Sensor_Payload_OnBeginOverlap` InPayload)))) 50.0))

(event `self.CollisionCapsule.OnComponentBeginOverlap`
  (params (OverlappedComponent :type "PrimitiveComponent Object Reference") (OtherActor :type "Actor Object Reference") (OtherComp :type "PrimitiveComponent Object Reference") (OtherBodyIndex :type Integer) (bFromSweep :type Boolean) (SweepResult :type "HitResult Structure (by ref)"))
  ;[0.6641 1 0] What it would look like WITHOUT Sensor/Marker
)

(fn `UserConstructionScript`)