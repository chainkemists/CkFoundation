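; Test gym ability for the rate-of-fire cooldown scenario that stays active briefly, then deactivates itself.
; On activation it adds or replaces a short, running Ck timer on its own ability entity and binds to that timer's done event.
; Timer completion requests deactivation, and deactivation removes the timer from the entity.
; No cooldown logic lives in this graph.
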(event `self.DoOnActivateAbility`
  (params (InActivationPayload :type "Ck_Ability_ActivationPayload Structure (by ref)"))
  (`parent.DoOnActivateAbility` InActivationPayload)
  (`Ck_Utils_Timer_UE.AddOrReplace` (`self.Self_Get_AbilityEntity`) (make `Ck_Fragment_Timer_ParamsData` (`self.TimerName`) (`Ck_Utils_Time_UE.Make_FromSeconds` 0.05) "CountUp" "PauseOnDone" "Running"))
  (`Ck_Utils_Timer_UE.BindTo_OnTimerDone` (`self.Self_Get_AbilityEntity`) (`self.TimerName`) "FireIfPayloadInFlightThisFrame" (delegate `OnDone`)))

(event `OnDone`
  (params (InHandle :type "Ck_Handle Structure") (InChrono :type "Ck_Chrono Structure"))
  (`self.Self_Request_DeactivateAbility`))

(event `self.DoOnDeactivateAbility`
  (`parent.DoOnDeactivateAbility`)
  (`Ck_Utils_Timer_UE.Remove` (`self.Self_Get_AbilityEntity`) (`self.TimerName`)))