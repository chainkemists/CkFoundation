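; Gym test jump ability for the Ck ability system that launches the actor named in its activation payload upward.
; On activation it reads the jumping actor from the payload's instanced struct and applies a mass-independent velocity-change impulse to its capsule.
; It then spawns a takeoff ability cue at the actor's location, applies its cooldown and immediately deactivates itself, all only when the payload is valid.
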(event `self.DoOnGiveAbility`
  (`parent.DoOnGiveAbility`))

(event `self.DoOnActivateAbility`
  (params (InActivationPayload :type "Ck_Ability_ActivationPayload Structure (by ref)"))
  (`parent.DoOnActivateAbility` InActivationPayload)
  (bind _value (`StructUtilsFunctionLibrary.GetInstancedStructValue` (`._Data` (break `Ck_Ability_ActivationPayload` InActivationPayload)))
    (:`Valid`
      (bind _injumpingactor (break `/CkFoundation/_Tests/Abilities/Abilities/Jump/Gym_Jump_Ability_Payload_CkST` _value))
      (`PrimitiveComponent.AddImpulse` (`Actor.GetComponentByClass` _injumpingactor "/Script/Engine.CapsuleComponent") (0.0 0.0 1000.0) "None" true)
      (`Ck_Utils_AbilityCue_UE.Request_Spawn_AbilityCue` (`self.Self_Get_AbilityEntity`) (make `Ck_Request_AbilityCue_Spawn` (struct :`TagName` "Ck.Gyms.Ability.Cue.JumpTakeoff") self (make `Ck_AbilityCue_Params` (`Actor.K2_GetActorLocation` _injumpingactor))))
      (`self.Self_Request_ApplyCooldown`)
      (`self.Self_Request_DeactivateAbility`))))

(event `self.DoOnDeactivateAbility`
  (`parent.DoOnDeactivateAbility`))