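; Gym test cost ability for firing projectiles, using a timer on the ability owner's lifetime owner as a stand-in bullet counter instead of attributes.
; Activation jumps the NumberOfBullets timer by one second.
; TryAddCostNotMet, also run when the ability is given, checks the timer's elapsed seconds and conditionally tries to activate the FireProjectileCostNotMet ability by name on the owner.
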(event `/CkFoundation/CkAbilities/Ability_ActivateByEvent_Base_CkBP.DoOnGiveAbility`
  (`self.TryAddCostNotMet`)
  (`parent.DoOnGiveAbility`))

(event `self.DoOnActivateAbility`
  (params (InActivationPayload :type "Ck_Ability_ActivationPayload Structure (by ref)"))
  (`Ck_Utils_Timer_UE.Request_Jump` (`Ck_Utils_Timer_UE.Get_Timer` (`Ck_Utils_EntityLifetime_UE.Get_LifetimeOwner` (`self.Self_Get_AbilityOwnerEntity`)) (`self._NumberOfBullets_TimerName`)) (make `Ck_Request_Timer_Jump` (`Ck_Utils_Time_UE.Make_FromSeconds` 1.0)))
  (`parent.DoOnActivateAbility` InActivationPayload))

(fn `TryAddCostNotMet`
  (`parent.TryAddCostNotMet`)
  (if (`/CkFoundation/CkCore/Math/BPML_CkCore_Math.==0float` (`._Seconds` (break `Ck_Time` (`.OutTimeElapsed` (`Ck_Utils_Chrono_UE.Break_Chrono` (`Ck_Utils_Timer_UE.Get_CurrentTimerValue` (`Ck_Utils_Timer_UE.Get_Timer` (`Ck_Utils_EntityLifetime_UE.Get_LifetimeOwner` (`self.Self_Get_AbilityOwnerEntity`)) (`self._NumberOfBullets_TimerName`))))))))
    (`Ck_Utils_AbilityOwner_UE.Request_TryActivateAbility` (`self.Self_Get_AbilityOwnerEntity`) (`Ck_Utils_AbilityOwner_UE.Make_Request_ActivateAbility_ByName` (struct :`TagName` "Ck.Gyms.Ability.FireProjectileCostNotMet")))))