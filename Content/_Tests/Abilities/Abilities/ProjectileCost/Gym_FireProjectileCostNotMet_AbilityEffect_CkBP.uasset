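; Gym test ability effect for the fire-projectile "cost not met" state, which watches the ability owner's bullet count.
; On activation it binds to the bullet-count timer on the owner's lifetime owner, also firing for updates already in flight that frame.
; Each update checks the timer's elapsed time against zero to decide whether the effect deactivates itself, using the timer as an ammo counter.
; Deactivation removes the binding.
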(event `self.DoOnActivateAbility`
  (`parent.DoOnActivateAbility`)
  (`Ck_Utils_Timer_UE.BindTo_OnTimerUpdate` (`Ck_Utils_EntityLifetime_UE.Get_LifetimeOwner` (`self.Self_Get_AbilityOwnerEntity`)) (`self.NumberOfBullets_TimerName`) "FireIfPayloadInFlightThisFrame" (delegate `OnUpdate`)))

(event `OnUpdate`
  (params (InHandle :type "Ck_Handle Structure") (InChrono :type "Ck_Chrono Structure"))
  (if (`/CkFoundation/CkCore/Math/BPML_CkCore_Math.>=0float` (`._Seconds` (break `Ck_Time` (`.OutTimeElapsed` (`Ck_Utils_Chrono_UE.Break_Chrono` InChrono)))))
    (`self.Self_Request_DeactivateAbility`)))

(event `self.DoOnDeactivateAbility`
  (`parent.DoOnDeactivateAbility`)
  (`Ck_Utils_Timer_UE.UnbindFrom_OnTimerUpdate` (`Ck_Utils_EntityLifetime_UE.Get_LifetimeOwner` (`self.Self_Get_AbilityOwnerEntity`)) (`self.NumberOfBullets_TimerName`) (delegate `OnUpdate`)))