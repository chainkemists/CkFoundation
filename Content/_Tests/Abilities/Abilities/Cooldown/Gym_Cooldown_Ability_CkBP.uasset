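; Test gym ability for cooldowns that stays active for a fixed timer duration, then deactivates itself.
; On activation it adds or replaces a named timer on its own ability entity, resumes it and binds to its completion, which requests deactivation.
; On deactivation it resets and pauses that timer and unbinds from the completion event.
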(event `self.DoOnDeactivateAbility`
  (bind _returnvalue (`self.Self_Get_AbilityEntity`))
  (bind _timername (`self.TimerName`))
  (`parent.DoOnDeactivateAbility`)
  (`Ck_Utils_Timer_UE.Request_Reset` _returnvalue _timername)
  (`Ck_Utils_Timer_UE.Request_Pause` _returnvalue _timername)
  (`Ck_Utils_Timer_UE.UnbindFrom_OnTimerDone` (`self.Self_Get_AbilityEntity`) (`self.TimerName`) (`|CreateDelegate` :!event `OnDone`)))

(event `self.DoOnActivateAbility`
  (`parent.DoOnActivateAbility`)
  (`Ck_Utils_Timer_UE.AddOrReplace` (`self.Self_Get_AbilityEntity`) (make `Ck_Fragment_Timer_ParamsData` (`self.TimerName`) (`Ck_Utils_Time_UE.Make_FromSeconds` 5.0) "CountUp" "PauseOnDone" "Running"))
  (`Ck_Utils_Timer_UE.Request_Resume` (`self.Self_Get_AbilityEntity`) (`self.TimerName`))
  (`Ck_Utils_Timer_UE.BindTo_OnTimerDone` (`self.Self_Get_AbilityEntity`) (`self.TimerName`) "FireIfPayloadInFlightThisFrame" (delegate `OnDone`)))

(event `OnDone`
  (params (InHandle :type "Ck_Handle Structure") (InChrono :type "Ck_Chrono Structure"))
  (`self.Self_Request_DeactivateAbility`))