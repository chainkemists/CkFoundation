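; Test gym Heat ability that runs a countdown timer and sends a cooldown event to its owner when the timer depletes.
; On activation it creates and completes the timer, binds to depletion, and tracks a task listening for activation-trigger events on the owner.
; Each trigger consumes a slice of the timer and resumes it.
; Depletion deactivates the ability, which removes the timer; the explicit unbind node is unconnected.
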(event `self.DoOnActivateAbility`
  (`parent.DoOnActivateAbility`)
  (`Ck_Utils_Timer_UE.AddOrReplace` (`self.Self_Get_AbilityEntity`) (make `Ck_Fragment_Timer_ParamsData` (`self.TimerName`) (`Ck_Utils_Time_UE.Make_FromSeconds` 5.0) "CountDown" "StopOnDone" "Running"))
  (bind _taskobject (`|Blueprint_Template` (`self.Self_Get_AbilityEntity`) (`self.Self_Get_AbilityOwnerEntity`) (`self.ActivationTriggers`))
    (:`then`
      (`self.Self_Request_TrackTask` _taskobject)
      (`Ck_Utils_Timer_UE.Request_Complete` (`self.Self_Get_AbilityEntity`) (`self.TimerName`))
      (`Ck_Utils_Timer_UE.BindTo_OnTimerDepleted` (`self.Self_Get_AbilityEntity`) (`self.TimerName`) "FireIfPayloadInFlightThisFrame" (delegate `OnDepleted`)))
    (:`EventFired`
      (`Ck_Utils_Timer_UE.Request_Consume` (`self.Self_Get_AbilityEntity`) (`self.TimerName`) (make `Ck_Request_Timer_Consume` (`Ck_Utils_Time_UE.Make_FromSeconds` 0.25)))
      (`Ck_Utils_Timer_UE.Request_Resume` (`self.Self_Get_AbilityEntity`) (`self.TimerName`)))))

(event `OnDepleted`
  (params (InHandle :type "Ck_Handle Structure") (InChrono :type "Ck_Chrono Structure"))
  (`Ck_Utils_AbilityOwner_UE.Request_SendEvent` (`self.Self_Get_AbilityOwnerEntity`) (make `Ck_Request_AbilityOwner_SendEvent` (make `Ck_AbilityOwner_Event` (struct :`TagName` "Ck.Gyms.Ability.Cooldown"))))
  (`self.Self_Request_DeactivateAbility`))

(event `self.DoOnDeactivateAbility`
  (`parent.DoOnDeactivateAbility`)
  (`Ck_Utils_Timer_UE.Remove` (`self.Self_Get_AbilityEntity`) (`self.TimerName`)))