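; Gym test ability that marks reload conditions as not met by toggling its own active state from a named timer.
; On give, it binds to that timer, found two lifetime owners above the ability owner, and starts inactive if elapsed time is zero, active otherwise.
; Each timer update activates it when remaining time is zero and deactivates it otherwise.
; Revoking the ability unbinds from the timer.
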(event `self.DoOnGiveAbility`
  (bind _returnvalue (`Ck_Utils_Timer_UE.Get_Timer` (`Ck_Utils_EntityLifetime_UE.Get_LifetimeOwner` (`Ck_Utils_EntityLifetime_UE.Get_LifetimeOwner` (`self.Self_Get_AbilityOwnerEntity`))) (`self.TimerName`)))
  (`parent.DoOnGiveAbility`)
  (`Ck_Utils_Timer_UE.BindTo_OnTimerUpdate` _returnvalue "FireIfPayloadInFlightThisFrame" (delegate `OnTimerUpdate`))
  (if (`Ck_Utils_Time_UE.Get_IsZero` (`.OutTimeElapsed` (`Ck_Utils_Chrono_UE.Break_Chrono` (`Ck_Utils_Timer_UE.Get_CurrentTimerValue` _returnvalue))))
    (`self.Self_Request_DeactivateAbility`)
    (else
      (`self.Self_Request_ActivateAbility` (struct)))))

(event `OnTimerUpdate`
  (params (InHandle :type "Ck_Handle Structure") (InChrono :type "Ck_Chrono Structure"))
  (if (`Ck_Utils_Time_UE.Get_IsZero` (`.OutTimeRemaining` (`Ck_Utils_Chrono_UE.Break_Chrono` InChrono)))
    (`self.Self_Request_ActivateAbility` (struct))
    (else
      (`self.Self_Request_DeactivateAbility`))))

(event `self.DoOnRevokeAbility`
  (`parent.DoOnRevokeAbility`)
  (`Ck_Utils_Timer_UE.UnbindFrom_OnTimerUpdate` (`Ck_Utils_Timer_UE.Get_Timer` (`Ck_Utils_EntityLifetime_UE.Get_LifetimeOwner` (`Ck_Utils_EntityLifetime_UE.Get_LifetimeOwner` (`self.Self_Get_AbilityOwnerEntity`))) (`self.TimerName`)) (`|CreateDelegate` :!event `OnTimerUpdate`)))