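; Test gym ability that fires a projectile from the ability owner, then immediately deactivates itself.
; On activation it sends the Fire gym event on its own ability entity and requests a server-only spawn of a replicated projectile at the owning actor's transform, ignoring collision.
; Deactivation sends the same Fire event again, so each activation emits it twice.
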(event `self.DoOnDeactivateAbility`
  (`parent.DoOnDeactivateAbility`)
  (`Ck_Utils_AbilityOwner_UE.Request_SendEvent` (`self.Self_Get_AbilityEntity`) (make `Ck_Request_AbilityOwner_SendEvent` (make `Ck_AbilityOwner_Event` (struct :`TagName` "Ck.Gyms.Ability.Fire")))))

(event `self.DoOnActivateAbility`
  (bind _returnvalue (`Ck_Utils_OwningActor_UE.Get_EntityOwningActor` (`self.Self_Get_AbilityOwnerEntity`)))
  (`parent.DoOnActivateAbility`)
  (`Ck_Utils_AbilityOwner_UE.Request_SendEvent` (`self.Self_Get_AbilityEntity`) (make `Ck_Request_AbilityOwner_SendEvent` (make `Ck_AbilityOwner_Event` (struct :`TagName` "Ck.Gyms.Ability.Fire"))))
  (`Ck_Utils_ActorModifier_UE.Request_SpawnActor` (`self.Self_Get_AbilityEntity`) (make `Ck_Request_ActorModifier_SpawnActor` (make `Ck_Utils_Actor_SpawnActor_Params` _returnvalue "/CkFoundation/_Tests/Abilities/Gym_Abilities_Projectile.Gym_Abilities_Projectile_C" null (`Actor.GetTransform` _returnvalue) "AlwaysSpawn" "Replicated") (struct :`_Params` (struct :`_AttachmentRules` (struct :`_LocationRule` "KeepWorld" :`_RotationRule` "KeepWorld" :`_ScaleRule` "KeepWorld"))) "SpawnOnServer"))
  (`self.Self_Request_DeactivateAbility`))