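; Test target dummy actor for the Ck ability gyms that triggers its Move ability shortly after play begins.
; On BeginPlay, only on the server, it waits a fixed delay, then requests activation of the Ck.Gyms.Ability.Move ability on its own entity handle.
; The ability's granting and behavior are not defined in these graphs, and Tick and overlap events are disabled.
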(event `self.ReceiveBeginPlay`
  (`parent.ReceiveBeginPlay`)
  (if (`KismetSystemLibrary.IsServer`)
    (`KismetSystemLibrary.Delay` 6.0)
    (`Ck_Utils_AbilityOwner_UE.Request_TryActivateAbility` (`Ck_Utils_OwningActor_UE.Get_ActorEntityHandleFromSelf`) (make `Ck_Request_AbilityOwner_ActivateAbility` "SearchByName" (struct :`TagName` "Ck.Gyms.Ability.Move")))))

(fn `UserConstructionScript`
  (`parent.UserConstructionScript`))