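; Test target dummy that displays a float gym attribute as its health on a HealthValue text element.
; On BeginPlay it binds to value changes of that attribute on its ECS construction-script entity, firing if a payload is already in flight, and sets the initial text.
; Each change rewrites the text with the final value rounded to an integer, while the initial text is left unrounded.
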(event `self.ReceiveBeginPlay`
  (bind __entity (`Ck_EcsConstructionScript_ActorComponent_UE._Entity` (`self.Ecs_ConstructionScript_AC`)))
  (`parent.ReceiveBeginPlay`)
  (`Ck_Utils_FloatAttribute_UE.BindTo_OnValueChanged` (struct :`TagName` "Ck.Gyms.Attribute.Float.A") __entity "FireIfPayloadInFlight" (delegate `OnHealthChanged`))
  (`TextRenderComponent.K2_SetText` (`self.HealthValue`) (`KismetTextLibrary.Conv_DoubleToText` (`Ck_Utils_FloatAttribute_UE.Get_FinalValue` (struct :`TagName` "Ck.Gyms.Attribute.Float.A") __entity) "HalfToEven")))

(event `OnHealthChanged`
  (params (InHandle :type "Ck_Handle Structure") (InPayload :type "Ck_Payload_FloatAttribute_OnValueChanged Structure"))
  (`TextRenderComponent.K2_SetText` (`self.HealthValue`) (`KismetTextLibrary.Conv_IntToText` (`KismetMathLibrary.Round` (`._FinalValue` (break `Ck_Payload_FloatAttribute_OnValueChanged` InPayload))))))

(fn `UserConstructionScript`
  (`parent.UserConstructionScript`))