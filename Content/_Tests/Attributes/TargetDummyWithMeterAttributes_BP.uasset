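; Test dummy actor that displays ECS meter attributes for the attribute gym and compares their server and client values.
; Once dependent entities finish replicating, it fills two text displays with the base values of Meters A and B and binds Meter A's change event to update its text.
; A gate opened at that point lets Tick print Meter A's min, current and max under separate server and client keys.
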(event `self.Ecs_ConstructionScript_AC._OnReplicationComplete_MC`
  (`Ck_Utils_EntityReplicationDriver_UE.Promise_OnReplicationCompleteAllDependents` (`Ck_Utils_OwningActor_UE.Get_ActorEcsHandle` null) (delegate `Future_OnDependentsReplicated`)))

(event `Future_OnDependentsReplicated`
  (params (InHandle :type "Ck_Handle Structure"))
  (bind (_outmetercapacity _outmetercurrentvalue _outremaining _outused) (`Ck_Utils_Meter_UE.Break_Meter` (`Ck_Utils_MeterAttribute_UE.Get_FinalValue` (`Ck_Utils_OwningActor_UE.Get_ActorEcsHandle` null) (struct :`TagName` "Ck.Gyms.Attribute.Meter.A"))))
  (bind (__mincapacity __maxcapacity) (break `Ck_Meter_Capacity` _outmetercapacity))
  (bind _result (`|FormatText` "[{Min},{Curr},{Max}]" __mincapacity (`._CurrentValue` (break `Ck_Meter_Current` _outmetercurrentvalue)) __maxcapacity))
  (`Ck_Utils_MeterAttribute_UE.BindTo_OnValueChanged` (`Ck_Utils_OwningActor_UE.Get_ActorEcsHandle` null) (struct :`TagName` "Ck.Gyms.Attribute.Meter.A") "FireIfPayloadInFlight" "DoNothing" (delegate `OnMeterValueChanged`))
  (`TextRenderComponent.K2_SetText` (`self.MeterValue`) (`Ck_Utils_Meter_UE.Conv_MeterToText` (`Ck_Utils_MeterAttribute_UE.Get_BaseValue` (`Ck_Utils_OwningActor_UE.Get_ActorEcsHandle` null) (struct :`TagName` "Ck.Gyms.Attribute.Meter.A"))))
  (`TextRenderComponent.K2_SetText` (`self.Meter2Value`) (`Ck_Utils_Meter_UE.Conv_MeterToText` (`Ck_Utils_MeterAttribute_UE.Get_BaseValue` (`Ck_Utils_OwningActor_UE.Get_ActorEcsHandle` null) (struct :`TagName` "Ck.Gyms.Attribute.Meter.B"))))
  (goto _label :!via `Open`))

(event `self.ReceiveTick`
  (params (DeltaSeconds :type "Float (single-precision)"))
  (bind (_outmetercapacity _outmetercurrentvalue _outremaining _outused) (`Ck_Utils_Meter_UE.Break_Meter` (`Ck_Utils_MeterAttribute_UE.Get_FinalValue` (`Ck_Utils_OwningActor_UE.Get_ActorEcsHandle` null) (struct :`TagName` "Ck.Gyms.Attribute.Meter.A"))))
  (bind (__mincapacity __maxcapacity) (break `Ck_Meter_Capacity` _outmetercapacity))
  (bind _result (`|FormatText` "[{Min},{Curr},{Max}]" __mincapacity (`._CurrentValue` (break `Ck_Meter_Current` _outmetercurrentvalue)) __maxcapacity))
  (`/Engine/EditorBlueprintResources/StandardMacros.Gate` true :!label _label
    (:`Exit`
      (if (`KismetSystemLibrary.IsServer`)
        (`KismetSystemLibrary.PrintText` _result true true (struct :`G` 0.66 :`B` 1.0 :`A` 1.0) 2.0 "ServerMeterPawn")
        (else
          (`KismetSystemLibrary.PrintText` _result true true (struct :`G` 0.66 :`B` 1.0 :`A` 1.0) 2.0 "ClientMeterPawn"))))))

(event `OnMeterValueChanged`
  (params (InHandle :type "Ck_Handle Structure") (InPayload :type "Ck_Payload_MeterAttribute_OnValueChanged Structure"))
  (`TextRenderComponent.K2_SetText` (`self.MeterValue`) (`Ck_Utils_Meter_UE.Conv_MeterToText` (`._FinalValue` (break `Ck_Payload_MeterAttribute_OnValueChanged` InPayload)))))

(fn `MeterToText`
  (params (InMeter :type "Ck_Meter Structure (by ref)"))
  (returns (Result :type Text))
  (bind (_outmetercapacity _outmetercurrentvalue _outremaining _outused) (`Ck_Utils_Meter_UE.Break_Meter` InMeter))
  (bind (__mincapacity __maxcapacity) (break `Ck_Meter_Capacity` _outmetercapacity))
  (return (`|FormatText` "{min},{curr},{max}" __mincapacity (`._AmountUsed` (break `Ck_Meter_Used` _outused)) __maxcapacity)))

(fn `UserConstructionScript`
  (`parent.UserConstructionScript`))