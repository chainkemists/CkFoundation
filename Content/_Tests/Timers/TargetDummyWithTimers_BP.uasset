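; Test target dummy that displays the elapsed time of two gameplay-tagged ECS timers, A and B, on its text elements.
; After the entity and all its dependents finish replicating, it looks up both timers and binds their Done and Update delegates, firing for payloads already in flight.
; Updates write elapsed seconds to each timer's text, and Done calls resume on that timer.
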(event `self.Ecs_ConstructionScript_AC._OnReplicationComplete_MC`
  (`Ck_Utils_EntityReplicationDriver_UE.Promise_OnReplicationCompleteAllDependents` (`Ck_Utils_OwningActor_UE.Get_ActorEntityHandleFromSelf`) (delegate `OnReplicaitonComplete`)))

(event `OnReplicaitonComplete`
  (params (InHandle :type "Ck_Handle Structure"))
  (set `self.TimerHandle_A` (`Ck_Utils_Timer_UE.Get_Timer` (`Ck_Utils_OwningActor_UE.Get_ActorEntityHandleFromSelf`) (struct :`TagName` "Ck.Gyms.Timer.A")))
  (set `self.TimerHandle_B` (`Ck_Utils_Timer_UE.Get_Timer` (`Ck_Utils_OwningActor_UE.Get_ActorEntityHandleFromSelf`) (struct :`TagName` "Ck.Gyms.Timer.B")))
  (`Ck_Utils_Timer_UE.BindTo_OnTimerDone` (`self.TimerHandle_A`) "FireIfPayloadInFlight" (delegate `OnTimerA_Done`))
  (`Ck_Utils_Timer_UE.BindTo_OnTimerDone` (`self.TimerHandle_B`) "FireIfPayloadInFlight" (delegate `OnTimerB_Done`))
  (`Ck_Utils_Timer_UE.BindTo_OnTimerUpdate` (`self.TimerHandle_A`) "FireIfPayloadInFlight" (delegate `OnTimerA_Update`))
  (`Ck_Utils_Timer_UE.BindTo_OnTimerUpdate` (`self.TimerHandle_B`) "FireIfPayloadInFlight" (delegate `OnTimerB_Update`)))

(event `OnTimerA_Done`
  (params (InHandle :type "Ck_Handle Structure") (InChrono :type "Ck_Chrono Structure"))
  (`Ck_Utils_Timer_UE.Request_Resume` InHandle))

(event `OnTimerA_Update`
  (params (InHandle :type "Ck_Handle Structure") (InChrono :type "Ck_Chrono Structure"))
  (`TextRenderComponent.K2_SetText` (`self.TimerA_Value`) (`KismetTextLibrary.Conv_DoubleToText` (`._Seconds` (break `Ck_Time` (`.OutTimeElapsed` (`Ck_Utils_Chrono_UE.Break_Chrono` InChrono)))) "HalfToEven" false true 1 324 0 2)))

(event `OnTimerB_Done`
  (params (InHandle :type "Ck_Handle Structure") (InChrono :type "Ck_Chrono Structure"))
  (`Ck_Utils_Timer_UE.Request_Resume` InHandle))

(event `OnTimerB_Update`
  (params (InHandle :type "Ck_Handle Structure") (InChrono :type "Ck_Chrono Structure"))
  (`TextRenderComponent.K2_SetText` (`self.TimerB_Value`) (`KismetTextLibrary.Conv_DoubleToText` (`._Seconds` (break `Ck_Time` (`.OutTimeElapsed` (`Ck_Utils_Chrono_UE.Break_Chrono` InChrono)))) "HalfToEven" false true 1 324 0 2)))

(fn `UserConstructionScript`
  (`parent.UserConstructionScript`))