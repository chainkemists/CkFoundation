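; Base Anim Notify State for ECS-ready actors, giving child notify states Begin, Tick and End hooks that receive the owner's entity handle.
; Each engine callback runs only in game on a valid owner whose role matches ReplicationType.
; It ensures the owner is ECS Ready, resolves and validates its entity, then returns the result of the matching Ck override.
; The overrides return false by default.
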(fn `[Ck] Received_NotifyBegin (Override)`
  (params (InOwnerActor :type "Actor Object Reference") (InOwnerEntity :type "Ck_Handle Structure") (InMeshComp :type "SkeletalMeshComponent Object Reference") (InAnimation :type "AnimSequenceBase Object Reference") (InEventReference :type "AnimNotifyEventReference Structure") (InTotalDuration :type "Float (double-precision)"))
  (returns (OutResult :type Boolean))
  (return false))

(fn `[Ck] Received_NotifyEnd (Override)`
  (params (InOwnerActor :type "Actor Object Reference") (InOwnerEntity :type "Ck_Handle Structure") (InMeshComp :type "SkeletalMeshComponent Object Reference") (InAnimation :type "AnimSequenceBase Object Reference") (InEventReference :type "AnimNotifyEventReference Structure"))
  (returns (OutResult :type Boolean))
  (return false))

(fn `[Ck] Received_NotifyTick (Override)`
  (params (InOwnerActor :type "Actor Object Reference") (InOwnerEntity :type "Ck_Handle Structure") (InMeshComp :type "SkeletalMeshComponent Object Reference") (InAnimation :type "AnimSequenceBase Object Reference") (InEventReference :type "AnimNotifyEventReference Structure") (InFrameDeltaT :type "Float (double-precision)"))
  (returns (OutResult :type Boolean))
  (return false))

(fn `Received_NotifyBegin`
  (params (MeshComp :type "SkeletalMeshComponent Object Reference") (Animation :type "AnimSequenceBase Object Reference") (TotalDuration :type "Float (single-precision)") (EventReference :type "AnimNotifyEventReference Structure (by ref)"))
  (returns (ReturnValue :type Boolean))
  (locals (L_Owner :type "Actor Object Reference") (L_OwnerEntity :type "Ck_Handle Structure"))
  (`/Engine/EditorBlueprintResources/StandardMacros.IsValid` MeshComp
    (:`Is Valid`
      (bind _output_get (set `local.L_Owner` (`ActorComponent.GetOwner` MeshComp)))
      (`/Engine/EditorBlueprintResources/StandardMacros.IsValid` _output_get
        (:`Is Valid`
          (if (`Ck_Utils_Game_UE.Get_IsInGame` MeshComp)
            ;[0 0.0625 1] Must match replication type
            (if (`Ck_Utils_Net_UE.Get_IsRoleMatching` (`local.L_Owner`) (`self.ReplicationType`))
              (`|K2Node_Ensure` self (`Ck_Utils_OwningActor_UE.Get_IsActorEcsReady` (`local.L_Owner`)) "Anim Notify State [{self}] used in Animation [{anim}] requires the Owner [{owner}] that is ECS Ready!" (`local.Animation`) (`local.L_Owner`)
                (:`Passed`
                  (bind _output_get_2 (set `local.L_OwnerEntity` (`Ck_Utils_OwningActor_UE.Get_ActorEntityHandle` (`local.L_Owner`))))
                  (`/CkFoundation/CkEcs/EntityHandle_CkEcs_ML.ValidateEntityHandle` _output_get_2
                    (:`IsValid`
                      (bind _outresult (`self.[Ck] Received_NotifyBegin (Override)` (`local.L_Owner`) (`local.L_OwnerEntity`) (`local.MeshComp`) (`local.Animation`) (`local.EventReference`) (`local.TotalDuration`)))
                      (return _outresult))))))))))))

(fn `Received_NotifyEnd`
  (params (MeshComp :type "SkeletalMeshComponent Object Reference") (Animation :type "AnimSequenceBase Object Reference") (EventReference :type "AnimNotifyEventReference Structure (by ref)"))
  (returns (ReturnValue :type Boolean))
  (locals (L_Owner :type "Actor Object Reference") (L_OwnerEntity :type "Ck_Handle Structure"))
  (`/Engine/EditorBlueprintResources/StandardMacros.IsValid` MeshComp
    (:`Is Valid`
      (bind _output_get (set `local.L_Owner` (`ActorComponent.GetOwner` MeshComp)))
      (`/Engine/EditorBlueprintResources/StandardMacros.IsValid` _output_get
        (:`Is Valid`
          (if (`Ck_Utils_Game_UE.Get_IsInGame` MeshComp)
            ;[0 0.0625 1] Must match replication type
            (if (`Ck_Utils_Net_UE.Get_IsRoleMatching` (`local.L_Owner`) (`self.ReplicationType`))
              (`|K2Node_Ensure` self (`Ck_Utils_OwningActor_UE.Get_IsActorEcsReady` (`local.L_Owner`)) "Anim Notify State [{self}] used in Animation [{anim}] requires the Owner [{owner}] that is ECS Ready!" (`local.Animation`) (`local.L_Owner`)
                (:`Passed`
                  (bind _output_get_2 (set `local.L_OwnerEntity` (`Ck_Utils_OwningActor_UE.Get_ActorEntityHandle` (`local.L_Owner`))))
                  (`/CkFoundation/CkEcs/EntityHandle_CkEcs_ML.ValidateEntityHandle` _output_get_2
                    (:`IsValid`
                      (bind _outresult (`self.[Ck] Received_NotifyEnd (Override)` (`local.L_Owner`) (`local.L_OwnerEntity`) (`local.MeshComp`) (`local.Animation`) (`local.EventReference`)))
                      (return _outresult))))))))))))

(fn `Received_NotifyTick`
  (params (MeshComp :type "SkeletalMeshComponent Object Reference") (Animation :type "AnimSequenceBase Object Reference") (FrameDeltaTime :type "Float (single-precision)") (EventReference :type "AnimNotifyEventReference Structure (by ref)"))
  (returns (ReturnValue :type Boolean))
  (locals (L_Owner :type "Actor Object Reference") (L_OwnerEntity :type "Ck_Handle Structure"))
  (`/Engine/EditorBlueprintResources/StandardMacros.IsValid` MeshComp
    (:`Is Valid`
      (bind _output_get (set `local.L_Owner` (`ActorComponent.GetOwner` MeshComp)))
      (`/Engine/EditorBlueprintResources/StandardMacros.IsValid` _output_get
        (:`Is Valid`
          (if (`Ck_Utils_Game_UE.Get_IsInGame` MeshComp)
            ;[0 0.0625 1] Must match replication type
            (if (`Ck_Utils_Net_UE.Get_IsRoleMatching` (`local.L_Owner`) (`self.ReplicationType`))
              (`|K2Node_Ensure` self (`Ck_Utils_OwningActor_UE.Get_IsActorEcsReady` (`local.L_Owner`)) "Anim Notify State [{self}] used in Animation [{anim}] requires the Owner [{owner}] that is ECS Ready!" (`local.Animation`) (`local.L_Owner`)
                (:`Passed`
                  (bind _output_get_2 (set `local.L_OwnerEntity` (`Ck_Utils_OwningActor_UE.Get_ActorEntityHandle` (`local.L_Owner`))))
                  (`/CkFoundation/CkEcs/EntityHandle_CkEcs_ML.ValidateEntityHandle` _output_get_2
                    (:`IsValid`
                      (bind _outresult (`self.[Ck] Received_NotifyTick (Override)` (`local.L_Owner`) (`local.L_OwnerEntity`) (`local.MeshComp`) (`local.Animation`) (`local.EventReference`) (`local.FrameDeltaTime`)))
                      (return _outresult))))))))))))