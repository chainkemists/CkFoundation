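; Base ability script for Cues in CkAbilities, acting as a one-shot, self-destroying ability.
; On activation it reads the cue params from the ability owner entity, passes them to the empty OnCueFired hook, then immediately requests its own deactivation.
; Deactivation calls DestroyCue, which force-destroys the ability owner entity, so that entity lives only for a single firing.
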(event `self.DoOnActivateAbility`
  (params (InActivationPayload :type "Ck_Ability_ActivationPayload Structure (by ref)"))
  (`parent.DoOnActivateAbility` InActivationPayload)
  (`self.OnCueFired` (`Ck_Utils_AbilityCue_UE.Get_Params` (`self.Self_Get_AbilityOwnerEntity`)))
  (`self.Self_Request_DeactivateAbility`))

(event `self.DoOnDeactivateAbility`
  (`parent.DoOnDeactivateAbility`)
  (`self.DestroyCue`))

(fn `DestroyCue`
  (`Ck_Utils_EntityLifetime_UE.Request_DestroyEntity` (`self.Self_Get_AbilityOwnerEntity`)))

(fn `OnCueFired`
  (params (InCueParams :type "Ck_AbilityCue_Params Structure")))