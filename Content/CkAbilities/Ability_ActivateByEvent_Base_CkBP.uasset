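; Base CkAbilities ability that activates or deactivates itself in response to named events on its ability owner.
; It binds to the owner's events when given, also firing for payloads already in flight that frame, and unbinds when revoked.
; Event names are exact-matched against ActivationTriggers when inactive or DeactivationTriggers when active.
; The first match ends the batch scan, and activation forwards the event's context entity and data.
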(event `self.DoOnGiveAbility`
  (`parent.DoOnGiveAbility`)
  (`Ck_Utils_AbilityOwner_UE.BindTo_OnEvents` (`self.Self_Get_AbilityOwnerEntity`) "FireIfPayloadInFlightThisFrame" (delegate `OnEvents`)))

(event `OnEvents`
  (params (InHandle :type "Ck_Handle Structure") (InEvents :type "Array of Ck_AbilityOwner_Event Structure (by ref)"))
  (`self.TryActivateOrDeactivateOnEvent` InEvents))

(event `self.DoOnRevokeAbility`
  (`parent.DoOnRevokeAbility`)
  (`Ck_Utils_AbilityOwner_UE.UnbindFrom_OnEvents` (`self.Self_Get_AbilityOwnerEntity`) (delegate `OnEvents`)))

(fn `TryActivateOrDeactivateOnEvent`
  (params (InEvents :type "Array of Ck_AbilityOwner_Event Structure"))
  (locals (L_AbilityOwnerEvent :type "Ck_AbilityOwner_Event Structure"))
  (bind (__eventname __contextentity __eventdata) (break `Ck_AbilityOwner_Event` (`local.L_AbilityOwnerEvent`)))
  (for _array_element InEvents
    (set `local.L_AbilityOwnerEvent` _array_element)
    (switch `ECk_Ability_Status` (`self.Self_Get_Status`)
      (:`NotActive`
        (if (`BlueprintGameplayTagLibrary.HasTag` (`self.ActivationTriggers`) (`._EventName` (break `Ck_AbilityOwner_Event` (`local.L_AbilityOwnerEvent`))) true)
          (`|ExecutionSequence`
            (:`then_0`
              (break))
            (:`then_1`
              (`self.Self_Request_ActivateAbility` (make `Ck_Ability_ActivationPayload` __contextentity __eventdata))))))
      (:`Active`
        (if (`BlueprintGameplayTagLibrary.HasTag` (`self.DeactivationTriggers`) (`._EventName` (break `Ck_AbilityOwner_Event` (`local.L_AbilityOwnerEvent`))) true)
          (`|ExecutionSequence`
            (:`then_0`
              (`self.Self_Request_DeactivateAbility`))
            (:`then_1`
              (break))))))))