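; Spline builder actor whose construction script fills a spline with spline mesh components, sized from the mesh's bounds on the chosen forward axis.
; Meshes are either spaced along the spline with a rotation offset, or bent end to end using length-clamped tangents.
; Bent sections blend up vectors from a per-point override map, falling back to the spline's own.
; Each component gets configured collision; optional arrows aid up-vector debugging.
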(fn `CalculateLocationAndTangent`
  (params (Index :type Integer) (SectionLength :type "Float (double-precision)"))
  (returns (OutLocation :type "Vector Structure") (OutTangent :type "Vector Structure"))
  (locals (L_Distance :type "Float (double-precision)"))
  (bind _output_get (set `local.L_Distance` (* Index SectionLength)))
  (return (`SplineComponent.GetLocationAtDistanceAlongSpline` (`self.Spline`) _output_get "Local") (`KismetMathLibrary.ClampVectorSize` (`SplineComponent.GetTangentAtDistanceAlongSpline` (`self.Spline`) _output_get "Local") 0.0 SectionLength)))

(fn `SetupSplineMeshCollisionSettings`
  (params (Target :type "PrimitiveComponent Object Reference"))
  (bind _keys (`BlueprintMapLibrary.Map_Keys` (`self.CollisionResponseToChannel`)))
  (for _array_element _keys
    (`PrimitiveComponent.SetCollisionResponseToChannel` Target _array_element (`BlueprintMapLibrary.Map_Find` (`self.CollisionResponseToChannel`) _array_element)))
  (`PrimitiveComponent.SetCollisionEnabled` Target (`self.SplineMeshCollision`)))

(fn `UserConstructionScript`
  (locals (L_Index :type Integer) (L_SplineMeshBoundingBox :type "Box Structure") (L_SplineMeshBounds :type "Vector Structure") (L_SplineMeshLength :type "Float (single-precision)" :default 0.0) (L_SectionLength :type "Float (double-precision)") (L_SectionStartPoint :type "Float (double-precision)") (L_SectionEndPoint :type "Float (double-precision)" :default 0.0) (L_SectionMidPoint :type "Float (double-precision)") (L_InputKey :type "Float (single-precision)" :default 0.0))
  (bind _returnvalue (`SplineComponent.GetSplineLength` (`self.Spline`)))
  (bind (_outmin _outmax) (`Ck_Utils_Geometry_UE.Break_Box_WithCenterAndExtents` (`local.L_SplineMeshBoundingBox`)))
  (bind _returnvalue_2 (+ (`local.L_SectionStartPoint`) (`local.L_SectionLength`)))
  (bind (_value _returnvalue_3) (`BlueprintMapLibrary.Map_Find` (`self.UpVectors`) (`KismetMathLibrary.FFloor` (`local.L_InputKey`))))
  (bind (_value_2 _returnvalue_4) (`BlueprintMapLibrary.Map_Find` (`self.UpVectors`) (`KismetMathLibrary.FCeil` (`local.L_InputKey`))))
  (set `local.L_SplineMeshBoundingBox` (`StaticMesh.GetBoundingBox` (`self.SplineMesh`)))
  (set `local.L_SplineMeshBounds` (- _outmax _outmin))
  (set `local.L_SplineMeshLength` (select `ESplineMeshAxis` (`self.ForwardAxis`) :`X` (.x (`local.L_SplineMeshBounds`)) :`Y` (.y (`local.L_SplineMeshBounds`)) :`Z` (.z (`local.L_SplineMeshBounds`)) :!type "Float (single-precision)"))
  (set `local.L_SectionLength` (`KismetMathLibrary.SelectFloat` (+ (`self.Spacing`) (`local.L_SplineMeshLength`)) (`local.L_SplineMeshLength`) (`self.SpaceMeshes`)))
  (bind _index (`/CkFoundation/CkCore/Container/Container_CkCore_ML.ForLoop_C++` 0 "LessThan" (`KismetMathLibrary.FTrunc` (/ (`SplineComponent.GetSplineLength` (`self.Spline`)) (`local.L_SectionLength`))))
    (:`LoopBody`
      (set `local.L_Index` _index)
      (set `local.L_SectionStartPoint` (* (`local.L_Index`) (`local.L_SectionLength`)))
      (if (`self.SpaceMeshes`)
        (bind _returnvalue_5 (`AddComponent|NODE_AddSplineMeshComponent-0` :`RelativeTransform` (`KismetMathLibrary.MakeTransform` (`SplineComponent.GetLocationAtDistanceAlongSpline` (`self.Spline`) (`local.L_SectionStartPoint`) "Local") (`KismetMathLibrary.ComposeRotators` (`self.SplineMeshRotation`) (`SplineComponent.GetRotationAtDistanceAlongSpline` (`self.Spline`) (`local.L_SectionStartPoint`) "Local")))))
        (`StaticMeshComponent.SetStaticMesh` _returnvalue_5 (`self.SplineMesh`))
        (`self.SetupSplineMeshCollisionSettings` _returnvalue_5)
        (`SplineMeshComponent.SetForwardAxis` _returnvalue_5 (`self.ForwardAxis`) true)
        (else
          (bind _returnvalue_6 (`AddComponent|NODE_AddSplineMeshComponent-4`))
          (`StaticMeshComponent.SetStaticMesh` _returnvalue_6 (`self.SplineMesh`))
          (`self.SetupSplineMeshCollisionSettings` _returnvalue_6)
          (`SplineMeshComponent.SetForwardAxis` _returnvalue_6 (`self.ForwardAxis`) true)
          (bind (_outlocation _outtangent) (`self.CalculateLocationAndTangent` (`local.L_Index`) (`local.L_SectionLength`)))
          (bind (_outlocation_2 _outtangent_2) (`self.CalculateLocationAndTangent` (`/CkFoundation/CkCore/Math/Math_CkCore_ML.+1 (int)` (`local.L_Index`)) (`local.L_SectionLength`)))
          (`SplineMeshComponent.SetStartAndEnd` _returnvalue_6 _outlocation _outtangent _outlocation_2 _outtangent_2 true)
          (set `local.L_SectionEndPoint` (`KismetMathLibrary.SelectFloat` _returnvalue_2 _returnvalue (< _returnvalue_2 _returnvalue)))
          (set `local.L_SectionMidPoint` (+ (`/CkFoundation/CkCore/Math/Math_CkCore_ML./2 (float)` (- (`local.L_SectionStartPoint`) (`local.L_SectionEndPoint`))) (`local.L_SectionEndPoint`)))
          (set `local.L_InputKey` (`SplineComponent.GetInputKeyValueAtDistanceAlongSpline` (`self.Spline`) (`/CkFoundation/CkCore/Math/Math_CkCore_ML./2 (float)` (+ (`local.L_SectionStartPoint`) (`local.L_SectionEndPoint`)))))
          (if (and _returnvalue_4 _returnvalue_3)
            (`SplineMeshComponent.SetSplineUpDir` _returnvalue_6 (`KismetMathLibrary.VLerp` _value_2 _value (`KismetMathLibrary.Fraction` (`local.L_InputKey`))) true)
            (else
              (`SplineMeshComponent.SetSplineUpDir` _returnvalue_6 (`SplineComponent.GetUpVectorAtDistanceAlongSpline` (`self.Spline`) (`local.L_SectionMidPoint`) "Local") true)))))
      (if (`self.ShowUpVector`)
        (`AddComponent|NODE_AddArrowComponent-0` :`RelativeTransform` (`KismetMathLibrary.MakeTransform` (`SplineComponent.GetLocationAtSplinePoint` (`self.Spline`) (`local.L_Index`) "Local") (`KismetMathLibrary.ComposeRotators` (struct :`Pitch` 90.0) (`SplineComponent.GetRotationAtSplinePoint` (`self.Spline`) (`local.L_Index`) "Local")) (1.0 5.0 5.0)))))))